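; BP_Turret is an enemy turret that tracks the player and fires BP_BadmanShot projectiles.
; Every Tick it rotates the whole actor toward the player and fires when the player's X position is within a set range of the turret sprite's.
; Shots spawn at the Arrow component with a rescaled flipbook, and a DoOnce reset after a short Delay limits the fire rate.
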(event Custom|TurretShoot
  ;[1 1 1] TurretShooting
  (Utilities|FlowControl|DoOnce false :!label _label
    (:Completed
      (bind _returnvalue (Game|SpawnActorfromClass "/Game/SpaceState/Blueprint/Enemies/DataTable/BP_BadmanShot.BP_BadmanShot_C" (Transformation|GetWorldTransform (Variables|Default|GetArrow)) "Undefined" 0 0))
      (Transformation|SetRelativeScale3D (Variables|/Game/SpaceState/Blueprint/Enemies/DataTable/BP_BadmanShot.BP_BadmanShot_C|GetPaperFlipbook _returnvalue) "1.000000,0.000000,3.000000")
      (Utilities|FlowControl|Delay 0.5)
      (goto _label Reset))))

(event EventBeginPlay)

(event Collision|EventActorBeginOverlap
  (params (OtherActor :type Actor%20Object%20Reference)))

(event EventTick
  (params (DeltaSeconds :type Float%20%28single-precision%29))
  (Utilities|FlowControl|Sequence
    (:then_0
      (bind _output_get (Variables|Default|SetDist (- (.x (Transformation|GetActorLocation (Game|GetPlayerCharacter 0))) (.x (Transformation|GetWorldLocation (Variables|Default|GetPaperSprite))))))
      (if (Math|Float|InRange(Float) _output_get -1e+02 1e+02)
        (CallFunction|TurretShoot)))
    (:then_1
      (Transformation|SetActorRotation (Math|Rotator|FindLookatRotation (Transformation|GetActorLocation) (Transformation|GetActorLocation (Game|GetPlayerCharacter 0)))))))

(fn ConstructionScript)