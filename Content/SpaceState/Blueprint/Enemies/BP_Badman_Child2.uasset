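; BP_Badman_Child2 is an enemy variant, apparently a child of BP_Badman, configured from a fixed row of EnemyTable.
; BeginPlay picks the row by hardcoded index and copies its health, movement, ranges, weapon, drop and flag values into variables, then sets the Paper2D sprite and scale.
; Its BeginPlay does not call the parent's, and it adds no other active logic beyond the parent construction script call.
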(event Collision|EventActorBeginOverlap
  (params (OtherActor :type Actor%20Object%20Reference)))

(event EventTick
  (params (DeltaSeconds :type Float%20%28single-precision%29))
  (|CallParentFunction 0.0))

(event EventBeginPlay
  (bind _outrownames (DataTable|GetDataTableRowNames "/Game/SpaceState/Blueprint/Enemies/EnemyTable.EnemyTable"))
  (Variables|Default|SetEnemyArray _outrownames)
  (bind _output_get (Variables|Default|SetEnemyIndex 3))
  (bind _returnvalue (Utilities|GetDataTableRow "/Game/SpaceState/Blueprint/Enemies/EnemyTable.EnemyTable" (Utilities|Array|Get(acopy) (Variables|Default|GetEnemyArray) _output_get))
    (:then
      (bind _output_get_2 (Variables|Default|SetCurrentEnemy _returnvalue))
      (Variables|Default|SetEnemyName (.EName (Utilities|Struct|BreakEnemyStrut _output_get_2)))
      (Variables|Default|SetEnemySprite (.ESprite (Utilities|Struct|BreakEnemyStrut _output_get_2)))
      (Variables|Default|SetBadman_Health (.EHP (Utilities|Struct|BreakEnemyStrut _output_get_2)))
      (Variables|Default|SetBadmanSpeed (.ESpeed (Utilities|Struct|BreakEnemyStrut _output_get_2)))
      (Variables|Default|SetEnemyScale (.EScale (Utilities|Struct|BreakEnemyStrut _output_get_2)))
      (Variables|Default|SetEnemyCRangeMinusX (.EChaseRMinusX (Utilities|Struct|BreakEnemyStrut _output_get_2)))
      (Variables|Default|SetEnemyCRangePlusX (.EChaseRPlusX (Utilities|Struct|BreakEnemyStrut _output_get_2)))
      (Variables|Default|SetEnemyRangeX (.ETargetRX (Utilities|Struct|BreakEnemyStrut _output_get_2)))
      (Variables|Default|SetEnemyWeaponSound (.EWeaponSound (Utilities|Struct|BreakEnemyStrut _output_get_2)))
      (Variables|Default|SetEnemyWeaponScale (.EWeaponScale (Utilities|Struct|BreakEnemyStrut _output_get_2)))
      (Variables|Default|SetEWeaponRangeSeconds (.EWeaponRangeSeconds (Utilities|Struct|BreakEnemyStrut _output_get_2)))
      (Variables|Default|SetEWeaponZMin (.EWeapZMin (Utilities|Struct|BreakEnemyStrut _output_get_2)))
      (Variables|Default|SetEWeapZmax (.EWeapZMax (Utilities|Struct|BreakEnemyStrut _output_get_2)))
      (Variables|Default|SetEWeaponSpeed (.EWeaponXVelocity (Utilities|Struct|BreakEnemyStrut _output_get_2)))
      (Variables|Default|SetEWeapFireRateSeconds (.EFireRateSeconds (Utilities|Struct|BreakEnemyStrut _output_get_2)))
      (Variables|Default|SetEWeaponDamage (.EDamage (Utilities|Struct|BreakEnemyStrut _output_get_2)))
      (Variables|Default|SetEItemDrop? (.EItemDrop? (Utilities|Struct|BreakEnemyStrut _output_get_2)))
      (Variables|Default|SetEStatic? (.EIsStatic? (Utilities|Struct|BreakEnemyStrut _output_get_2)))
      (Variables|Default|SetEIsposter (.IsPoster? (Utilities|Struct|BreakEnemyStrut _output_get_2)))
      (Rendering|Components|Sprite|SetSprite (Variables|Default|GetPaperSprite) (Variables|Default|GetEnemySprite))
      (Transformation|SetRelativeScale3D (Variables|Default|GetPaperSprite) (Variables|Default|GetEnemyScale)))))

(fn ConstructionScript
  (|CallParentFunction))