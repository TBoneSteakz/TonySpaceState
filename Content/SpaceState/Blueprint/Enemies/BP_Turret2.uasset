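; BP_Turret2 is a space-game enemy turret that turns to face the player every tick.
; Tick also calls TurretShoot when the player's X position is within a fixed range of the turret's PaperSprite.
; TurretShoot is empty: the DoOnce and Delay throttled logic that spawns BP_BadmanShot from the Arrow is disconnected, so the turret never fires.
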(event Custom|TurretShoot
  ;[1 1 1] TurretShooting
)

(event EventBeginPlay)

(event Collision|EventActorBeginOverlap
  (params (OtherActor :type Actor%20Object%20Reference)))

(event EventTick
  (params (DeltaSeconds :type Float%20%28single-precision%29))
  (Utilities|FlowControl|Sequence
    (:then_0
      (bind _output_get (Variables|Default|SetDist (- (.x (Transformation|GetActorLocation (Game|GetPlayerCharacter 0))) (.x (Transformation|GetWorldLocation (Variables|Default|GetPaperSprite))))))
      (if (Math|Float|InRange(Float) _output_get -1e+02 1e+02)
        (CallFunction|TurretShoot)))
    (:then_1
      (Transformation|SetActorRotation (Math|Rotator|FindLookatRotation (Transformation|GetActorLocation) (Transformation|GetActorLocation (Game|GetPlayerCharacter 0)))))))

(fn ConstructionScript)