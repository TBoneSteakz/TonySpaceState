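; BP_Boss1 is a boss enemy that takes its stats from a data table and flags its own defeat.
; On the first Tick, after the parent Tick, a DoOnce copies the EnemyTable row at hardcoded index 3 into inherited-style health, movement, targeting, weapon and drop variables, clearing EnemySprite.
; Every Tick also sets Miscom to true once BadmanHealth reaches zero or below.
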(event Collision|EventActorBeginOverlap
  (params (OtherActor :type Actor%20Object%20Reference)))

(event EventTick
  (params (DeltaSeconds :type Float%20%28single-precision%29))
  (|CallParentFunction 0.0)
  (Utilities|FlowControl|Sequence
    (:then_0
      (Utilities|FlowControl|DoOnce false
        (:Completed
          ;[1 1 1] Data Table
          (bind _outrownames (DataTable|GetDataTableRowNames "/Game/SpaceState/Blueprint/Enemies/DataTable/EnemyTable.EnemyTable"))
          (Variables|Default|SetEnemyArray _outrownames)
          (bind _output_get (Variables|Default|SetEnemyIndex 3))
          (bind _returnvalue (Utilities|GetDataTableRow "/Game/SpaceState/Blueprint/Enemies/DataTable/EnemyTable.EnemyTable" (Utilities|Array|Get(acopy) (Variables|Default|GetEnemyArray) _output_get))
            (:then
              (bind _output_get_2 (Variables|Default|SetCurrentEnemy _returnvalue))
              (Variables|Default|SetEnemyName (.Name (Utilities|Struct|BreakEnemyStrut _output_get_2)))
              (Variables|Default|SetEnemySprite 0)
              (Variables|Default|SetBadman_Health (.HP (Utilities|Struct|BreakEnemyStrut _output_get_2)))
              (Variables|Default|SetBadmanSpeed (.EnemySpeed (Utilities|Struct|BreakEnemyStrut _output_get_2)))
              (Variables|Default|SetEnemyScale (.Scale (Utilities|Struct|BreakEnemyStrut _output_get_2)))
              (Variables|Default|SetEnemyCRangeMinusX (.ChaseRMinusX (Utilities|Struct|BreakEnemyStrut _output_get_2)))
              (Variables|Default|SetEnemyCRangePlusX (.ChaseRPlusX (Utilities|Struct|BreakEnemyStrut _output_get_2)))
              (Variables|Default|SetEnemyRangeX (.TargetRangeX (Utilities|Struct|BreakEnemyStrut _output_get_2)))
              (Variables|Default|SetEnemyWeaponSound (.ShotSound (Utilities|Struct|BreakEnemyStrut _output_get_2)))
              (Variables|Default|SetEnemyWeaponScale (.ShotScale (Utilities|Struct|BreakEnemyStrut _output_get_2)))
              (Variables|Default|SetEWeaponRangeSeconds (.ShotRangeSeconds (Utilities|Struct|BreakEnemyStrut _output_get_2)))
              (Variables|Default|SetEWeaponZMin (.ShotZMin (Utilities|Struct|BreakEnemyStrut _output_get_2)))
              (Variables|Default|SetEWeapZmax (.ShotZMax (Utilities|Struct|BreakEnemyStrut _output_get_2)))
              (Variables|Default|SetEWeaponSpeed (.ShotXVelocity (Utilities|Struct|BreakEnemyStrut _output_get_2)))
              (Variables|Default|SetEWeapFireRateSeconds (.FireRateSeconds (Utilities|Struct|BreakEnemyStrut _output_get_2)))
              (Variables|Default|SetEWeaponDamage (.ShotDamage (Utilities|Struct|BreakEnemyStrut _output_get_2)))
              (Variables|Default|SetEItemDrop? (.ItemDrop (Utilities|Struct|BreakEnemyStrut _output_get_2)))
              (Variables|Default|SetEStatic? (.IsStatic (Utilities|Struct|BreakEnemyStrut _output_get_2)))
              (Variables|Default|SetEIsposter (.IsPoster (Utilities|Struct|BreakEnemyStrut _output_get_2)))
              (Variables|Default|SetERotate? (.CanRotate (Utilities|Struct|BreakEnemyStrut _output_get_2)))
              (Variables|Default|SetETwinShot (.TwinShot (Utilities|Struct|BreakEnemyStrut _output_get_2)))
              (Variables|Default|SetEColor (.ShotColor (Utilities|Struct|BreakEnemyStrut _output_get_2)))
              (Variables|Default|SetEnemyRangeXMinus (.TargetRXMinus (Utilities|Struct|BreakEnemyStrut _output_get_2)))
              (Variables|Default|SetEWeight (.EnemyWeight (Utilities|Struct|BreakEnemyStrut _output_get_2))))))))
    (:then_1
      (if (<= (Variables|Default|GetBadman_Health) 0)
        (Variables|Default|Setmiscom true)))))

(fn ConstructionScript
  (|CallParentFunction))