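; BP_BadmanShot is an enemy shot actor that damages the player's BP_Dude when it hits.
; On Hit it plays a ricochet sound once, starts a short delayed self-destroy, and passes EShotDamage to DamageSystem if the other actor is BP_Dude.
; The sound spawns at world origin rather than at the impact point.
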(event Custom|BadHit
  (Utilities|FlowControl|Delay 0.2)
  (Actor|DestroyActor))

(event Custom|BHSound
  (Utilities|FlowControl|DoOnce false
    (:Completed
      (Audio|SpawnSoundatLocation "/Game/SpaceState/Allsounds/Sounds/Ricochet.Ricochet" "0, 0, 0"))))

(event EventBeginPlay)

(event Collision|EventActorBeginOverlap
  (params (OtherActor :type Actor%20Object%20Reference)))

(event EventTick
  (params (DeltaSeconds :type Float%20%28single-precision%29)))

(event Collision|EventHit
  (params (MyComp :type Primitive%20Component%20Object%20Reference) (Other :type Actor%20Object%20Reference) (OtherComp :type Primitive%20Component%20Object%20Reference) (bSelfMoved :type Boolean) (HitLocation :type Vector) (HitNormal :type Vector :default "0, 0, 0") (NormalImpulse :type Vector :default "0, 0, 0") (Hit :type Hit%20Result%20Structure%20%28by%20ref%29))
  (CallFunction|BHSound)
  (CallFunction|BadHit)
  (bind _asbp_dude (Utilities|Casting|CastToBP_Dude Other))
  (Default|DamageSystem _asbp_dude (Variables|Default|GetEShotDamage)))

(fn ConstructionScript)