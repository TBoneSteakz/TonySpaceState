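; Master Paper2D enemy Blueprint that chases and shoots the player, configured from the first row of EnemyTable.
; Tick uses X distance to trigger movement and rate-limited single or twin BP_BadmanShot fire, with optional gun aiming, unless static.
; Damage flashes the sprite; low health halves speed and swaps to damaged flipbooks, while death decrements poster count or drops random items.
; UpdateAnimation selects state flipbooks and plays frame-synced footsteps.
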(event Custom|DMGBadman
  (params (DMGTaken :type Integer))
  (bind _paperflipbook (Variables|Default|GetPaperFlipbook))
  ;[1 1 1] Damage to Enemy
  (Utilities|FlowControl|Sequence
    (:then_0
      (Sprite|SetSpriteColor _paperflipbook (Variables|Default|GetFlash)))
    (:then_1
      (bind _output_get (Variables|Default|SetBadman_Health (- (Variables|Default|GetBadman_Health) DMGTaken)))
      (Utilities|FlowControl|Delay 0.2)
      (Sprite|SetSpriteColor _paperflipbook (Variables|Default|GetBadcolor))
      (CallFunction|UpdateAnimation)
      (if (<= _output_get 0)
        (Actor|DestroyActor)
        ;[1 1 1] poster quest
        (if (Variables|Default|GetEIsposter)
          (bind _asbp_dude (Utilities|Casting|CastToBP_Dude (Game|GetPlayerCharacter 0)))
          (Variables|/Game/SpaceState/Blueprint/BP_Dude/BP_Dude.BP_Dude_C|Setpostersleft _asbp_dude (- (Variables|/Game/SpaceState/Blueprint/BP_Dude/BP_Dude.BP_Dude_C|Getpostersleft _asbp_dude) 1))
          (else
            ;[1 1 1] Item Drops
            (if (Variables|Default|GetEItemDrop?)
              (Game|SpawnActorfromClass (Utilities|Array|Get(acopy) (Variables|Default|GetItemDrop) (Math|Random|RandomIntegerinRange (Variables|Default|GetItemIndexMin) (Variables|Default|GetItemIndexMax))) (Math|Conversions|ToTransform(Vector) (Transformation|GetActorLocation)) "Undefined" 0 0))))))))

(event Custom|ShootAni
  ;[1 1 1] ShootingAnimation
  (Utilities|FlowControl|Delay 0.5)
  (bind _output_get (Variables|Default|SetFrame (Class|PaperFlipbookComponent|GetPlaybackPositioninFrames (Variables|Default|GetPaperFlipbook))))
  (Variables|Default|SetStates "NewEnumerator3"))

(event Custom|UpdateAnimation
  (bind _returnvalue (Transformation|GetActorLocation))
  (bind _paperflipbook (Variables|Default|GetPaperFlipbook))
  (bind _paperflipbook_2 (Variables|Default|GetPaperFlipbook))
  (bind _paperflipbook_3 (Variables|Default|GetPaperFlipbook))
  (bind _returnvalue_2 (Class|PaperFlipbookComponent|GetPlaybackPositioninFrames _paperflipbook))
  (bind _returnvalue_3 (Class|PaperFlipbookComponent|GetPlaybackPositioninFrames _paperflipbook_3))
  ;[1 1 1] Animation States
  (switch Utilities|FlowControl|Switch|SwitchonEnemy_States (Variables|Default|GetStates)
    (:NewEnumerator0
      (if (<= (Variables|Default|GetBadman_Health) (Variables|Default|GetBadDMGHealth))
        (Sprite|SetFlipbook _paperflipbook_2 (Variables|Default|GetDStance))
        (else
          (Sprite|SetFlipbook _paperflipbook_2 (Variables|Default|GetStanceFlip)))))
    (:NewEnumerator1
      (if (<= (Variables|Default|GetBadman_Health) (Variables|Default|GetBadDMGHealth))
        (Sprite|SetFlipbook _paperflipbook_2 (Variables|Default|GetDRun))
        (else
          (Sprite|SetFlipbook _paperflipbook_2 (Variables|Default|GetRunFlip))))
      ;[1 1 1] Footsteps
      (Utilities|FlowControl|Sequence
        (:then_0
          (if (== _returnvalue_2 0)
            (Utilities|FlowControl|DoOnce false :!label _label
              (:Completed
                (if (== (Class|PaperFlipbookComponent|GetFlipbook _paperflipbook) "/Game/SpaceState/Sprites/Bad/A_BadRun.A_BadRun") :!label _label_2
                  (Audio|PlaySoundatLocation "/Game/SpaceState/Allsounds/Sounds/metalfootstep_Cue.metalfootstep_Cue" _returnvalue)
                  (elif (== (Class|PaperFlipbookComponent|GetFlipbook _paperflipbook) "/Game/SpaceState/Sprites/Bad/A_BadDRun.A_BadDRun")
                    (Audio|PlaySoundatLocation "/Game/SpaceState/Allsounds/Sounds/metalfootstep_Cue.metalfootstep_Cue" _returnvalue)))))))
        (:then_1
          (if (not (== _returnvalue_2 0))
            (goto _label Reset)))
        (:then_2
          (if (== _returnvalue_2 6)
            (Utilities|FlowControl|DoOnce false :!label _label_3
              (:Completed
                (goto _label_2)))))
        (:then_3
          (if (not (== _returnvalue_2 6))
            (goto _label_3 Reset)))))
    (:NewEnumerator2
      (if (<= (Variables|Default|GetBadman_Health) (Variables|Default|GetBadDMGHealth))
        (Sprite|SetFlipbook _paperflipbook_2 (Variables|Default|GetDShoot))
        (else
          (Sprite|SetFlipbook _paperflipbook_2 (Variables|Default|GetShootFlip))))
      ;[1 1 1] ShootingAnimation
      (Class|PaperFlipbookComponent|SetPlaybackPositioninFrames _paperflipbook_2 (stale Custom|ShootAni _output_get) false)
      ;[1 1 1] Footsteps
      (Utilities|FlowControl|Sequence
        (:then_0
          (if (== _returnvalue_3 0)
            (Utilities|FlowControl|DoOnce false :!label _label_4
              (:Completed
                (if (== (Class|PaperFlipbookComponent|GetFlipbook _paperflipbook_3) "/Game/SpaceState/Sprites/Bad/A_BadRun.A_BadRun") :!label _label_5
                  (Audio|PlaySoundatLocation "/Game/SpaceState/Allsounds/Sounds/metalfootstep_Cue.metalfootstep_Cue" (Transformation|GetActorLocation)))))))
        (:then_1
          (if (not (== _returnvalue_3 0))
            (goto _label_4 Reset)))
        (:then_2
          (if (== _returnvalue_3 6)
            (Utilities|FlowControl|DoOnce false :!label _label_6
              (:Completed
                (goto _label_5)))))
        (:then_3
          (if (not (== _returnvalue_3 6))
            (goto _label_6 Reset)))))
    (:NewEnumerator3
      (if (<= (Variables|Default|GetBadman_Health) (Variables|Default|GetBadDMGHealth))
        (Sprite|SetFlipbook _paperflipbook_2 (Variables|Default|GetDRunShoot))
        (else
          (Sprite|SetFlipbook _paperflipbook_2 (Variables|Default|GetRunShootFlip)))))))

(event Custom|Badman_shoot
  (bind _ecolor (Variables|Default|GetEColor))
  (bind _arrow (Variables|Default|GetArrow))
  (bind _returnvalue (Transformation|GetWorldTransform _arrow))
  (Utilities|FlowControl|DoOnce false :!label _label
    (:Completed
      ;[1 1 1] Shooting
      (Utilities|FlowControl|Sequence
        (:then_0
          (bind _returnvalue_2 (Game|SpawnActorfromClass "/Game/SpaceState/Blueprint/Enemies/DataTable/BP_BadmanShot.BP_BadmanShot_C" _returnvalue "Undefined" 0 0))
          (CallFunction|ShootAni)
          (Audio|PlaySoundatLocation (Variables|Default|GetEnemyWeaponSound) (Transformation|GetActorLocation _returnvalue_2))
          (Transformation|SetRelativeScale3D (Variables|/Game/SpaceState/Blueprint/Enemies/DataTable/BP_BadmanShot.BP_BadmanShot_C|GetPaperFlipbook _returnvalue_2) (Variables|Default|GetEnemyWeaponScale))
          (Rendering|Material|SetVectorParameterValueonMaterials (Variables|/Game/SpaceState/Blueprint/Enemies/DataTable/BP_BadmanShot.BP_BadmanShot_C|GetPaperFlipbook _returnvalue_2) "Colour" (Math|Conversions|ToVector(LinearColor) _ecolor))
          (Game|Components|ProjectileMovement|SetVelocityinLocalSpace (Variables|/Game/SpaceState/Blueprint/Enemies/DataTable/BP_BadmanShot.BP_BadmanShot_C|GetProjectileMovement _returnvalue_2) (Math|Vector|MakeVector (Variables|Default|GetEWeaponSpeed) 0.0 (Math|Random|RandomFloatinRange (Variables|Default|GetEWeaponZMin) (Variables|Default|GetEWeapZmax))))
          (Variables|/Game/SpaceState/Blueprint/Enemies/DataTable/BP_BadmanShot.BP_BadmanShot_C|SetEShotDamage _returnvalue_2 (Variables|Default|GetEWeaponDamage))
          (Actor|SetLifeSpan _returnvalue_2 (Variables|Default|GetEWeaponRangeSeconds))
          (Utilities|FlowControl|Delay (Variables|Default|GetEWeapFireRateSeconds) :!label _label_2)
          (goto _label Reset))
        (:then_1
          ;[1 1 1] Twin Shot
          (if (Variables|Default|GetETwinShot)
            (Audio|PlaySoundatLocation (Variables|Default|GetEnemyWeaponSound) (Transformation|GetWorldLocation (Variables|Default|Getgun)))
            (bind _returnvalue_3 (Game|SpawnActorfromClass "/Game/SpaceState/Blueprint/Enemies/DataTable/BP_BadmanShot.BP_BadmanShot_C" _returnvalue "Undefined" 0 0))
            (Transformation|SetActorRelativeLocation _returnvalue_3 (+ (Transformation|GetActorLocation _returnvalue_3) "0.000000,0.000000,20.000000"))
            (Transformation|SetRelativeScale3D (Variables|/Game/SpaceState/Blueprint/Enemies/DataTable/BP_BadmanShot.BP_BadmanShot_C|GetPaperFlipbook _returnvalue_3) (Variables|Default|GetEnemyWeaponScale))
            (Rendering|Material|SetVectorParameterValueonMaterials (Variables|/Game/SpaceState/Blueprint/Enemies/DataTable/BP_BadmanShot.BP_BadmanShot_C|GetPaperFlipbook _returnvalue_3) "Colour" (Math|Conversions|ToVector(LinearColor) _ecolor))
            (Game|Components|ProjectileMovement|SetVelocityinLocalSpace (Variables|/Game/SpaceState/Blueprint/Enemies/DataTable/BP_BadmanShot.BP_BadmanShot_C|GetProjectileMovement _returnvalue_3) (Math|Vector|MakeVector (Variables|Default|GetEWeaponSpeed) 0.0 (Math|Random|RandomFloatinRange (Variables|Default|GetEWeaponZMin) (Variables|Default|GetEWeapZmax))))
            (Variables|/Game/SpaceState/Blueprint/Enemies/DataTable/BP_BadmanShot.BP_BadmanShot_C|SetEShotDamage _returnvalue_3 (Variables|Default|GetEWeaponDamage))
            (Actor|SetLifeSpan _returnvalue_3 (Variables|Default|GetEWeaponRangeSeconds))
            (goto _label_2)))))))

(event Custom|InitEnemy
  ;[1 1 1] Data Table
  (bind _outrownames (DataTable|GetDataTableRowNames "/Game/SpaceState/Blueprint/Enemies/DataTable/EnemyTable.EnemyTable"))
  (Variables|Default|SetEnemyArray _outrownames)
  (bind _output_get (Variables|Default|SetEnemyIndex 0))
  (bind _returnvalue (Utilities|GetDataTableRow "/Game/SpaceState/Blueprint/Enemies/DataTable/EnemyTable.EnemyTable" (Utilities|Array|Get(acopy) (Variables|Default|GetEnemyArray) _output_get))
    (:then
      (bind _output_get_2 (Variables|Default|SetCurrentEnemy _returnvalue))
      (Variables|Default|SetEnemyName (.Name (Utilities|Struct|BreakEnemyStrut _output_get_2)))
      (Variables|Default|SetBadman_Health (.HP (Utilities|Struct|BreakEnemyStrut _output_get_2)))
      (Variables|Default|SetBadmanSpeed (.EnemySpeed (Utilities|Struct|BreakEnemyStrut _output_get_2)))
      (Variables|Default|SetEnemyScale (.Scale (Utilities|Struct|BreakEnemyStrut _output_get_2)))
      (Variables|Default|SetEnemyCRangeMinusX (.ChaseRMinusX (Utilities|Struct|BreakEnemyStrut _output_get_2)))
      (Variables|Default|SetEnemyCRangePlusX (.ChaseRPlusX (Utilities|Struct|BreakEnemyStrut _output_get_2)))
      (Variables|Default|SetEnemyRangeX (.TargetRangeX (Utilities|Struct|BreakEnemyStrut _output_get_2)))
      (Variables|Default|SetEnemyWeaponSound (.ShotSound (Utilities|Struct|BreakEnemyStrut _output_get_2)))
      (Variables|Default|SetEnemyWeaponScale (.ShotScale (Utilities|Struct|BreakEnemyStrut _output_get_2)))
      (Variables|Default|SetEWeaponRangeSeconds (.ShotRangeSeconds (Utilities|Struct|BreakEnemyStrut _output_get_2)))
      (Variables|Default|SetEWeaponZMin (.ShotZMin (Utilities|Struct|BreakEnemyStrut _output_get_2)))
      (Variables|Default|SetEWeapZmax (.ShotZMax (Utilities|Struct|BreakEnemyStrut _output_get_2)))
      (Variables|Default|SetEWeaponSpeed (.ShotXVelocity (Utilities|Struct|BreakEnemyStrut _output_get_2)))
      (Variables|Default|SetEWeapFireRateSeconds (.FireRateSeconds (Utilities|Struct|BreakEnemyStrut _output_get_2)))
      (Variables|Default|SetEWeaponDamage (.ShotDamage (Utilities|Struct|BreakEnemyStrut _output_get_2)))
      (Variables|Default|SetEItemDrop? (.ItemDrop (Utilities|Struct|BreakEnemyStrut _output_get_2)))
      (Variables|Default|SetEStatic? (.IsStatic (Utilities|Struct|BreakEnemyStrut _output_get_2)))
      (Variables|Default|SetEIsposter (.IsPoster (Utilities|Struct|BreakEnemyStrut _output_get_2)))
      (Variables|Default|SetERotate? (.CanRotate (Utilities|Struct|BreakEnemyStrut _output_get_2)))
      (Variables|Default|SetETwinShot (.TwinShot (Utilities|Struct|BreakEnemyStrut _output_get_2)))
      (Variables|Default|SetEColor (.ShotColor (Utilities|Struct|BreakEnemyStrut _output_get_2)))
      (Variables|Default|SetEnemyRangeXMinus (.TargetRXMinus (Utilities|Struct|BreakEnemyStrut _output_get_2)))
      (Variables|Default|SetEWeight (.EnemyWeight (Utilities|Struct|BreakEnemyStrut _output_get_2)))
      (Variables|Default|SetItemIndexMin (.IndexMin (Utilities|Struct|BreakEnemyStrut _output_get_2)))
      (Variables|Default|SetItemIndexMax (.IndexMax (Utilities|Struct|BreakEnemyStrut _output_get_2)))
      (Variables|Default|SetStanceFlip (.StanceFlip (Utilities|Struct|BreakEnemyStrut _output_get_2)))
      (Variables|Default|SetRunFlip (.RunFlip (Utilities|Struct|BreakEnemyStrut _output_get_2)))
      (Variables|Default|SetShootFlip (.ShootFlip (Utilities|Struct|BreakEnemyStrut _output_get_2)))
      (Variables|Default|SetRunShootFlip (.RunShootFlip (Utilities|Struct|BreakEnemyStrut _output_get_2)))
      (Variables|Default|SetDStance (.DStance (Utilities|Struct|BreakEnemyStrut _output_get_2)))
      (Variables|Default|SetDRun (.DRun (Utilities|Struct|BreakEnemyStrut _output_get_2)))
      (Variables|Default|SetDShoot (.DShoot (Utilities|Struct|BreakEnemyStrut _output_get_2)))
      (Variables|Default|SetDRunShoot (.DRunShoot (Utilities|Struct|BreakEnemyStrut _output_get_2)))
      (Variables|Default|SetBadDMGHealth (.BDMGed (Utilities|Struct|BreakEnemyStrut _output_get_2)))
      (Variables|Default|SetBadcolor (.Badcolor (Utilities|Struct|BreakEnemyStrut _output_get_2))))))

(event EventBeginPlay
  (bind _paperflipbook (Variables|Default|GetPaperFlipbook))
  ;[1 1 1] Initialize
  (CallFunction|InitEnemy)
  (Class|PrimitiveComponent|SetMassOverrideinKg (Variables|Default|GetCapsule1) "None" (Variables|Default|GetEWeight) true)
  (Utilities|FlowControl|Delay 0.2)
  (Sprite|SetFlipbook _paperflipbook (Variables|Default|GetStanceFlip))
  (Transformation|SetRelativeScale3D (Variables|Default|GetCapsule1) (Variables|Default|GetEnemyScale))
  (Sprite|SetSpriteColor _paperflipbook (Variables|Default|GetBadcolor)))

(event EventTick
  (params (DeltaSeconds :type Float%20%28single-precision%29))
  (bind _returnvalue (Transformation|GetActorLocation))
  ;[1 1 1] Move and Target
  (if (not (Variables|Default|GetEStatic?))
    (Utilities|FlowControl|Sequence
      (:then_0
        (bind _output_get (Variables|Default|Setdistance (- (.x (Transformation|GetWorldLocation (Variables|Default|GetPaperFlipbook))) (.x (Transformation|GetActorLocation (Game|GetPlayerCharacter 0))))))
        (if (Math|Float|InRange(Float) _output_get (Variables|Default|GetEnemyRangeXMinus) (Variables|Default|GetEnemyRangeX))
          (CallFunction|BadmanShoot)))
      (:then_1
        (Transformation|SetRelativeRotation (Variables|Default|GetPaperFlipbook) (Math|Rotator|MakeRotator 0.0 0.0 (.yaw (Math|Rotator|FindLookatRotation (Transformation|GetActorLocation) (Transformation|GetActorLocation (Game|GetPlayerCharacter 0))))) false false))
      (:then_2
        (Variables|Default|SetActorX (.x _returnvalue)))
      (:then_3
        (Variables|Default|SetActorY (.y _returnvalue)))
      (:then_4
        (Variables|Default|SetActorZ (.z _returnvalue)))
      (:then_5
        (if (Math|Float|InRange(Float) (Variables|Default|Getdistance) 0.0 (Variables|Default|GetEnemyCRangePlusX))
          (Utilities|FlowControl|Delay 0.05)
          (Transformation|SetActorLocation (Math|Vector|MakeVector (- (Variables|Default|GetActorX) (Variables|Default|GetBadmanSpeed)) (Variables|Default|GetActorY) (Variables|Default|GetActorZ)) false false)))
      (:then_6
        (if (Math|Float|InRange(Float) (Variables|Default|Getdistance) (Variables|Default|GetEnemyCRangeMinusX) 0.0)
          (Utilities|FlowControl|Delay 0.05)
          (Transformation|SetActorLocation (Math|Vector|MakeVector (+ (Variables|Default|GetActorX) (Variables|Default|GetBadmanSpeed)) (Variables|Default|GetActorY) (Variables|Default|GetActorZ)) false false)))
      (:then_7
        ;[1 1 1] Rotate Fire
        (if (Variables|Default|GetERotate?)
          (Transformation|SetRelativeRotation (Variables|Default|Getgun) (Math|Rotator|FindLookatRotation (Transformation|GetActorLocation) (Transformation|GetActorLocation (Game|GetPlayerCharacter 0))) false false)))
      (:then_8
        (Class|PrimitiveComponent|SetMassOverrideinKg (Variables|Default|GetCapsule1) "None" (Variables|Default|GetEWeight) true))
      (:then_9
        (if (Math|Float|InRange(Float) (Variables|Default|Getdistance) (Variables|Default|GetEnemyCRangeMinusX) (Variables|Default|GetEnemyCRangePlusX))
          (Variables|Default|SetStates "NewEnumerator1")
          (CallFunction|UpdateAnimation)))
      (:then_10
        (if (<= (Variables|Default|GetBadman_Health) (Variables|Default|GetBadDMGHealth))
          (Utilities|FlowControl|DoOnce false
            (:Completed
              (Variables|Default|SetBadmanSpeed (/ (Variables|Default|GetBadmanSpeed) 2.0)))))))))

(fn ConstructionScript)