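; BP_Badman is a Paper2D enemy that chases and shoots the player, with stats, sprite and weapon loaded from an EnemyTable row at fixed index 2.
; Non-static enemies face the player on Tick, step along X within chase ranges and trigger shooting within target range.
; Shooting spawns rate-limited, tinted BP_BadmanShot projectiles with random vertical velocity and optional twin shot.
; On death, posters decrement BP_Dude's remaining count; others may drop random items.
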(event Custom|DMGBadman
  (params (DMGTaken :type Integer))
  ;[1 1 1] Damage to badman
  (bind _output_get (Variables|Default|SetBadman_Health (- (Variables|Default|GetBadman_Health) DMGTaken)))
  (if (<= _output_get 0)
    (Utilities|FlowControl|Delay 0.2)
    (Actor|DestroyActor)
    (if (Variables|Default|GetEIsposter)
      (bind _asbp_dude (Utilities|Casting|CastToBP_Dude (Game|GetPlayerCharacter 0)))
      (Variables|/Game/SpaceState/Blueprint/BP_Dude.BP_Dude_C|Setpostersleft _asbp_dude (- (Variables|/Game/SpaceState/Blueprint/BP_Dude.BP_Dude_C|Getpostersleft _asbp_dude) 1))
      (elif (Variables|Default|GetEItemDrop?)
        (Game|SpawnActorfromClass (Utilities|Array|Get(acopy) (Variables|Default|GetItemDrop) (Math|Random|RandomIntegerinRange 0 2)) (Math|Conversions|ToTransform(Vector) (Transformation|GetActorLocation)) "Undefined" 0 0)))))

(event Custom|Badman_shoot
  (bind _ecolor (Variables|Default|GetEColor))
  (bind _arrow (Variables|Default|GetArrow))
  (bind _returnvalue (Transformation|GetWorldTransform _arrow))
  ;[1 1 1] badman shooting
  (Utilities|FlowControl|DoOnce false :!label _label
    (:Completed
      (Utilities|FlowControl|Sequence
        (:then_0
          (Audio|PlaySoundatLocation (Variables|Default|GetEnemyWeaponSound) "0, 0, 0")
          (bind _returnvalue_2 (Game|SpawnActorfromClass "/Game/SpaceState/Blueprint/Enemies/BP_BadmanShot.BP_BadmanShot_C" _returnvalue "Undefined" 0 0))
          (Transformation|SetRelativeScale3D (Variables|/Game/SpaceState/Blueprint/Enemies/BP_BadmanShot.BP_BadmanShot_C|GetPaperFlipbook _returnvalue_2) (Variables|Default|GetEnemyWeaponScale))
          (Rendering|Material|SetVectorParameterValueonMaterials (Variables|/Game/SpaceState/Blueprint/Enemies/BP_BadmanShot.BP_BadmanShot_C|GetPaperFlipbook _returnvalue_2) "Colour" (Math|Conversions|ToVector(LinearColor) _ecolor))
          (Game|Components|ProjectileMovement|SetVelocityinLocalSpace (Variables|/Game/SpaceState/Blueprint/Enemies/BP_BadmanShot.BP_BadmanShot_C|GetProjectileMovement _returnvalue_2) (Math|Vector|MakeVector (Variables|Default|GetEWeaponSpeed) 0.0 (Math|Random|RandomFloatinRange (Variables|Default|GetEWeaponZMin) (Variables|Default|GetEWeapZmax))))
          (Variables|/Game/SpaceState/Blueprint/Enemies/BP_BadmanShot.BP_BadmanShot_C|SetEShotDamage _returnvalue_2 (Variables|Default|GetEWeaponDamage))
          (Actor|SetLifeSpan _returnvalue_2 (Variables|Default|GetEWeaponRangeSeconds))
          (Utilities|FlowControl|Delay (Variables|Default|GetEWeapFireRateSeconds) :!label _label_2)
          (goto _label Reset))
        (:then_1
          (if (Variables|Default|GetETwinShot)
            (Audio|PlaySoundatLocation (Variables|Default|GetEnemyWeaponSound) "0, 0, 0")
            (bind _returnvalue_3 (Game|SpawnActorfromClass "/Game/SpaceState/Blueprint/Enemies/BP_BadmanShot.BP_BadmanShot_C" _returnvalue "Undefined" 0 0))
            (Transformation|SetActorRelativeLocation _returnvalue_3 (+ (Transformation|GetActorLocation _returnvalue_3) "0.000000,0.000000,20.000000"))
            (Transformation|SetRelativeScale3D (Variables|/Game/SpaceState/Blueprint/Enemies/BP_BadmanShot.BP_BadmanShot_C|GetPaperFlipbook _returnvalue_3) (Variables|Default|GetEnemyWeaponScale))
            (Rendering|Material|SetVectorParameterValueonMaterials (Variables|/Game/SpaceState/Blueprint/Enemies/BP_BadmanShot.BP_BadmanShot_C|GetPaperFlipbook _returnvalue_3) "Colour" (Math|Conversions|ToVector(LinearColor) _ecolor))
            (Game|Components|ProjectileMovement|SetVelocityinLocalSpace (Variables|/Game/SpaceState/Blueprint/Enemies/BP_BadmanShot.BP_BadmanShot_C|GetProjectileMovement _returnvalue_3) (Math|Vector|MakeVector (Variables|Default|GetEWeaponSpeed) 0.0 (Math|Random|RandomFloatinRange (Variables|Default|GetEWeaponZMin) (Variables|Default|GetEWeapZmax))))
            (Variables|/Game/SpaceState/Blueprint/Enemies/BP_BadmanShot.BP_BadmanShot_C|SetEShotDamage _returnvalue_3 (Variables|Default|GetEWeaponDamage))
            (Actor|SetLifeSpan _returnvalue_3 (Variables|Default|GetEWeaponRangeSeconds))
            (goto _label_2)))))))

(event Custom|InitEnemy
  (bind _outrownames (DataTable|GetDataTableRowNames "/Game/SpaceState/Blueprint/Enemies/EnemyTable.EnemyTable"))
  (Variables|Default|SetEnemyArray _outrownames)
  (bind _output_get (Variables|Default|SetEnemyIndex 2))
  (bind _returnvalue (Utilities|GetDataTableRow "/Game/SpaceState/Blueprint/Enemies/EnemyTable.EnemyTable" (Utilities|Array|Get(acopy) (Variables|Default|GetEnemyArray) _output_get))
    (:then
      (bind _output_get_2 (Variables|Default|SetCurrentEnemy _returnvalue))
      (Variables|Default|SetEnemyName (.EName (Utilities|Struct|BreakEnemyStrut _output_get_2)))
      (Variables|Default|SetEnemySprite (.ESprite (Utilities|Struct|BreakEnemyStrut _output_get_2)))
      (Variables|Default|SetBadman_Health (.EHP (Utilities|Struct|BreakEnemyStrut _output_get_2)))
      (Variables|Default|SetBadmanSpeed (.ESpeed (Utilities|Struct|BreakEnemyStrut _output_get_2)))
      (Variables|Default|SetEnemyScale (.EScale (Utilities|Struct|BreakEnemyStrut _output_get_2)))
      (Variables|Default|SetEnemyCRangeMinusX (.EChaseRMinusX (Utilities|Struct|BreakEnemyStrut _output_get_2)))
      (Variables|Default|SetEnemyCRangePlusX (.EChaseRPlusX (Utilities|Struct|BreakEnemyStrut _output_get_2)))
      (Variables|Default|SetEnemyRangeX (.ETargetRX (Utilities|Struct|BreakEnemyStrut _output_get_2)))
      (Variables|Default|SetEnemyWeaponSound (.EWeaponSound (Utilities|Struct|BreakEnemyStrut _output_get_2)))
      (Variables|Default|SetEnemyWeaponScale (.EWeaponScale (Utilities|Struct|BreakEnemyStrut _output_get_2)))
      (Variables|Default|SetEWeaponRangeSeconds (.EWeaponRangeSeconds (Utilities|Struct|BreakEnemyStrut _output_get_2)))
      (Variables|Default|SetEWeaponZMin (.EWeapZMin (Utilities|Struct|BreakEnemyStrut _output_get_2)))
      (Variables|Default|SetEWeapZmax (.EWeapZMax (Utilities|Struct|BreakEnemyStrut _output_get_2)))
      (Variables|Default|SetEWeaponSpeed (.EWeaponXVelocity (Utilities|Struct|BreakEnemyStrut _output_get_2)))
      (Variables|Default|SetEWeapFireRateSeconds (.EFireRateSeconds (Utilities|Struct|BreakEnemyStrut _output_get_2)))
      (Variables|Default|SetEWeaponDamage (.EDamage (Utilities|Struct|BreakEnemyStrut _output_get_2)))
      (Variables|Default|SetEItemDrop? (.EItemDrop? (Utilities|Struct|BreakEnemyStrut _output_get_2)))
      (Variables|Default|SetEStatic? (.EIsStatic? (Utilities|Struct|BreakEnemyStrut _output_get_2)))
      (Variables|Default|SetEIsposter (.IsPoster? (Utilities|Struct|BreakEnemyStrut _output_get_2)))
      (Variables|Default|SetERotate? (.CanRotate (Utilities|Struct|BreakEnemyStrut _output_get_2)))
      (Variables|Default|SetETwinShot (.TwinShot (Utilities|Struct|BreakEnemyStrut _output_get_2)))
      (Variables|Default|SetEColor (.EColor (Utilities|Struct|BreakEnemyStrut _output_get_2))))))

(event Collision|EventActorBeginOverlap
  (params (OtherActor :type Actor%20Object%20Reference)))

(event EventBeginPlay
  (CallFunction|InitEnemy)
  (Utilities|FlowControl|Delay 0.2)
  (Rendering|Components|Sprite|SetSprite (Variables|Default|GetPaperSprite) (Variables|Default|GetEnemySprite))
  (Transformation|SetRelativeScale3D (Variables|Default|GetPaperSprite) (Variables|Default|GetEnemyScale)))

(event EventTick
  (params (DeltaSeconds :type Float%20%28single-precision%29))
  (bind _returnvalue (Transformation|GetActorLocation))
  (bind _badmanspeed (Variables|Default|GetBadmanSpeed))
  ;[1 1 1] Move and Target
  (if (not (Variables|Default|GetEStatic?))
    (Utilities|FlowControl|Sequence
      (:then_0
        (bind _output_get (Variables|Default|Setdistance (- (.x (Transformation|GetWorldLocation (Variables|Default|GetPaperSprite))) (.x (Transformation|GetActorLocation (Game|GetPlayerCharacter 0))))))
        (if (<= _output_get (Variables|Default|GetEnemyRangeX))
          (CallFunction|BadmanShoot)))
      (:then_1
        (Transformation|SetActorRotation (Math|Rotator|MakeRotator 0.0 0.0 (.yaw (Math|Rotator|FindLookatRotation (Transformation|GetActorLocation) (Transformation|GetActorLocation (Game|GetPlayerCharacter 0)))))))
      (:then_2
        (Variables|Default|SetActorX (.x _returnvalue)))
      (:then_3
        (Variables|Default|SetActorY (.y _returnvalue)))
      (:then_4
        (Variables|Default|SetActorZ (.z _returnvalue)))
      (:then_5
        (if (Math|Float|InRange(Float) (Variables|Default|Getdistance) 0.0 (Variables|Default|GetEnemyCRangePlusX))
          (Utilities|FlowControl|Delay 0.05)
          (Transformation|SetActorLocation (Math|Vector|MakeVector (- (Variables|Default|GetActorX) _badmanspeed) (Variables|Default|GetActorY) (Variables|Default|GetActorZ)) false false)))
      (:then_6
        (if (Math|Float|InRange(Float) (Variables|Default|Getdistance) (Variables|Default|GetEnemyCRangeMinusX) 0.0)
          (Utilities|FlowControl|Delay 0.05)
          (Transformation|SetActorLocation (Math|Vector|MakeVector (+ (Variables|Default|GetActorX) _badmanspeed) (Variables|Default|GetActorY) (Variables|Default|GetActorZ)) false false)))
      (:then_7
        (if (Variables|Default|GetERotate?)
          (Transformation|SetActorRotation (Math|Rotator|FindLookatRotation (Transformation|GetActorLocation) (Transformation|GetActorLocation (Game|GetPlayerCharacter 0)))))))))

(fn ConstructionScript)