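; BP_bombtimer is an overlap-triggered bomb countdown that loads MainMenu when its 40-second timer runs out.
; The first overlap stops the player BP_Dude's M1 audio, starts its own audio component partway in, and caches the first BP_Bocc2.
; A self-looping short Delay refreshes the Timeelap text with remaining time.
; Tick polls that BP_Bocc2's Miscom flag, pausing the timer and stopping the audio once it is set.
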(event Custom|CustomEvent_0
  (Game|OpenLevel(byName) "MainMenu"))

(event EventBeginPlay)

(event Collision|EventActorBeginOverlap
  (params (OtherActor :type Actor%20Object%20Reference))
  (Utilities|FlowControl|Sequence
    (:then_0
      (Utilities|FlowControl|DoOnce false
        (:Completed
          (bind _asbp_dude (Utilities|Casting|CastToBP_Dude (Game|GetPlayerCharacter 0)))
          (Audio|Components|Audio|Stop (Variables|/Game/SpaceState/Blueprint/BP_Dude.BP_Dude_C|GetM1 _asbp_dude))
          (bind _returnvalue (AddComponent|AddAudioComponent false))
          (Audio|Components|Audio|Play _returnvalue 4.7e+02))))
    (:then_1
      (Utilities|FlowControl|DoOnce false
        (:Completed
          (bind _returnvalue_2 (Utilities|Time|SetTimerbyEvent (delegate Custom|CustomEvent_0) 4e+01))
          (bind _outactors (Actor|GetAllActorsOfClass "/Game/SpaceState/Blueprint/Enemies/BP_Bocc2.BP_Bocc2_C"))
          (Variables|Default|SetNewVar_0 _outactors)
          (bind _asbp_bocc_2 (Utilities|Casting|CastToBP_Bocc2 (Utilities|Array|Get(acopy) (Variables|Default|GetNewVar_0))))
          (Utilities|FlowControl|Delay 0.01 :!label _label)
          (Variables|Default|Settimeelap (Utilities|Text|ToText(Float) (Utilities|Time|GetTimerRemainingTimebyHandle _returnvalue_2) "HalfToEven" true 1 324 0 2))
          (goto _label))))))

(event EventTick
  (params (DeltaSeconds :type Float%20%28single-precision%29))
  (if (Variables|/Game/SpaceState/Blueprint/Enemies/BP_Bocc2.BP_Bocc2_C|Getmiscom (stale Collision|EventActorBeginOverlap _asbp_bocc_2))
    (Utilities|FlowControl|DoOnce false
      (:Completed
        (Utilities|Time|PauseTimerbyHandle (stale Collision|EventActorBeginOverlap _returnvalue_2))
        (Audio|Components|Audio|Stop (stale Collision|EventActorBeginOverlap _returnvalue))))))

(fn ConstructionScript)