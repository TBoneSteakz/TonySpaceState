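; BP_Chattyman is an NPC vendor that sells health, ammo and a shotgun to BP_Dude for credits through dialogue.
; Overlap opens Widget_Dialogue with a mouse cursor, and leaving or Answer4 closes it.
; Answer events set AnswerInt for a shared branch chain keyed on menu state UpdateArray, which selects button texts, checks credits and limits, and updates the player.
; A first-contact branch sets MainQuest, and a railgun purchase branch is unconnected.
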(event Custom|Leaving
  ;[1 1 1] Start/End Encounter, Enable/disable input
  (Input|DisableInput (Game|GetPlayerController 0))
  (Rendering|Components|TextRender|SetText (Variables|Components|GetTextRender) (Variables|Default|GetR_Leaving))
  (if (== (Variables|/Game/SpaceState/Blueprint/BP_Dude/BP_Dude.BP_Dude_C|GetMainQuest (stale Collision|EventActorBeginOverlap _asbp_dude)) 5)
    (Variables|Default|SetUpdateArray 0)
    (else
      (Variables|Default|SetUpdateArray 0)))
  (Widget|RemovefromParent (stale Collision|EventActorBeginOverlap _output_get))
  (bind _asplayer_controller (Utilities|Casting|CastToPlayerController (Game|GetPlayerController 0)))
  (Variables|/Script/Engine.PlayerController|SetbShowMouseCursor _asplayer_controller false))

(event Custom|Answer1
  (bind _returnvalue (Game|GetPlayerCharacter 0))
  (bind _answers (Variables|Default|GetAnswers))
  (bind _answers_2 (Variables|Default|GetAnswers))
  (bind _answers_3 (Variables|Default|GetAnswers))
  (bind _answers_4 (Variables|Default|GetAnswers))
  (bind _answers_5 (Variables|Default|GetAnswers))
  (bind _answers_6 (Variables|Default|GetAnswers))
  (bind _nhp1 (Variables|Default|GetNhp1))
  (bind _answers_7 (Variables|Default|GetAnswers))
  ;[1 1 1] Input
  (Variables|Default|SetAnswerInt 0)
  ;[1 1 1] FirstTime
  (if (== (Variables|Default|GetUpdateArray) 5)
    (if (== (Variables|Default|GetAnswerInt) 0)
      (Variables|/Game/SpaceState/Blueprint/Widget_Dialogue.Widget_Dialogue_C|SetNPCDia _answers (Variables|Default|Getnext))
      (bind _asbp_dude (Utilities|Casting|CastToBP_Dude (Game|GetPlayerCharacter 0)))
      (Variables|/Game/SpaceState/Blueprint/BP_Dude/BP_Dude.BP_Dude_C|SetMainQuest _asbp_dude 2)
      (Variables|Default|SetUpdateArray 6)
      (Variables|Default|SetButtonText (Utilities|Select :Index (Variables|Default|GetUpdateArray) :Option%200 (Utilities|Array|MakeArray (Variables|Default|GetA1) (Variables|Default|GetA2) (Variables|Default|GetA3)) :Option%201 (Utilities|Array|MakeArray (Variables|Default|Getphp1) (Variables|Default|Getphp2) (Variables|Default|Getphp3)) :Option%202 (Utilities|Array|MakeArray (Variables|Default|GetPQ2a) (Variables|Default|GetPQ2b) (Variables|Default|Getpmore)) :Option%203 (Utilities|Array|MakeArray (Variables|Default|GetPWeap1) (Variables|Default|GetPweap2) (Variables|Default|GetPweap3)) :Option%204 (Utilities|Array|MakeArray (Variables|Default|GetPflamerammo) (Variables|Default|GetPpowercells) (Variables|Default|Getpmore2)) :Option%205 (Utilities|Array|MakeArray (Variables|Default|GetQ_G_0) (Variables|Default|GetQ_G_1) (Variables|Default|GetQ_G_2)) :Option%206 (Utilities|Array|MakeArray (Variables|Default|GetQ_H_0) (Variables|Default|GetQ_H_1) (Variables|Default|GetQ_H_2)) :Option%207 (Utilities|Array|MakeArray (Variables|Default|GetQ_I_0)) :Option%208 (Utilities|Array|MakeArray (Variables|Default|GetQ_J_0)) :Option%209 (Utilities|Array|MakeArray (Variables|Default|GetQ_K_0)) :Option%2010 (Utilities|Array|MakeArray (Variables|Default|GetQ_L_0)) :Option%2011 (Utilities|Array|MakeArray (Variables|Default|GetQ_M_0)) :Option%2012 (Utilities|Array|MakeArray (Variables|Default|GetQ_E_0) (Variables|Default|GetQ_E_1) (Variables|Default|GetQ_E_2)) :Option%2013 (Utilities|Array|MakeArray (Variables|Default|GetQW) (Variables|Default|GetQW1) (Variables|Default|Getnext))) :!label _label)
      (elif (== (Variables|Default|GetAnswerInt) 1)
        (Variables|/Game/SpaceState/Blueprint/Widget_Dialogue.Widget_Dialogue_C|SetNPCDia _answers "")
        (Variables|Default|SetUpdateArray 2)
        (goto _label)
        (elif (== (Variables|Default|GetAnswerInt) 2)
          (Variables|/Game/SpaceState/Blueprint/Widget_Dialogue.Widget_Dialogue_C|SetNPCDia _answers "")
          (Variables|Default|SetUpdateArray 3)
          (goto _label))))
    (else
      ;[1 1 1] What would you like?
      (if (== (Variables|Default|GetUpdateArray) 0)
        (if (== (Variables|Default|GetAnswerInt) 0)
          (Variables|/Game/SpaceState/Blueprint/Widget_Dialogue.Widget_Dialogue_C|SetNPCDia _answers_7 (Variables|Default|GetNHP))
          (Variables|Default|SetUpdateArray 1)
          (Variables|Default|SetButtonText (Utilities|Select :Index (Variables|Default|GetUpdateArray) :Option%200 (Utilities|Array|MakeArray (Variables|Default|GetA1) (Variables|Default|GetA2) (Variables|Default|GetA3)) :Option%201 (Utilities|Array|MakeArray (Variables|Default|Getphp1) (Variables|Default|Getphp2) (Variables|Default|Getphp3)) :Option%202 (Utilities|Array|MakeArray (Variables|Default|GetPQ2a) (Variables|Default|GetPQ2b) (Variables|Default|Getpmore)) :Option%203 (Utilities|Array|MakeArray (Variables|Default|GetPWeap1) (Variables|Default|GetPweap2) (Variables|Default|GetPweap3)) :Option%204 (Utilities|Array|MakeArray (Variables|Default|GetPflamerammo) (Variables|Default|GetPpowercells) (Variables|Default|Getpmore2)) :Option%205 (Utilities|Array|MakeArray (Variables|Default|GetQ_G_0) (Variables|Default|GetQ_G_1) (Variables|Default|GetQ_G_2)) :Option%206 (Utilities|Array|MakeArray (Variables|Default|GetQ_H_0) (Variables|Default|GetQ_H_1) (Variables|Default|GetQ_H_2)) :Option%207 (Utilities|Array|MakeArray (Variables|Default|GetQ_I_0)) :Option%208 (Utilities|Array|MakeArray (Variables|Default|GetQ_J_0)) :Option%209 (Utilities|Array|MakeArray (Variables|Default|GetQ_K_0)) :Option%2010 (Utilities|Array|MakeArray (Variables|Default|GetQ_L_0)) :Option%2011 (Utilities|Array|MakeArray (Variables|Default|GetQ_M_0)) :Option%2012 (Utilities|Array|MakeArray (Variables|Default|GetQ_E_0) (Variables|Default|GetQ_E_1) (Variables|Default|GetQ_E_2)) :Option%2013 (Utilities|Array|MakeArray (Variables|Default|GetQW) (Variables|Default|GetQW1) (Variables|Default|Getnext))) :!label _label_2)
          (elif (== (Variables|Default|GetAnswerInt) 1)
            (Variables|/Game/SpaceState/Blueprint/Widget_Dialogue.Widget_Dialogue_C|SetNPCDia _answers_7 (Variables|Default|GetNPCAmmo))
            (Variables|Default|SetUpdateArray 2)
            (goto _label_2)
            (elif (== (Variables|Default|GetAnswerInt) 2)
              (Variables|/Game/SpaceState/Blueprint/Widget_Dialogue.Widget_Dialogue_C|SetNPCDia _answers_7 (Variables|Default|GetNPCWeapons))
              (Variables|Default|SetUpdateArray 3)
              (goto _label_2))))
        (else
          ;[1 1 1] HP
          (if (== (Variables|Default|GetUpdateArray) 1)
            (if (== (Variables|Default|GetAnswerInt) 0)
              (bind _asbp_dude_2 (Utilities|Casting|CastToBP_Dude _returnvalue))
              (if (> (Variables|/Game/SpaceState/Blueprint/BP_Dude/BP_Dude.BP_Dude_C|GetCharCredits _asbp_dude_2) 100)
                (if (>= (Variables|/Game/SpaceState/Blueprint/BP_Dude/BP_Dude.BP_Dude_C|GetHealth%20Current _asbp_dude_2) 1.0)
                  (Variables|/Game/SpaceState/Blueprint/Widget_Dialogue.Widget_Dialogue_C|SetNPCDia _answers_2 (Variables|Default|GetNFullHP) :!label _label_3)
                  (Variables|Default|SetUpdateArray 0)
                  (goto _label_2)
                  (else
                    (Default|Creditsystem _asbp_dude_2 -100)
                    (Variables|/Game/SpaceState/Blueprint/BP_Dude/BP_Dude.BP_Dude_C|SetHealth%20Current _asbp_dude_2 (+ (Variables|/Game/SpaceState/Blueprint/BP_Dude/BP_Dude.BP_Dude_C|GetHealth%20Current _asbp_dude_2) 0.25))
                    (Variables|/Game/SpaceState/Blueprint/Widget_Dialogue.Widget_Dialogue_C|SetNPCDia _answers_2 _nhp1)
                    (Variables|Default|SetUpdateArray 0)
                    (goto _label_2)))
                (else
                  (Variables|/Game/SpaceState/Blueprint/Widget_Dialogue.Widget_Dialogue_C|SetNPCDia _answers_2 (Variables|Default|GetNPCNotEnoughCreds) :!label _label_4)
                  (Variables|Default|SetUpdateArray 0)
                  (goto _label_2)))
              (elif (== (Variables|Default|GetAnswerInt) 1)
                (bind _asbp_dude_3 (Utilities|Casting|CastToBP_Dude _returnvalue))
                (if (> (Variables|/Game/SpaceState/Blueprint/BP_Dude/BP_Dude.BP_Dude_C|GetCharCredits _asbp_dude_3) 200)
                  (if (>= (Variables|/Game/SpaceState/Blueprint/BP_Dude/BP_Dude.BP_Dude_C|GetHealth%20Current _asbp_dude_3) 0.75)
                    (goto _label_3)
                    (else
                      (Default|Creditsystem _asbp_dude_3 -200)
                      (Variables|/Game/SpaceState/Blueprint/BP_Dude/BP_Dude.BP_Dude_C|SetHealth%20Current _asbp_dude_3 (+ (Variables|/Game/SpaceState/Blueprint/BP_Dude/BP_Dude.BP_Dude_C|GetHealth%20Current _asbp_dude_3) 0.5))
                      (Variables|/Game/SpaceState/Blueprint/Widget_Dialogue.Widget_Dialogue_C|SetNPCDia _answers_2 _nhp1)
                      (Variables|Default|SetUpdateArray 0)
                      ;[1 1 1] Set UMG Text
                      (Variables|Default|SetButtonText (Utilities|Select :Index (Variables|Default|GetUpdateArray) :Option%200 (Utilities|Array|MakeArray (Variables|Default|GetA1) (Variables|Default|GetA2) (Variables|Default|GetA3)) :Option%201 (Utilities|Array|MakeArray (Variables|Default|Getphp1) (Variables|Default|Getphp2) (Variables|Default|Getphp3)) :Option%202 (Utilities|Array|MakeArray (Variables|Default|GetPQ2a) (Variables|Default|GetPQ2b) (Variables|Default|Getpmore)) :Option%203 (Utilities|Array|MakeArray (Variables|Default|GetPWeap1) (Variables|Default|GetPweap2) (Variables|Default|GetPweap3)) :Option%204 (Utilities|Array|MakeArray (Variables|Default|GetPflamerammo) (Variables|Default|GetPpowercells) (Variables|Default|Getpmore2)) :Option%205 (Utilities|Array|MakeArray (Variables|Default|GetQ_G_0) (Variables|Default|GetQ_G_1) (Variables|Default|GetQ_G_2)) :Option%206 (Utilities|Array|MakeArray (Variables|Default|GetQ_H_0) (Variables|Default|GetQ_H_1) (Variables|Default|GetQ_H_2)) :Option%207 (Utilities|Array|MakeArray (Variables|Default|GetQ_I_0)) :Option%208 (Utilities|Array|MakeArray (Variables|Default|GetQ_J_0)) :Option%209 (Utilities|Array|MakeArray (Variables|Default|GetQ_K_0)) :Option%2010 (Utilities|Array|MakeArray (Variables|Default|GetQ_L_0)) :Option%2011 (Utilities|Array|MakeArray (Variables|Default|GetQ_M_0)) :Option%2012 (Utilities|Array|MakeArray (Variables|Default|GetQ_E_0) (Variables|Default|GetQ_E_1) (Variables|Default|GetQ_E_2)) :Option%2013 (Utilities|Array|MakeArray (Variables|Default|GetQW) (Variables|Default|GetQW1) (Variables|Default|Getnext))) :!label _label_5)))
                  (else
                    (goto _label_4)))
                (elif (== (Variables|Default|GetAnswerInt) 2)
                  (bind _asbp_dude_4 (Utilities|Casting|CastToBP_Dude _returnvalue))
                  (if (> (Variables|/Game/SpaceState/Blueprint/BP_Dude/BP_Dude.BP_Dude_C|GetCharCredits _asbp_dude_4) 300)
                    (if (>= (Variables|/Game/SpaceState/Blueprint/BP_Dude/BP_Dude.BP_Dude_C|GetHealth%20Current _asbp_dude_4) 0.5)
                      (goto _label_3)
                      (else
                        (Default|Creditsystem _asbp_dude_4 -300)
                        (Variables|/Game/SpaceState/Blueprint/BP_Dude/BP_Dude.BP_Dude_C|SetHealth%20Current _asbp_dude_4 (+ (Variables|/Game/SpaceState/Blueprint/BP_Dude/BP_Dude.BP_Dude_C|GetHealth%20Current _asbp_dude_4) 1.0))
                        (Variables|/Game/SpaceState/Blueprint/Widget_Dialogue.Widget_Dialogue_C|SetNPCDia _answers_2 (Variables|Default|GetNhp2))
                        (Variables|Default|SetUpdateArray 0)
                        (goto _label_5)))
                    (else
                      (goto _label_4))))))
            (else
              ;[1 1 1] Ammo1
              (if (== (Variables|Default|GetUpdateArray) 2)
                (if (== (Variables|Default|GetAnswerInt) 0)
                  (bind _asbp_dude_5 (Utilities|Casting|CastToBP_Dude (Game|GetPlayerCharacter 0)))
                  (if (< (Variables|/Game/SpaceState/Blueprint/BP_Dude/BP_Dude.BP_Dude_C|GetCharCredits _asbp_dude_5) 100)
                    (Variables|/Game/SpaceState/Blueprint/Widget_Dialogue.Widget_Dialogue_C|SetNPCDia _answers_5 (Variables|Default|GetNPCNotEnoughCreds))
                    (Variables|Default|SetUpdateArray 2)
                    (goto _label_5)
                    (elif (>= (Utilities|Array|Get(acopy) (Variables|/Game/SpaceState/Blueprint/BP_Dude/BP_Dude.BP_Dude_C|GetBulletCountsArray _asbp_dude_5) 1) (Variables|/Game/SpaceState/Blueprint/BP_Dude/BP_Dude.BP_Dude_C|GetMaxBullets _asbp_dude_5))
                      (Variables|/Game/SpaceState/Blueprint/Widget_Dialogue.Widget_Dialogue_C|SetNPCDia _answers_5 (Variables|Default|GetNPCFull))
                      (Variables|Default|SetUpdateArray 2)
                      (goto _label_5)
                      (else
                        (Default|BulletSystem _asbp_dude_5 10)
                        (Default|Creditsystem _asbp_dude_5 -100)
                        (Variables|/Game/SpaceState/Blueprint/Widget_Dialogue.Widget_Dialogue_C|SetNPCDia _answers_5 (Variables|Default|GetNPCAmmoR))
                        (Variables|Default|SetUpdateArray 2)
                        (goto _label_5))))
                  (elif (== (Variables|Default|GetAnswerInt) 1)
                    (bind _asbp_dude_6 (Utilities|Casting|CastToBP_Dude (Game|GetPlayerCharacter 0)))
                    (if (< (Variables|/Game/SpaceState/Blueprint/BP_Dude/BP_Dude.BP_Dude_C|GetCharCredits _asbp_dude_6) 100)
                      (Variables|/Game/SpaceState/Blueprint/Widget_Dialogue.Widget_Dialogue_C|SetNPCDia _answers_5 (Variables|Default|GetNPCNotEnoughCreds))
                      (Variables|Default|SetUpdateArray 2)
                      (goto _label_5)
                      (elif (>= (Utilities|Array|Get(acopy) (Variables|/Game/SpaceState/Blueprint/BP_Dude/BP_Dude.BP_Dude_C|GetBulletCountsArray _asbp_dude_6) 2) (Variables|/Game/SpaceState/Blueprint/BP_Dude/BP_Dude.BP_Dude_C|GetMaxShells _asbp_dude_6))
                        (Variables|/Game/SpaceState/Blueprint/Widget_Dialogue.Widget_Dialogue_C|SetNPCDia _answers_5 (Variables|Default|GetNPCFull))
                        (Variables|Default|SetUpdateArray 2)
                        (goto _label_5)
                        (else
                          (Default|ShellSystem _asbp_dude_6 10)
                          (Default|Creditsystem _asbp_dude_6 -100)
                          (Variables|/Game/SpaceState/Blueprint/Widget_Dialogue.Widget_Dialogue_C|SetNPCDia _answers_5 (Variables|Default|GetNPCAmmoS))
                          (Variables|Default|SetUpdateArray 2)
                          (goto _label_5))))
                    (elif (== (Variables|Default|GetAnswerInt) 2)
                      (Variables|/Game/SpaceState/Blueprint/Widget_Dialogue.Widget_Dialogue_C|SetNPCDia _answers_5 (Variables|Default|GetNPCAmmo))
                      (Variables|Default|SetUpdateArray 4)
                      (Variables|Default|SetButtonText (Utilities|Select :Index (Variables|Default|GetUpdateArray) :Option%200 (Utilities|Array|MakeArray (Variables|Default|GetA1) (Variables|Default|GetA2) (Variables|Default|GetA3)) :Option%201 (Utilities|Array|MakeArray (Variables|Default|Getphp1) (Variables|Default|Getphp2) (Variables|Default|Getphp3)) :Option%202 (Utilities|Array|MakeArray (Variables|Default|GetPQ2a) (Variables|Default|GetPQ2b) (Variables|Default|Getpmore)) :Option%203 (Utilities|Array|MakeArray (Variables|Default|GetPWeap1) (Variables|Default|GetPweap2) (Variables|Default|GetPweap3)) :Option%204 (Utilities|Array|MakeArray (Variables|Default|GetPflamerammo) (Variables|Default|GetPpowercells) (Variables|Default|Getpmore2)) :Option%205 (Utilities|Array|MakeArray (Variables|Default|GetQ_G_0) (Variables|Default|GetQ_G_1) (Variables|Default|GetQ_G_2)) :Option%206 (Utilities|Array|MakeArray (Variables|Default|GetQ_H_0) (Variables|Default|GetQ_H_1) (Variables|Default|GetQ_H_2)) :Option%207 (Utilities|Array|MakeArray (Variables|Default|GetQ_I_0)) :Option%208 (Utilities|Array|MakeArray (Variables|Default|GetQ_J_0)) :Option%209 (Utilities|Array|MakeArray (Variables|Default|GetQ_K_0)) :Option%2010 (Utilities|Array|MakeArray (Variables|Default|GetQ_L_0)) :Option%2011 (Utilities|Array|MakeArray (Variables|Default|GetQ_M_0)) :Option%2012 (Utilities|Array|MakeArray (Variables|Default|GetQ_E_0) (Variables|Default|GetQ_E_1) (Variables|Default|GetQ_E_2)) :Option%2013 (Utilities|Array|MakeArray (Variables|Default|GetQW) (Variables|Default|GetQW1) (Variables|Default|Getnext)))))))
                (else
                  ;[1 1 1] Weapons
                  (if (== (Variables|Default|GetUpdateArray) 3)
                    (if (== (Variables|Default|GetAnswerInt) 0)
                      (bind _asbp_dude_7 (Utilities|Casting|CastToBP_Dude (Game|GetPlayerCharacter 0)))
                      (if (< (Variables|/Game/SpaceState/Blueprint/BP_Dude/BP_Dude.BP_Dude_C|GetCharCredits _asbp_dude_7) 500)
                        (Variables|/Game/SpaceState/Blueprint/Widget_Dialogue.Widget_Dialogue_C|SetNPCDia _answers_6 (Variables|Default|GetNPCNotEnoughCreds))
                        (Variables|Default|SetUpdateArray 0)
                        (goto _label)
                        (elif (>= (Variables|/Game/SpaceState/Blueprint/BP_Dude/BP_Dude.BP_Dude_C|GetMaxWeaps _asbp_dude_7) 3)
                          (Variables|/Game/SpaceState/Blueprint/Widget_Dialogue.Widget_Dialogue_C|SetNPCDia _answers_6 (Variables|Default|GetNWeapHave))
                          (Variables|Default|SetUpdateArray 0)
                          (goto _label)
                          (else
                            (Default|Creditsystem _asbp_dude_7 -500)
                            (Variables|/Game/SpaceState/Blueprint/BP_Dude/BP_Dude.BP_Dude_C|SetMaxWeaps _asbp_dude_7 3)
                            (Variables|/Game/SpaceState/Blueprint/Widget_Dialogue.Widget_Dialogue_C|SetNPCDia _answers_6 (Variables|Default|GetNShotgun))
                            (Variables|Default|SetUpdateArray 0)
                            (goto _label))))
                      (elif (== (Variables|Default|GetAnswerInt) 1)
                        (Variables|/Game/SpaceState/Blueprint/Widget_Dialogue.Widget_Dialogue_C|SetNPCDia _answers_6 (Variables|Default|GetNFlamer))
                        (Variables|Default|SetUpdateArray 0)
                        (goto _label)))
                    (else
                      ;[1 1 1] Ammo2
                      (if (== (Variables|Default|GetUpdateArray) 4)
                        (if (== (Variables|Default|GetAnswerInt) 0)
                          (bind _asbp_dude_8 (Utilities|Casting|CastToBP_Dude (Game|GetPlayerCharacter 0)))
                          (if (< (Variables|/Game/SpaceState/Blueprint/BP_Dude/BP_Dude.BP_Dude_C|GetCharCredits _asbp_dude_8) 100)
                            (Variables|/Game/SpaceState/Blueprint/Widget_Dialogue.Widget_Dialogue_C|SetNPCDia _answers_3 (Variables|Default|GetNPCNotEnoughCreds))
                            (Variables|Default|SetUpdateArray 4)
                            (goto _label)
                            (elif (>= (Utilities|Array|Get(acopy) (Variables|/Game/SpaceState/Blueprint/BP_Dude/BP_Dude.BP_Dude_C|GetBulletCountsArray _asbp_dude_8) 4) (Variables|/Game/SpaceState/Blueprint/BP_Dude/BP_Dude.BP_Dude_C|GetMaxFuel _asbp_dude_8))
                              (Variables|/Game/SpaceState/Blueprint/Widget_Dialogue.Widget_Dialogue_C|SetNPCDia _answers_3 (Variables|Default|GetNPCFull))
                              (Variables|Default|SetUpdateArray 4)
                              (goto _label)
                              (else
                                (Default|FuelSystem _asbp_dude_8 100)
                                (Default|Creditsystem _asbp_dude_8 -100)
                                (Variables|/Game/SpaceState/Blueprint/Widget_Dialogue.Widget_Dialogue_C|SetNPCDia _answers_4 (Variables|Default|GetNPCAmmoF))
                                (Variables|Default|SetUpdateArray 4)
                                (goto _label))))
                          (elif (== (Variables|Default|GetAnswerInt) 1)
                            (bind _asbp_dude_9 (Utilities|Casting|CastToBP_Dude (Game|GetPlayerCharacter 0)))
                            (if (< (Variables|/Game/SpaceState/Blueprint/BP_Dude/BP_Dude.BP_Dude_C|GetCharCredits _asbp_dude_9) 100)
                              (Variables|/Game/SpaceState/Blueprint/Widget_Dialogue.Widget_Dialogue_C|SetNPCDia _answers_3 (Variables|Default|GetNPCNotEnoughCreds))
                              (Variables|Default|SetUpdateArray 4)
                              (goto _label)
                              (elif (>= (Utilities|Array|Get(acopy) (Variables|/Game/SpaceState/Blueprint/BP_Dude/BP_Dude.BP_Dude_C|GetBulletCountsArray _asbp_dude_9) 3) (Variables|/Game/SpaceState/Blueprint/BP_Dude/BP_Dude.BP_Dude_C|GetMaxCells _asbp_dude_9))
                                (Variables|/Game/SpaceState/Blueprint/Widget_Dialogue.Widget_Dialogue_C|SetNPCDia _answers_3 (Variables|Default|GetNPCFull))
                                (Variables|Default|SetUpdateArray 4)
                                (goto _label)
                                (else
                                  (Default|CellSystem _asbp_dude_9 1)
                                  (Default|Creditsystem _asbp_dude_9 -100)
                                  (Variables|/Game/SpaceState/Blueprint/Widget_Dialogue.Widget_Dialogue_C|SetNPCDia _answers_4 (Variables|Default|GetNPCAmmoRG))
                                  (Variables|Default|SetUpdateArray 4)
                                  (goto _label))))
                            (elif (== (Variables|Default|GetAnswerInt) 2)
                              (Variables|/Game/SpaceState/Blueprint/Widget_Dialogue.Widget_Dialogue_C|SetNPCDia _answers_4 (Variables|Default|GetNPCAmmo))
                              (Variables|Default|SetUpdateArray 2)
                              (goto _label))))))))))))))))

(event Custom|Answer4
  ;[1 1 1] Leaving now response
  (CallFunction|Leaving))

(event Custom|Answer2
  (bind _returnvalue (Game|GetPlayerCharacter 0))
  (bind _answers (Variables|Default|GetAnswers))
  (bind _answers_2 (Variables|Default|GetAnswers))
  (bind _answers_3 (Variables|Default|GetAnswers))
  (bind _answers_4 (Variables|Default|GetAnswers))
  (bind _answers_5 (Variables|Default|GetAnswers))
  (bind _answers_6 (Variables|Default|GetAnswers))
  (bind _nhp1 (Variables|Default|GetNhp1))
  (bind _answers_7 (Variables|Default|GetAnswers))
  ;[1 1 1] Input
  (Variables|Default|SetAnswerInt 1)
  ;[1 1 1] FirstTime
  (if (== (Variables|Default|GetUpdateArray) 5)
    (if (== (Variables|Default|GetAnswerInt) 0)
      (Variables|/Game/SpaceState/Blueprint/Widget_Dialogue.Widget_Dialogue_C|SetNPCDia _answers (Variables|Default|Getnext))
      (bind _asbp_dude (Utilities|Casting|CastToBP_Dude (Game|GetPlayerCharacter 0)))
      (Variables|/Game/SpaceState/Blueprint/BP_Dude/BP_Dude.BP_Dude_C|SetMainQuest _asbp_dude 2)
      (Variables|Default|SetUpdateArray 6)
      (Variables|Default|SetButtonText (Utilities|Select :Index (Variables|Default|GetUpdateArray) :Option%200 (Utilities|Array|MakeArray (Variables|Default|GetA1) (Variables|Default|GetA2) (Variables|Default|GetA3)) :Option%201 (Utilities|Array|MakeArray (Variables|Default|Getphp1) (Variables|Default|Getphp2) (Variables|Default|Getphp3)) :Option%202 (Utilities|Array|MakeArray (Variables|Default|GetPQ2a) (Variables|Default|GetPQ2b) (Variables|Default|Getpmore)) :Option%203 (Utilities|Array|MakeArray (Variables|Default|GetPWeap1) (Variables|Default|GetPweap2) (Variables|Default|GetPweap3)) :Option%204 (Utilities|Array|MakeArray (Variables|Default|GetPflamerammo) (Variables|Default|GetPpowercells) (Variables|Default|Getpmore2)) :Option%205 (Utilities|Array|MakeArray (Variables|Default|GetQ_G_0) (Variables|Default|GetQ_G_1) (Variables|Default|GetQ_G_2)) :Option%206 (Utilities|Array|MakeArray (Variables|Default|GetQ_H_0) (Variables|Default|GetQ_H_1) (Variables|Default|GetQ_H_2)) :Option%207 (Utilities|Array|MakeArray (Variables|Default|GetQ_I_0)) :Option%208 (Utilities|Array|MakeArray (Variables|Default|GetQ_J_0)) :Option%209 (Utilities|Array|MakeArray (Variables|Default|GetQ_K_0)) :Option%2010 (Utilities|Array|MakeArray (Variables|Default|GetQ_L_0)) :Option%2011 (Utilities|Array|MakeArray (Variables|Default|GetQ_M_0)) :Option%2012 (Utilities|Array|MakeArray (Variables|Default|GetQ_E_0) (Variables|Default|GetQ_E_1) (Variables|Default|GetQ_E_2)) :Option%2013 (Utilities|Array|MakeArray (Variables|Default|GetQW) (Variables|Default|GetQW1) (Variables|Default|Getnext))) :!label _label)
      (elif (== (Variables|Default|GetAnswerInt) 1)
        (Variables|/Game/SpaceState/Blueprint/Widget_Dialogue.Widget_Dialogue_C|SetNPCDia _answers "")
        (Variables|Default|SetUpdateArray 2)
        (goto _label)
        (elif (== (Variables|Default|GetAnswerInt) 2)
          (Variables|/Game/SpaceState/Blueprint/Widget_Dialogue.Widget_Dialogue_C|SetNPCDia _answers "")
          (Variables|Default|SetUpdateArray 3)
          (goto _label))))
    (else
      ;[1 1 1] What would you like?
      (if (== (Variables|Default|GetUpdateArray) 0)
        (if (== (Variables|Default|GetAnswerInt) 0)
          (Variables|/Game/SpaceState/Blueprint/Widget_Dialogue.Widget_Dialogue_C|SetNPCDia _answers_7 (Variables|Default|GetNHP))
          (Variables|Default|SetUpdateArray 1)
          (Variables|Default|SetButtonText (Utilities|Select :Index (Variables|Default|GetUpdateArray) :Option%200 (Utilities|Array|MakeArray (Variables|Default|GetA1) (Variables|Default|GetA2) (Variables|Default|GetA3)) :Option%201 (Utilities|Array|MakeArray (Variables|Default|Getphp1) (Variables|Default|Getphp2) (Variables|Default|Getphp3)) :Option%202 (Utilities|Array|MakeArray (Variables|Default|GetPQ2a) (Variables|Default|GetPQ2b) (Variables|Default|Getpmore)) :Option%203 (Utilities|Array|MakeArray (Variables|Default|GetPWeap1) (Variables|Default|GetPweap2) (Variables|Default|GetPweap3)) :Option%204 (Utilities|Array|MakeArray (Variables|Default|GetPflamerammo) (Variables|Default|GetPpowercells) (Variables|Default|Getpmore2)) :Option%205 (Utilities|Array|MakeArray (Variables|Default|GetQ_G_0) (Variables|Default|GetQ_G_1) (Variables|Default|GetQ_G_2)) :Option%206 (Utilities|Array|MakeArray (Variables|Default|GetQ_H_0) (Variables|Default|GetQ_H_1) (Variables|Default|GetQ_H_2)) :Option%207 (Utilities|Array|MakeArray (Variables|Default|GetQ_I_0)) :Option%208 (Utilities|Array|MakeArray (Variables|Default|GetQ_J_0)) :Option%209 (Utilities|Array|MakeArray (Variables|Default|GetQ_K_0)) :Option%2010 (Utilities|Array|MakeArray (Variables|Default|GetQ_L_0)) :Option%2011 (Utilities|Array|MakeArray (Variables|Default|GetQ_M_0)) :Option%2012 (Utilities|Array|MakeArray (Variables|Default|GetQ_E_0) (Variables|Default|GetQ_E_1) (Variables|Default|GetQ_E_2)) :Option%2013 (Utilities|Array|MakeArray (Variables|Default|GetQW) (Variables|Default|GetQW1) (Variables|Default|Getnext))) :!label _label_2)
          (elif (== (Variables|Default|GetAnswerInt) 1)
            (Variables|/Game/SpaceState/Blueprint/Widget_Dialogue.Widget_Dialogue_C|SetNPCDia _answers_7 (Variables|Default|GetNPCAmmo))
            (Variables|Default|SetUpdateArray 2)
            (goto _label_2)
            (elif (== (Variables|Default|GetAnswerInt) 2)
              (Variables|/Game/SpaceState/Blueprint/Widget_Dialogue.Widget_Dialogue_C|SetNPCDia _answers_7 (Variables|Default|GetNPCWeapons))
              (Variables|Default|SetUpdateArray 3)
              (goto _label_2))))
        (else
          ;[1 1 1] HP
          (if (== (Variables|Default|GetUpdateArray) 1)
            (if (== (Variables|Default|GetAnswerInt) 0)
              (bind _asbp_dude_2 (Utilities|Casting|CastToBP_Dude _returnvalue))
              (if (> (Variables|/Game/SpaceState/Blueprint/BP_Dude/BP_Dude.BP_Dude_C|GetCharCredits _asbp_dude_2) 100)
                (if (>= (Variables|/Game/SpaceState/Blueprint/BP_Dude/BP_Dude.BP_Dude_C|GetHealth%20Current _asbp_dude_2) 1.0)
                  (Variables|/Game/SpaceState/Blueprint/Widget_Dialogue.Widget_Dialogue_C|SetNPCDia _answers_2 (Variables|Default|GetNFullHP) :!label _label_3)
                  (Variables|Default|SetUpdateArray 0)
                  (goto _label_2)
                  (else
                    (Default|Creditsystem _asbp_dude_2 -100)
                    (Variables|/Game/SpaceState/Blueprint/BP_Dude/BP_Dude.BP_Dude_C|SetHealth%20Current _asbp_dude_2 (+ (Variables|/Game/SpaceState/Blueprint/BP_Dude/BP_Dude.BP_Dude_C|GetHealth%20Current _asbp_dude_2) 0.25))
                    (Variables|/Game/SpaceState/Blueprint/Widget_Dialogue.Widget_Dialogue_C|SetNPCDia _answers_2 _nhp1)
                    (Variables|Default|SetUpdateArray 0)
                    (goto _label_2)))
                (else
                  (Variables|/Game/SpaceState/Blueprint/Widget_Dialogue.Widget_Dialogue_C|SetNPCDia _answers_2 (Variables|Default|GetNPCNotEnoughCreds) :!label _label_4)
                  (Variables|Default|SetUpdateArray 0)
                  (goto _label_2)))
              (elif (== (Variables|Default|GetAnswerInt) 1)
                (bind _asbp_dude_3 (Utilities|Casting|CastToBP_Dude _returnvalue))
                (if (> (Variables|/Game/SpaceState/Blueprint/BP_Dude/BP_Dude.BP_Dude_C|GetCharCredits _asbp_dude_3) 200)
                  (if (>= (Variables|/Game/SpaceState/Blueprint/BP_Dude/BP_Dude.BP_Dude_C|GetHealth%20Current _asbp_dude_3) 0.75)
                    (goto _label_3)
                    (else
                      (Default|Creditsystem _asbp_dude_3 -200)
                      (Variables|/Game/SpaceState/Blueprint/BP_Dude/BP_Dude.BP_Dude_C|SetHealth%20Current _asbp_dude_3 (+ (Variables|/Game/SpaceState/Blueprint/BP_Dude/BP_Dude.BP_Dude_C|GetHealth%20Current _asbp_dude_3) 0.5))
                      (Variables|/Game/SpaceState/Blueprint/Widget_Dialogue.Widget_Dialogue_C|SetNPCDia _answers_2 _nhp1)
                      (Variables|Default|SetUpdateArray 0)
                      ;[1 1 1] Set UMG Text
                      (Variables|Default|SetButtonText (Utilities|Select :Index (Variables|Default|GetUpdateArray) :Option%200 (Utilities|Array|MakeArray (Variables|Default|GetA1) (Variables|Default|GetA2) (Variables|Default|GetA3)) :Option%201 (Utilities|Array|MakeArray (Variables|Default|Getphp1) (Variables|Default|Getphp2) (Variables|Default|Getphp3)) :Option%202 (Utilities|Array|MakeArray (Variables|Default|GetPQ2a) (Variables|Default|GetPQ2b) (Variables|Default|Getpmore)) :Option%203 (Utilities|Array|MakeArray (Variables|Default|GetPWeap1) (Variables|Default|GetPweap2) (Variables|Default|GetPweap3)) :Option%204 (Utilities|Array|MakeArray (Variables|Default|GetPflamerammo) (Variables|Default|GetPpowercells) (Variables|Default|Getpmore2)) :Option%205 (Utilities|Array|MakeArray (Variables|Default|GetQ_G_0) (Variables|Default|GetQ_G_1) (Variables|Default|GetQ_G_2)) :Option%206 (Utilities|Array|MakeArray (Variables|Default|GetQ_H_0) (Variables|Default|GetQ_H_1) (Variables|Default|GetQ_H_2)) :Option%207 (Utilities|Array|MakeArray (Variables|Default|GetQ_I_0)) :Option%208 (Utilities|Array|MakeArray (Variables|Default|GetQ_J_0)) :Option%209 (Utilities|Array|MakeArray (Variables|Default|GetQ_K_0)) :Option%2010 (Utilities|Array|MakeArray (Variables|Default|GetQ_L_0)) :Option%2011 (Utilities|Array|MakeArray (Variables|Default|GetQ_M_0)) :Option%2012 (Utilities|Array|MakeArray (Variables|Default|GetQ_E_0) (Variables|Default|GetQ_E_1) (Variables|Default|GetQ_E_2)) :Option%2013 (Utilities|Array|MakeArray (Variables|Default|GetQW) (Variables|Default|GetQW1) (Variables|Default|Getnext))) :!label _label_5)))
                  (else
                    (goto _label_4)))
                (elif (== (Variables|Default|GetAnswerInt) 2)
                  (bind _asbp_dude_4 (Utilities|Casting|CastToBP_Dude _returnvalue))
                  (if (> (Variables|/Game/SpaceState/Blueprint/BP_Dude/BP_Dude.BP_Dude_C|GetCharCredits _asbp_dude_4) 300)
                    (if (>= (Variables|/Game/SpaceState/Blueprint/BP_Dude/BP_Dude.BP_Dude_C|GetHealth%20Current _asbp_dude_4) 0.5)
                      (goto _label_3)
                      (else
                        (Default|Creditsystem _asbp_dude_4 -300)
                        (Variables|/Game/SpaceState/Blueprint/BP_Dude/BP_Dude.BP_Dude_C|SetHealth%20Current _asbp_dude_4 (+ (Variables|/Game/SpaceState/Blueprint/BP_Dude/BP_Dude.BP_Dude_C|GetHealth%20Current _asbp_dude_4) 1.0))
                        (Variables|/Game/SpaceState/Blueprint/Widget_Dialogue.Widget_Dialogue_C|SetNPCDia _answers_2 (Variables|Default|GetNhp2))
                        (Variables|Default|SetUpdateArray 0)
                        (goto _label_5)))
                    (else
                      (goto _label_4))))))
            (else
              ;[1 1 1] Ammo1
              (if (== (Variables|Default|GetUpdateArray) 2)
                (if (== (Variables|Default|GetAnswerInt) 0)
                  (bind _asbp_dude_5 (Utilities|Casting|CastToBP_Dude (Game|GetPlayerCharacter 0)))
                  (if (< (Variables|/Game/SpaceState/Blueprint/BP_Dude/BP_Dude.BP_Dude_C|GetCharCredits _asbp_dude_5) 100)
                    (Variables|/Game/SpaceState/Blueprint/Widget_Dialogue.Widget_Dialogue_C|SetNPCDia _answers_5 (Variables|Default|GetNPCNotEnoughCreds))
                    (Variables|Default|SetUpdateArray 2)
                    (goto _label_5)
                    (elif (>= (Utilities|Array|Get(acopy) (Variables|/Game/SpaceState/Blueprint/BP_Dude/BP_Dude.BP_Dude_C|GetBulletCountsArray _asbp_dude_5) 1) (Variables|/Game/SpaceState/Blueprint/BP_Dude/BP_Dude.BP_Dude_C|GetMaxBullets _asbp_dude_5))
                      (Variables|/Game/SpaceState/Blueprint/Widget_Dialogue.Widget_Dialogue_C|SetNPCDia _answers_5 (Variables|Default|GetNPCFull))
                      (Variables|Default|SetUpdateArray 2)
                      (goto _label_5)
                      (else
                        (Default|BulletSystem _asbp_dude_5 10)
                        (Default|Creditsystem _asbp_dude_5 -100)
                        (Variables|/Game/SpaceState/Blueprint/Widget_Dialogue.Widget_Dialogue_C|SetNPCDia _answers_5 (Variables|Default|GetNPCAmmoR))
                        (Variables|Default|SetUpdateArray 2)
                        (goto _label_5))))
                  (elif (== (Variables|Default|GetAnswerInt) 1)
                    (bind _asbp_dude_6 (Utilities|Casting|CastToBP_Dude (Game|GetPlayerCharacter 0)))
                    (if (< (Variables|/Game/SpaceState/Blueprint/BP_Dude/BP_Dude.BP_Dude_C|GetCharCredits _asbp_dude_6) 100)
                      (Variables|/Game/SpaceState/Blueprint/Widget_Dialogue.Widget_Dialogue_C|SetNPCDia _answers_5 (Variables|Default|GetNPCNotEnoughCreds))
                      (Variables|Default|SetUpdateArray 2)
                      (goto _label_5)
                      (elif (>= (Utilities|Array|Get(acopy) (Variables|/Game/SpaceState/Blueprint/BP_Dude/BP_Dude.BP_Dude_C|GetBulletCountsArray _asbp_dude_6) 2) (Variables|/Game/SpaceState/Blueprint/BP_Dude/BP_Dude.BP_Dude_C|GetMaxShells _asbp_dude_6))
                        (Variables|/Game/SpaceState/Blueprint/Widget_Dialogue.Widget_Dialogue_C|SetNPCDia _answers_5 (Variables|Default|GetNPCFull))
                        (Variables|Default|SetUpdateArray 2)
                        (goto _label_5)
                        (else
                          (Default|ShellSystem _asbp_dude_6 10)
                          (Default|Creditsystem _asbp_dude_6 -100)
                          (Variables|/Game/SpaceState/Blueprint/Widget_Dialogue.Widget_Dialogue_C|SetNPCDia _answers_5 (Variables|Default|GetNPCAmmoS))
                          (Variables|Default|SetUpdateArray 2)
                          (goto _label_5))))
                    (elif (== (Variables|Default|GetAnswerInt) 2)
                      (Variables|/Game/SpaceState/Blueprint/Widget_Dialogue.Widget_Dialogue_C|SetNPCDia _answers_5 (Variables|Default|GetNPCAmmo))
                      (Variables|Default|SetUpdateArray 4)
                      (Variables|Default|SetButtonText (Utilities|Select :Index (Variables|Default|GetUpdateArray) :Option%200 (Utilities|Array|MakeArray (Variables|Default|GetA1) (Variables|Default|GetA2) (Variables|Default|GetA3)) :Option%201 (Utilities|Array|MakeArray (Variables|Default|Getphp1) (Variables|Default|Getphp2) (Variables|Default|Getphp3)) :Option%202 (Utilities|Array|MakeArray (Variables|Default|GetPQ2a) (Variables|Default|GetPQ2b) (Variables|Default|Getpmore)) :Option%203 (Utilities|Array|MakeArray (Variables|Default|GetPWeap1) (Variables|Default|GetPweap2) (Variables|Default|GetPweap3)) :Option%204 (Utilities|Array|MakeArray (Variables|Default|GetPflamerammo) (Variables|Default|GetPpowercells) (Variables|Default|Getpmore2)) :Option%205 (Utilities|Array|MakeArray (Variables|Default|GetQ_G_0) (Variables|Default|GetQ_G_1) (Variables|Default|GetQ_G_2)) :Option%206 (Utilities|Array|MakeArray (Variables|Default|GetQ_H_0) (Variables|Default|GetQ_H_1) (Variables|Default|GetQ_H_2)) :Option%207 (Utilities|Array|MakeArray (Variables|Default|GetQ_I_0)) :Option%208 (Utilities|Array|MakeArray (Variables|Default|GetQ_J_0)) :Option%209 (Utilities|Array|MakeArray (Variables|Default|GetQ_K_0)) :Option%2010 (Utilities|Array|MakeArray (Variables|Default|GetQ_L_0)) :Option%2011 (Utilities|Array|MakeArray (Variables|Default|GetQ_M_0)) :Option%2012 (Utilities|Array|MakeArray (Variables|Default|GetQ_E_0) (Variables|Default|GetQ_E_1) (Variables|Default|GetQ_E_2)) :Option%2013 (Utilities|Array|MakeArray (Variables|Default|GetQW) (Variables|Default|GetQW1) (Variables|Default|Getnext)))))))
                (else
                  ;[1 1 1] Weapons
                  (if (== (Variables|Default|GetUpdateArray) 3)
                    (if (== (Variables|Default|GetAnswerInt) 0)
                      (bind _asbp_dude_7 (Utilities|Casting|CastToBP_Dude (Game|GetPlayerCharacter 0)))
                      (if (< (Variables|/Game/SpaceState/Blueprint/BP_Dude/BP_Dude.BP_Dude_C|GetCharCredits _asbp_dude_7) 500)
                        (Variables|/Game/SpaceState/Blueprint/Widget_Dialogue.Widget_Dialogue_C|SetNPCDia _answers_6 (Variables|Default|GetNPCNotEnoughCreds))
                        (Variables|Default|SetUpdateArray 0)
                        (goto _label)
                        (elif (>= (Variables|/Game/SpaceState/Blueprint/BP_Dude/BP_Dude.BP_Dude_C|GetMaxWeaps _asbp_dude_7) 3)
                          (Variables|/Game/SpaceState/Blueprint/Widget_Dialogue.Widget_Dialogue_C|SetNPCDia _answers_6 (Variables|Default|GetNWeapHave))
                          (Variables|Default|SetUpdateArray 0)
                          (goto _label)
                          (else
                            (Default|Creditsystem _asbp_dude_7 -500)
                            (Variables|/Game/SpaceState/Blueprint/BP_Dude/BP_Dude.BP_Dude_C|SetMaxWeaps _asbp_dude_7 3)
                            (Variables|/Game/SpaceState/Blueprint/Widget_Dialogue.Widget_Dialogue_C|SetNPCDia _answers_6 (Variables|Default|GetNShotgun))
                            (Variables|Default|SetUpdateArray 0)
                            (goto _label))))
                      (elif (== (Variables|Default|GetAnswerInt) 1)
                        (Variables|/Game/SpaceState/Blueprint/Widget_Dialogue.Widget_Dialogue_C|SetNPCDia _answers_6 (Variables|Default|GetNFlamer))
                        (Variables|Default|SetUpdateArray 0)
                        (goto _label)))
                    (else
                      ;[1 1 1] Ammo2
                      (if (== (Variables|Default|GetUpdateArray) 4)
                        (if (== (Variables|Default|GetAnswerInt) 0)
                          (bind _asbp_dude_8 (Utilities|Casting|CastToBP_Dude (Game|GetPlayerCharacter 0)))
                          (if (< (Variables|/Game/SpaceState/Blueprint/BP_Dude/BP_Dude.BP_Dude_C|GetCharCredits _asbp_dude_8) 100)
                            (Variables|/Game/SpaceState/Blueprint/Widget_Dialogue.Widget_Dialogue_C|SetNPCDia _answers_3 (Variables|Default|GetNPCNotEnoughCreds))
                            (Variables|Default|SetUpdateArray 4)
                            (goto _label)
                            (elif (>= (Utilities|Array|Get(acopy) (Variables|/Game/SpaceState/Blueprint/BP_Dude/BP_Dude.BP_Dude_C|GetBulletCountsArray _asbp_dude_8) 4) (Variables|/Game/SpaceState/Blueprint/BP_Dude/BP_Dude.BP_Dude_C|GetMaxFuel _asbp_dude_8))
                              (Variables|/Game/SpaceState/Blueprint/Widget_Dialogue.Widget_Dialogue_C|SetNPCDia _answers_3 (Variables|Default|GetNPCFull))
                              (Variables|Default|SetUpdateArray 4)
                              (goto _label)
                              (else
                                (Default|FuelSystem _asbp_dude_8 100)
                                (Default|Creditsystem _asbp_dude_8 -100)
                                (Variables|/Game/SpaceState/Blueprint/Widget_Dialogue.Widget_Dialogue_C|SetNPCDia _answers_4 (Variables|Default|GetNPCAmmoF))
                                (Variables|Default|SetUpdateArray 4)
                                (goto _label))))
                          (elif (== (Variables|Default|GetAnswerInt) 1)
                            (bind _asbp_dude_9 (Utilities|Casting|CastToBP_Dude (Game|GetPlayerCharacter 0)))
                            (if (< (Variables|/Game/SpaceState/Blueprint/BP_Dude/BP_Dude.BP_Dude_C|GetCharCredits _asbp_dude_9) 100)
                              (Variables|/Game/SpaceState/Blueprint/Widget_Dialogue.Widget_Dialogue_C|SetNPCDia _answers_3 (Variables|Default|GetNPCNotEnoughCreds))
                              (Variables|Default|SetUpdateArray 4)
                              (goto _label)
                              (elif (>= (Utilities|Array|Get(acopy) (Variables|/Game/SpaceState/Blueprint/BP_Dude/BP_Dude.BP_Dude_C|GetBulletCountsArray _asbp_dude_9) 3) (Variables|/Game/SpaceState/Blueprint/BP_Dude/BP_Dude.BP_Dude_C|GetMaxCells _asbp_dude_9))
                                (Variables|/Game/SpaceState/Blueprint/Widget_Dialogue.Widget_Dialogue_C|SetNPCDia _answers_3 (Variables|Default|GetNPCFull))
                                (Variables|Default|SetUpdateArray 4)
                                (goto _label)
                                (else
                                  (Default|CellSystem _asbp_dude_9 1)
                                  (Default|Creditsystem _asbp_dude_9 -100)
                                  (Variables|/Game/SpaceState/Blueprint/Widget_Dialogue.Widget_Dialogue_C|SetNPCDia _answers_4 (Variables|Default|GetNPCAmmoRG))
                                  (Variables|Default|SetUpdateArray 4)
                                  (goto _label))))
                            (elif (== (Variables|Default|GetAnswerInt) 2)
                              (Variables|/Game/SpaceState/Blueprint/Widget_Dialogue.Widget_Dialogue_C|SetNPCDia _answers_4 (Variables|Default|GetNPCAmmo))
                              (Variables|Default|SetUpdateArray 2)
                              (goto _label))))))))))))))))

(event Custom|Answer3
  (bind _returnvalue (Game|GetPlayerCharacter 0))
  (bind _answers (Variables|Default|GetAnswers))
  (bind _answers_2 (Variables|Default|GetAnswers))
  (bind _answers_3 (Variables|Default|GetAnswers))
  (bind _answers_4 (Variables|Default|GetAnswers))
  (bind _answers_5 (Variables|Default|GetAnswers))
  (bind _answers_6 (Variables|Default|GetAnswers))
  (bind _nhp1 (Variables|Default|GetNhp1))
  (bind _answers_7 (Variables|Default|GetAnswers))
  ;[1 1 1] Input
  (Variables|Default|SetAnswerInt 2)
  ;[1 1 1] FirstTime
  (if (== (Variables|Default|GetUpdateArray) 5)
    (if (== (Variables|Default|GetAnswerInt) 0)
      (Variables|/Game/SpaceState/Blueprint/Widget_Dialogue.Widget_Dialogue_C|SetNPCDia _answers (Variables|Default|Getnext))
      (bind _asbp_dude (Utilities|Casting|CastToBP_Dude (Game|GetPlayerCharacter 0)))
      (Variables|/Game/SpaceState/Blueprint/BP_Dude/BP_Dude.BP_Dude_C|SetMainQuest _asbp_dude 2)
      (Variables|Default|SetUpdateArray 6)
      (Variables|Default|SetButtonText (Utilities|Select :Index (Variables|Default|GetUpdateArray) :Option%200 (Utilities|Array|MakeArray (Variables|Default|GetA1) (Variables|Default|GetA2) (Variables|Default|GetA3)) :Option%201 (Utilities|Array|MakeArray (Variables|Default|Getphp1) (Variables|Default|Getphp2) (Variables|Default|Getphp3)) :Option%202 (Utilities|Array|MakeArray (Variables|Default|GetPQ2a) (Variables|Default|GetPQ2b) (Variables|Default|Getpmore)) :Option%203 (Utilities|Array|MakeArray (Variables|Default|GetPWeap1) (Variables|Default|GetPweap2) (Variables|Default|GetPweap3)) :Option%204 (Utilities|Array|MakeArray (Variables|Default|GetPflamerammo) (Variables|Default|GetPpowercells) (Variables|Default|Getpmore2)) :Option%205 (Utilities|Array|MakeArray (Variables|Default|GetQ_G_0) (Variables|Default|GetQ_G_1) (Variables|Default|GetQ_G_2)) :Option%206 (Utilities|Array|MakeArray (Variables|Default|GetQ_H_0) (Variables|Default|GetQ_H_1) (Variables|Default|GetQ_H_2)) :Option%207 (Utilities|Array|MakeArray (Variables|Default|GetQ_I_0)) :Option%208 (Utilities|Array|MakeArray (Variables|Default|GetQ_J_0)) :Option%209 (Utilities|Array|MakeArray (Variables|Default|GetQ_K_0)) :Option%2010 (Utilities|Array|MakeArray (Variables|Default|GetQ_L_0)) :Option%2011 (Utilities|Array|MakeArray (Variables|Default|GetQ_M_0)) :Option%2012 (Utilities|Array|MakeArray (Variables|Default|GetQ_E_0) (Variables|Default|GetQ_E_1) (Variables|Default|GetQ_E_2)) :Option%2013 (Utilities|Array|MakeArray (Variables|Default|GetQW) (Variables|Default|GetQW1) (Variables|Default|Getnext))) :!label _label)
      (elif (== (Variables|Default|GetAnswerInt) 1)
        (Variables|/Game/SpaceState/Blueprint/Widget_Dialogue.Widget_Dialogue_C|SetNPCDia _answers "")
        (Variables|Default|SetUpdateArray 2)
        (goto _label)
        (elif (== (Variables|Default|GetAnswerInt) 2)
          (Variables|/Game/SpaceState/Blueprint/Widget_Dialogue.Widget_Dialogue_C|SetNPCDia _answers "")
          (Variables|Default|SetUpdateArray 3)
          (goto _label))))
    (else
      ;[1 1 1] What would you like?
      (if (== (Variables|Default|GetUpdateArray) 0)
        (if (== (Variables|Default|GetAnswerInt) 0)
          (Variables|/Game/SpaceState/Blueprint/Widget_Dialogue.Widget_Dialogue_C|SetNPCDia _answers_7 (Variables|Default|GetNHP))
          (Variables|Default|SetUpdateArray 1)
          (Variables|Default|SetButtonText (Utilities|Select :Index (Variables|Default|GetUpdateArray) :Option%200 (Utilities|Array|MakeArray (Variables|Default|GetA1) (Variables|Default|GetA2) (Variables|Default|GetA3)) :Option%201 (Utilities|Array|MakeArray (Variables|Default|Getphp1) (Variables|Default|Getphp2) (Variables|Default|Getphp3)) :Option%202 (Utilities|Array|MakeArray (Variables|Default|GetPQ2a) (Variables|Default|GetPQ2b) (Variables|Default|Getpmore)) :Option%203 (Utilities|Array|MakeArray (Variables|Default|GetPWeap1) (Variables|Default|GetPweap2) (Variables|Default|GetPweap3)) :Option%204 (Utilities|Array|MakeArray (Variables|Default|GetPflamerammo) (Variables|Default|GetPpowercells) (Variables|Default|Getpmore2)) :Option%205 (Utilities|Array|MakeArray (Variables|Default|GetQ_G_0) (Variables|Default|GetQ_G_1) (Variables|Default|GetQ_G_2)) :Option%206 (Utilities|Array|MakeArray (Variables|Default|GetQ_H_0) (Variables|Default|GetQ_H_1) (Variables|Default|GetQ_H_2)) :Option%207 (Utilities|Array|MakeArray (Variables|Default|GetQ_I_0)) :Option%208 (Utilities|Array|MakeArray (Variables|Default|GetQ_J_0)) :Option%209 (Utilities|Array|MakeArray (Variables|Default|GetQ_K_0)) :Option%2010 (Utilities|Array|MakeArray (Variables|Default|GetQ_L_0)) :Option%2011 (Utilities|Array|MakeArray (Variables|Default|GetQ_M_0)) :Option%2012 (Utilities|Array|MakeArray (Variables|Default|GetQ_E_0) (Variables|Default|GetQ_E_1) (Variables|Default|GetQ_E_2)) :Option%2013 (Utilities|Array|MakeArray (Variables|Default|GetQW) (Variables|Default|GetQW1) (Variables|Default|Getnext))) :!label _label_2)
          (elif (== (Variables|Default|GetAnswerInt) 1)
            (Variables|/Game/SpaceState/Blueprint/Widget_Dialogue.Widget_Dialogue_C|SetNPCDia _answers_7 (Variables|Default|GetNPCAmmo))
            (Variables|Default|SetUpdateArray 2)
            (goto _label_2)
            (elif (== (Variables|Default|GetAnswerInt) 2)
              (Variables|/Game/SpaceState/Blueprint/Widget_Dialogue.Widget_Dialogue_C|SetNPCDia _answers_7 (Variables|Default|GetNPCWeapons))
              (Variables|Default|SetUpdateArray 3)
              (goto _label_2))))
        (else
          ;[1 1 1] HP
          (if (== (Variables|Default|GetUpdateArray) 1)
            (if (== (Variables|Default|GetAnswerInt) 0)
              (bind _asbp_dude_2 (Utilities|Casting|CastToBP_Dude _returnvalue))
              (if (> (Variables|/Game/SpaceState/Blueprint/BP_Dude/BP_Dude.BP_Dude_C|GetCharCredits _asbp_dude_2) 100)
                (if (>= (Variables|/Game/SpaceState/Blueprint/BP_Dude/BP_Dude.BP_Dude_C|GetHealth%20Current _asbp_dude_2) 1.0)
                  (Variables|/Game/SpaceState/Blueprint/Widget_Dialogue.Widget_Dialogue_C|SetNPCDia _answers_2 (Variables|Default|GetNFullHP) :!label _label_3)
                  (Variables|Default|SetUpdateArray 0)
                  (goto _label_2)
                  (else
                    (Default|Creditsystem _asbp_dude_2 -100)
                    (Variables|/Game/SpaceState/Blueprint/BP_Dude/BP_Dude.BP_Dude_C|SetHealth%20Current _asbp_dude_2 (+ (Variables|/Game/SpaceState/Blueprint/BP_Dude/BP_Dude.BP_Dude_C|GetHealth%20Current _asbp_dude_2) 0.25))
                    (Variables|/Game/SpaceState/Blueprint/Widget_Dialogue.Widget_Dialogue_C|SetNPCDia _answers_2 _nhp1)
                    (Variables|Default|SetUpdateArray 0)
                    (goto _label_2)))
                (else
                  (Variables|/Game/SpaceState/Blueprint/Widget_Dialogue.Widget_Dialogue_C|SetNPCDia _answers_2 (Variables|Default|GetNPCNotEnoughCreds) :!label _label_4)
                  (Variables|Default|SetUpdateArray 0)
                  (goto _label_2)))
              (elif (== (Variables|Default|GetAnswerInt) 1)
                (bind _asbp_dude_3 (Utilities|Casting|CastToBP_Dude _returnvalue))
                (if (> (Variables|/Game/SpaceState/Blueprint/BP_Dude/BP_Dude.BP_Dude_C|GetCharCredits _asbp_dude_3) 200)
                  (if (>= (Variables|/Game/SpaceState/Blueprint/BP_Dude/BP_Dude.BP_Dude_C|GetHealth%20Current _asbp_dude_3) 0.75)
                    (goto _label_3)
                    (else
                      (Default|Creditsystem _asbp_dude_3 -200)
                      (Variables|/Game/SpaceState/Blueprint/BP_Dude/BP_Dude.BP_Dude_C|SetHealth%20Current _asbp_dude_3 (+ (Variables|/Game/SpaceState/Blueprint/BP_Dude/BP_Dude.BP_Dude_C|GetHealth%20Current _asbp_dude_3) 0.5))
                      (Variables|/Game/SpaceState/Blueprint/Widget_Dialogue.Widget_Dialogue_C|SetNPCDia _answers_2 _nhp1)
                      (Variables|Default|SetUpdateArray 0)
                      ;[1 1 1] Set UMG Text
                      (Variables|Default|SetButtonText (Utilities|Select :Index (Variables|Default|GetUpdateArray) :Option%200 (Utilities|Array|MakeArray (Variables|Default|GetA1) (Variables|Default|GetA2) (Variables|Default|GetA3)) :Option%201 (Utilities|Array|MakeArray (Variables|Default|Getphp1) (Variables|Default|Getphp2) (Variables|Default|Getphp3)) :Option%202 (Utilities|Array|MakeArray (Variables|Default|GetPQ2a) (Variables|Default|GetPQ2b) (Variables|Default|Getpmore)) :Option%203 (Utilities|Array|MakeArray (Variables|Default|GetPWeap1) (Variables|Default|GetPweap2) (Variables|Default|GetPweap3)) :Option%204 (Utilities|Array|MakeArray (Variables|Default|GetPflamerammo) (Variables|Default|GetPpowercells) (Variables|Default|Getpmore2)) :Option%205 (Utilities|Array|MakeArray (Variables|Default|GetQ_G_0) (Variables|Default|GetQ_G_1) (Variables|Default|GetQ_G_2)) :Option%206 (Utilities|Array|MakeArray (Variables|Default|GetQ_H_0) (Variables|Default|GetQ_H_1) (Variables|Default|GetQ_H_2)) :Option%207 (Utilities|Array|MakeArray (Variables|Default|GetQ_I_0)) :Option%208 (Utilities|Array|MakeArray (Variables|Default|GetQ_J_0)) :Option%209 (Utilities|Array|MakeArray (Variables|Default|GetQ_K_0)) :Option%2010 (Utilities|Array|MakeArray (Variables|Default|GetQ_L_0)) :Option%2011 (Utilities|Array|MakeArray (Variables|Default|GetQ_M_0)) :Option%2012 (Utilities|Array|MakeArray (Variables|Default|GetQ_E_0) (Variables|Default|GetQ_E_1) (Variables|Default|GetQ_E_2)) :Option%2013 (Utilities|Array|MakeArray (Variables|Default|GetQW) (Variables|Default|GetQW1) (Variables|Default|Getnext))) :!label _label_5)))
                  (else
                    (goto _label_4)))
                (elif (== (Variables|Default|GetAnswerInt) 2)
                  (bind _asbp_dude_4 (Utilities|Casting|CastToBP_Dude _returnvalue))
                  (if (> (Variables|/Game/SpaceState/Blueprint/BP_Dude/BP_Dude.BP_Dude_C|GetCharCredits _asbp_dude_4) 300)
                    (if (>= (Variables|/Game/SpaceState/Blueprint/BP_Dude/BP_Dude.BP_Dude_C|GetHealth%20Current _asbp_dude_4) 0.5)
                      (goto _label_3)
                      (else
                        (Default|Creditsystem _asbp_dude_4 -300)
                        (Variables|/Game/SpaceState/Blueprint/BP_Dude/BP_Dude.BP_Dude_C|SetHealth%20Current _asbp_dude_4 (+ (Variables|/Game/SpaceState/Blueprint/BP_Dude/BP_Dude.BP_Dude_C|GetHealth%20Current _asbp_dude_4) 1.0))
                        (Variables|/Game/SpaceState/Blueprint/Widget_Dialogue.Widget_Dialogue_C|SetNPCDia _answers_2 (Variables|Default|GetNhp2))
                        (Variables|Default|SetUpdateArray 0)
                        (goto _label_5)))
                    (else
                      (goto _label_4))))))
            (else
              ;[1 1 1] Ammo1
              (if (== (Variables|Default|GetUpdateArray) 2)
                (if (== (Variables|Default|GetAnswerInt) 0)
                  (bind _asbp_dude_5 (Utilities|Casting|CastToBP_Dude (Game|GetPlayerCharacter 0)))
                  (if (< (Variables|/Game/SpaceState/Blueprint/BP_Dude/BP_Dude.BP_Dude_C|GetCharCredits _asbp_dude_5) 100)
                    (Variables|/Game/SpaceState/Blueprint/Widget_Dialogue.Widget_Dialogue_C|SetNPCDia _answers_5 (Variables|Default|GetNPCNotEnoughCreds))
                    (Variables|Default|SetUpdateArray 2)
                    (goto _label_5)
                    (elif (>= (Utilities|Array|Get(acopy) (Variables|/Game/SpaceState/Blueprint/BP_Dude/BP_Dude.BP_Dude_C|GetBulletCountsArray _asbp_dude_5) 1) (Variables|/Game/SpaceState/Blueprint/BP_Dude/BP_Dude.BP_Dude_C|GetMaxBullets _asbp_dude_5))
                      (Variables|/Game/SpaceState/Blueprint/Widget_Dialogue.Widget_Dialogue_C|SetNPCDia _answers_5 (Variables|Default|GetNPCFull))
                      (Variables|Default|SetUpdateArray 2)
                      (goto _label_5)
                      (else
                        (Default|BulletSystem _asbp_dude_5 10)
                        (Default|Creditsystem _asbp_dude_5 -100)
                        (Variables|/Game/SpaceState/Blueprint/Widget_Dialogue.Widget_Dialogue_C|SetNPCDia _answers_5 (Variables|Default|GetNPCAmmoR))
                        (Variables|Default|SetUpdateArray 2)
                        (goto _label_5))))
                  (elif (== (Variables|Default|GetAnswerInt) 1)
                    (bind _asbp_dude_6 (Utilities|Casting|CastToBP_Dude (Game|GetPlayerCharacter 0)))
                    (if (< (Variables|/Game/SpaceState/Blueprint/BP_Dude/BP_Dude.BP_Dude_C|GetCharCredits _asbp_dude_6) 100)
                      (Variables|/Game/SpaceState/Blueprint/Widget_Dialogue.Widget_Dialogue_C|SetNPCDia _answers_5 (Variables|Default|GetNPCNotEnoughCreds))
                      (Variables|Default|SetUpdateArray 2)
                      (goto _label_5)
                      (elif (>= (Utilities|Array|Get(acopy) (Variables|/Game/SpaceState/Blueprint/BP_Dude/BP_Dude.BP_Dude_C|GetBulletCountsArray _asbp_dude_6) 2) (Variables|/Game/SpaceState/Blueprint/BP_Dude/BP_Dude.BP_Dude_C|GetMaxShells _asbp_dude_6))
                        (Variables|/Game/SpaceState/Blueprint/Widget_Dialogue.Widget_Dialogue_C|SetNPCDia _answers_5 (Variables|Default|GetNPCFull))
                        (Variables|Default|SetUpdateArray 2)
                        (goto _label_5)
                        (else
                          (Default|ShellSystem _asbp_dude_6 10)
                          (Default|Creditsystem _asbp_dude_6 -100)
                          (Variables|/Game/SpaceState/Blueprint/Widget_Dialogue.Widget_Dialogue_C|SetNPCDia _answers_5 (Variables|Default|GetNPCAmmoS))
                          (Variables|Default|SetUpdateArray 2)
                          (goto _label_5))))
                    (elif (== (Variables|Default|GetAnswerInt) 2)
                      (Variables|/Game/SpaceState/Blueprint/Widget_Dialogue.Widget_Dialogue_C|SetNPCDia _answers_5 (Variables|Default|GetNPCAmmo))
                      (Variables|Default|SetUpdateArray 4)
                      (Variables|Default|SetButtonText (Utilities|Select :Index (Variables|Default|GetUpdateArray) :Option%200 (Utilities|Array|MakeArray (Variables|Default|GetA1) (Variables|Default|GetA2) (Variables|Default|GetA3)) :Option%201 (Utilities|Array|MakeArray (Variables|Default|Getphp1) (Variables|Default|Getphp2) (Variables|Default|Getphp3)) :Option%202 (Utilities|Array|MakeArray (Variables|Default|GetPQ2a) (Variables|Default|GetPQ2b) (Variables|Default|Getpmore)) :Option%203 (Utilities|Array|MakeArray (Variables|Default|GetPWeap1) (Variables|Default|GetPweap2) (Variables|Default|GetPweap3)) :Option%204 (Utilities|Array|MakeArray (Variables|Default|GetPflamerammo) (Variables|Default|GetPpowercells) (Variables|Default|Getpmore2)) :Option%205 (Utilities|Array|MakeArray (Variables|Default|GetQ_G_0) (Variables|Default|GetQ_G_1) (Variables|Default|GetQ_G_2)) :Option%206 (Utilities|Array|MakeArray (Variables|Default|GetQ_H_0) (Variables|Default|GetQ_H_1) (Variables|Default|GetQ_H_2)) :Option%207 (Utilities|Array|MakeArray (Variables|Default|GetQ_I_0)) :Option%208 (Utilities|Array|MakeArray (Variables|Default|GetQ_J_0)) :Option%209 (Utilities|Array|MakeArray (Variables|Default|GetQ_K_0)) :Option%2010 (Utilities|Array|MakeArray (Variables|Default|GetQ_L_0)) :Option%2011 (Utilities|Array|MakeArray (Variables|Default|GetQ_M_0)) :Option%2012 (Utilities|Array|MakeArray (Variables|Default|GetQ_E_0) (Variables|Default|GetQ_E_1) (Variables|Default|GetQ_E_2)) :Option%2013 (Utilities|Array|MakeArray (Variables|Default|GetQW) (Variables|Default|GetQW1) (Variables|Default|Getnext)))))))
                (else
                  ;[1 1 1] Weapons
                  (if (== (Variables|Default|GetUpdateArray) 3)
                    (if (== (Variables|Default|GetAnswerInt) 0)
                      (bind _asbp_dude_7 (Utilities|Casting|CastToBP_Dude (Game|GetPlayerCharacter 0)))
                      (if (< (Variables|/Game/SpaceState/Blueprint/BP_Dude/BP_Dude.BP_Dude_C|GetCharCredits _asbp_dude_7) 500)
                        (Variables|/Game/SpaceState/Blueprint/Widget_Dialogue.Widget_Dialogue_C|SetNPCDia _answers_6 (Variables|Default|GetNPCNotEnoughCreds))
                        (Variables|Default|SetUpdateArray 0)
                        (goto _label)
                        (elif (>= (Variables|/Game/SpaceState/Blueprint/BP_Dude/BP_Dude.BP_Dude_C|GetMaxWeaps _asbp_dude_7) 3)
                          (Variables|/Game/SpaceState/Blueprint/Widget_Dialogue.Widget_Dialogue_C|SetNPCDia _answers_6 (Variables|Default|GetNWeapHave))
                          (Variables|Default|SetUpdateArray 0)
                          (goto _label)
                          (else
                            (Default|Creditsystem _asbp_dude_7 -500)
                            (Variables|/Game/SpaceState/Blueprint/BP_Dude/BP_Dude.BP_Dude_C|SetMaxWeaps _asbp_dude_7 3)
                            (Variables|/Game/SpaceState/Blueprint/Widget_Dialogue.Widget_Dialogue_C|SetNPCDia _answers_6 (Variables|Default|GetNShotgun))
                            (Variables|Default|SetUpdateArray 0)
                            (goto _label))))
                      (elif (== (Variables|Default|GetAnswerInt) 1)
                        (Variables|/Game/SpaceState/Blueprint/Widget_Dialogue.Widget_Dialogue_C|SetNPCDia _answers_6 (Variables|Default|GetNFlamer))
                        (Variables|Default|SetUpdateArray 0)
                        (goto _label)))
                    (else
                      ;[1 1 1] Ammo2
                      (if (== (Variables|Default|GetUpdateArray) 4)
                        (if (== (Variables|Default|GetAnswerInt) 0)
                          (bind _asbp_dude_8 (Utilities|Casting|CastToBP_Dude (Game|GetPlayerCharacter 0)))
                          (if (< (Variables|/Game/SpaceState/Blueprint/BP_Dude/BP_Dude.BP_Dude_C|GetCharCredits _asbp_dude_8) 100)
                            (Variables|/Game/SpaceState/Blueprint/Widget_Dialogue.Widget_Dialogue_C|SetNPCDia _answers_3 (Variables|Default|GetNPCNotEnoughCreds))
                            (Variables|Default|SetUpdateArray 4)
                            (goto _label)
                            (elif (>= (Utilities|Array|Get(acopy) (Variables|/Game/SpaceState/Blueprint/BP_Dude/BP_Dude.BP_Dude_C|GetBulletCountsArray _asbp_dude_8) 4) (Variables|/Game/SpaceState/Blueprint/BP_Dude/BP_Dude.BP_Dude_C|GetMaxFuel _asbp_dude_8))
                              (Variables|/Game/SpaceState/Blueprint/Widget_Dialogue.Widget_Dialogue_C|SetNPCDia _answers_3 (Variables|Default|GetNPCFull))
                              (Variables|Default|SetUpdateArray 4)
                              (goto _label)
                              (else
                                (Default|FuelSystem _asbp_dude_8 100)
                                (Default|Creditsystem _asbp_dude_8 -100)
                                (Variables|/Game/SpaceState/Blueprint/Widget_Dialogue.Widget_Dialogue_C|SetNPCDia _answers_4 (Variables|Default|GetNPCAmmoF))
                                (Variables|Default|SetUpdateArray 4)
                                (goto _label))))
                          (elif (== (Variables|Default|GetAnswerInt) 1)
                            (bind _asbp_dude_9 (Utilities|Casting|CastToBP_Dude (Game|GetPlayerCharacter 0)))
                            (if (< (Variables|/Game/SpaceState/Blueprint/BP_Dude/BP_Dude.BP_Dude_C|GetCharCredits _asbp_dude_9) 100)
                              (Variables|/Game/SpaceState/Blueprint/Widget_Dialogue.Widget_Dialogue_C|SetNPCDia _answers_3 (Variables|Default|GetNPCNotEnoughCreds))
                              (Variables|Default|SetUpdateArray 4)
                              (goto _label)
                              (elif (>= (Utilities|Array|Get(acopy) (Variables|/Game/SpaceState/Blueprint/BP_Dude/BP_Dude.BP_Dude_C|GetBulletCountsArray _asbp_dude_9) 3) (Variables|/Game/SpaceState/Blueprint/BP_Dude/BP_Dude.BP_Dude_C|GetMaxCells _asbp_dude_9))
                                (Variables|/Game/SpaceState/Blueprint/Widget_Dialogue.Widget_Dialogue_C|SetNPCDia _answers_3 (Variables|Default|GetNPCFull))
                                (Variables|Default|SetUpdateArray 4)
                                (goto _label)
                                (else
                                  (Default|CellSystem _asbp_dude_9 1)
                                  (Default|Creditsystem _asbp_dude_9 -100)
                                  (Variables|/Game/SpaceState/Blueprint/Widget_Dialogue.Widget_Dialogue_C|SetNPCDia _answers_4 (Variables|Default|GetNPCAmmoRG))
                                  (Variables|Default|SetUpdateArray 4)
                                  (goto _label))))
                            (elif (== (Variables|Default|GetAnswerInt) 2)
                              (Variables|/Game/SpaceState/Blueprint/Widget_Dialogue.Widget_Dialogue_C|SetNPCDia _answers_4 (Variables|Default|GetNPCAmmo))
                              (Variables|Default|SetUpdateArray 2)
                              (goto _label))))))))))))))))

(event Collision|EventActorBeginOverlap
  (params (OtherActor :type Actor%20Object%20Reference))
  (bind _returnvalue (Game|GetPlayerController 0))
  ;[1 1 1] Start/End Encounter, Enable/disable input
  (bind _asbp_dude (Utilities|Casting|CastToBP_Dude OtherActor))
  (Input|EnableInput _asbp_dude (Game|GetPlayerController 0))
  (Rendering|Components|TextRender|SetText (Variables|Components|GetTextRender) (Variables|Default|GetR_Contact))
  (bind _returnvalue_2 (UserInterface|CreateWidget "/Game/SpaceState/Blueprint/Widget_Dialogue.Widget_Dialogue_C" _returnvalue))
  (bind _output_get (Variables|Default|SetAnswers _returnvalue_2))
  (if (== (Variables|/Game/SpaceState/Blueprint/BP_Dude/BP_Dude.BP_Dude_C|GetMainQuest _asbp_dude) 5)
    (Variables|Default|SetUpdateArray 0))
  (UserInterface|Viewport|AddtoViewport _output_get 0)
  (if (== (Variables|/Game/SpaceState/Blueprint/BP_Dude/BP_Dude.BP_Dude_C|GetMainQuest _asbp_dude) 5)
    (Variables|/Game/SpaceState/Blueprint/Widget_Dialogue.Widget_Dialogue_C|SetNPCDia _output_get (Variables|Default|Get2))
    (else
      (Variables|/Game/SpaceState/Blueprint/Widget_Dialogue.Widget_Dialogue_C|SetNPCDia _output_get (Variables|Default|GetWelcomeText))))
  (bind _asplayer_controller (Utilities|Casting|CastToPlayerController _returnvalue))
  (Variables|/Script/Engine.PlayerController|SetbShowMouseCursor _asplayer_controller true)
  (Variables|Default|SetButtonText (Utilities|Select :Index (Variables|Default|GetUpdateArray) :Option%200 (Utilities|Array|MakeArray (Variables|Default|GetA1) (Variables|Default|GetA2) (Variables|Default|GetA3)) :Option%201 (Utilities|Array|MakeArray (Variables|Default|Getphp1) (Variables|Default|Getphp2) (Variables|Default|Getphp3)) :Option%202 (Utilities|Array|MakeArray (Variables|Default|GetPQ2a) (Variables|Default|GetPQ2b) (Variables|Default|Getpmore)) :Option%203 (Utilities|Array|MakeArray (Variables|Default|GetPWeap1) (Variables|Default|GetPweap2) (Variables|Default|GetPweap3)) :Option%204 (Utilities|Array|MakeArray (Variables|Default|GetPflamerammo) (Variables|Default|GetPpowercells) (Variables|Default|Getpmore2)) :Option%205 (Utilities|Array|MakeArray (Variables|Default|GetQ_G_0) (Variables|Default|GetQ_G_1) (Variables|Default|GetQ_G_2)) :Option%206 (Utilities|Array|MakeArray (Variables|Default|GetQ_H_0) (Variables|Default|GetQ_H_1) (Variables|Default|GetQ_H_2)) :Option%207 (Utilities|Array|MakeArray (Variables|Default|GetQ_I_0)) :Option%208 (Utilities|Array|MakeArray (Variables|Default|GetQ_J_0)) :Option%209 (Utilities|Array|MakeArray (Variables|Default|GetQ_K_0)) :Option%2010 (Utilities|Array|MakeArray (Variables|Default|GetQ_L_0)) :Option%2011 (Utilities|Array|MakeArray (Variables|Default|GetQ_M_0)) :Option%2012 (Utilities|Array|MakeArray (Variables|Default|GetQ_E_0) (Variables|Default|GetQ_E_1) (Variables|Default|GetQ_E_2)) :Option%2013 (Utilities|Array|MakeArray (Variables|Default|GetQW) (Variables|Default|GetQW1) (Variables|Default|Getnext)))))

(event Collision|EventActorEndOverlap
  (params (OtherActor :type Actor%20Object%20Reference))
  ;[1 1 1] Start/End Encounter, Enable/disable input
  (Utilities|Casting|CastToBP_Dude OtherActor)
  (Input|DisableInput (Game|GetPlayerController 0))
  (Rendering|Components|TextRender|SetText (Variables|Components|GetTextRender) (Variables|Default|GetR_Leaving))
  (if (== (Variables|/Game/SpaceState/Blueprint/BP_Dude/BP_Dude.BP_Dude_C|GetMainQuest (stale Collision|EventActorBeginOverlap _asbp_dude)) 5)
    (Variables|Default|SetUpdateArray 0)
    (else
      (Variables|Default|SetUpdateArray 0)))
  (Widget|RemovefromParent (stale Collision|EventActorBeginOverlap _output_get))
  (bind _asplayer_controller (Utilities|Casting|CastToPlayerController (Game|GetPlayerController 0)))
  (Variables|/Script/Engine.PlayerController|SetbShowMouseCursor _asplayer_controller false))

(fn ConstructionScript)