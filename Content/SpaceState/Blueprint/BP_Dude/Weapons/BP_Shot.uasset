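; BP_Shot is a Paper2D flipbook projectile that damages players and enemies, with its launch speed set from BulletSpeed at construction.
; On hit it plays a ricochet, swaps to an explosion flipbook and destroys itself after a short delay.
; A DoOnce gates target handling: BP_Dude takes damage only if Kills is set, AI_Enemy always does, and BP_MasterBad is damaged or stunned by that flag.
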(event Custom|Hit
  (params (NewParam :type Boolean))
  (Sprite|SetFlipbook (Variables|Default|GetPaperFlipbook) "/Game/SpaceState/Sprites/Weapons/A_Explo.A_Explo")
  (Utilities|FlowControl|Delay 0.2)
  (Actor|DestroyActor))

(event Custom|Sound
  (Utilities|FlowControl|DoOnce false
    (:Completed
      (Audio|SpawnSoundatLocation "/Game/SpaceState/Allsounds/Sounds/Ricochet.Ricochet" (stale Collision|EventHit HitLocation)))))

(event Custom|HitSound
  (Utilities|FlowControl|DoOnce false
    (:Completed
      (Audio|SpawnSoundatLocation "/Game/SpaceState/Allsounds/Sounds/Ricochet2.Ricochet2" (stale Collision|EventHit HitLocation)))))

(event Collision|EventActorBeginOverlap
  (params (OtherActor :type Actor%20Object%20Reference)))

(event Collision|EventHit
  (params (MyComp :type Primitive%20Component%20Object%20Reference) (Other :type Actor%20Object%20Reference) (OtherComp :type Primitive%20Component%20Object%20Reference) (bSelfMoved :type Boolean) (HitLocation :type Vector) (HitNormal :type Vector :default "0, 0, 0") (NormalImpulse :type Vector :default "0, 0, 0") (Hit :type Hit%20Result%20Structure%20%28by%20ref%29))
  (bind _returnvalue (Utilities|GetClass Other))
  (bind _damage (Variables|Default|GetDamage))
  (bind _returnvalue_2 (Utilities|GetClassDisplayName _returnvalue))
  (CallFunction|Sound)
  (CallFunction|Hit false)
  (Utilities|FlowControl|DoOnce false
    (:Completed
      (if (Utilities|Enum|Equal(Enum) _returnvalue_2 "BP_Dude_C")
        (bind _asbp_dude (Utilities|Casting|CastToBP_Dude Other))
        (if (Variables|Default|GetKills)
          (Default|DamageSystem _asbp_dude (Math|Conversions|ToFloat(Integer) (Variables|Default|GetDamage)))
          (CallFunction|HitSound))
        (elif (Utilities|Enum|Equal(Enum) _returnvalue_2 "AI_Enemy_C")
          (bind _asai_enemy (Utilities|Casting|CastToAI_Enemy Other))
          (if (Variables|Default|GetKills)
            _
            (else
              _))
          (Default|DMGBadman _asai_enemy (Variables|Default|GetDamage))
          (CallFunction|HitSound)
          (else
            (bind _asbp_master_bad (Utilities|Casting|CastToBP_MasterBad Other))
            (if (Variables|Default|GetKills)
              (Default|DMGBadman _asbp_master_bad _damage)
              (CallFunction|HitSound)
              (else
                (Default|STNBadman _asbp_master_bad _damage)))))))))

(fn ConstructionScript
  (Variables|/Script/Engine.ProjectileMovementComponent|SetInitialSpeed (Variables|Default|GetProjectileMovement) (Variables|Default|GetBulletSpeed)))