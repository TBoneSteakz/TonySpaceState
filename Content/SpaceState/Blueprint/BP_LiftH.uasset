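; BP_LiftH is a paper-sprite actor, named as a horizontal lift, that turns to face the player and tracks them along the X axis.
; Each Tick it measures the sprite-to-player X offset, yaws toward the player and, within a narrow band, shifts by Speed toward the player's X.
; Outside that band it calls Play on its audio.
; The sprite's first-tick location is saved to DefaultLoc but never read here.
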(event EventBeginPlay)

(event Collision|EventActorBeginOverlap
  (params (OtherActor :type Actor%20Object%20Reference)))

(event EventTick
  (params (DeltaSeconds :type Float%20%28single-precision%29))
  (bind _returnvalue (Transformation|GetActorLocation))
  (bind _papersprite (Variables|Default|GetPaperSprite))
  (bind _speed (Variables|Default|GetSpeed))
  (bind _returnvalue_2 (Transformation|GetWorldLocation _papersprite))
  ;[1 1 1] Move and Target
  (Utilities|FlowControl|Sequence
    (:then_0
      (Variables|Default|Setdistance (- (.x _returnvalue_2) (.x (Transformation|GetActorLocation (Game|GetPlayerCharacter 0)))))
      (Utilities|FlowControl|DoOnce false
        (:Completed
          (Variables|Default|SetDefaultLoc (Math|Vector|MakeVector (.x _returnvalue_2) (.y _returnvalue_2) (.z _returnvalue_2))))))
    (:then_1
      (Transformation|SetActorRotation (Math|Rotator|MakeRotator 0.0 0.0 (.yaw (Math|Rotator|FindLookatRotation (Transformation|GetActorLocation) (Transformation|GetActorLocation (Game|GetPlayerCharacter 0)))))))
    (:then_2
      (Variables|Default|SetActorX (.x _returnvalue)))
    (:then_3
      (Variables|Default|SetActorY (.y _returnvalue)))
    (:then_4
      (Variables|Default|SetActorZ (.z _returnvalue)))
    (:then_5
      (if (Math|Float|InRange(Float) (Variables|Default|Getdistance) 0.0 3e+01)
        (Utilities|FlowControl|Delay 0.0)
        (Transformation|SetActorLocation (Math|Vector|MakeVector (- (Variables|Default|GetActorX) _speed) (Variables|Default|GetActorY) (Variables|Default|GetActorZ)) false false)))
    (:then_6
      (if (Math|Float|InRange(Float) (Variables|Default|Getdistance) -3e+01 0.0)
        (Utilities|FlowControl|Delay 0.0)
        (Transformation|SetActorLocation (Math|Vector|MakeVector (+ (Variables|Default|GetActorX) _speed) (Variables|Default|GetActorY) (Variables|Default|GetActorZ)) false false)))
    (:then_7
      (if (not (Math|Float|InRange(Float) (Variables|Default|Getdistance) -3e+01 3e+01))
        (Audio|Components|Audio|Play (Variables|Default|GetAudio) 0.0)))))

(fn ConstructionScript)