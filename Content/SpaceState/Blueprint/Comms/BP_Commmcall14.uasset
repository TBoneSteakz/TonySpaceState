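; BP_Commmcall14 is a one-shot trigger that plays a scripted comms call, apparently from Francis, when BP_Dude enters its box.
; The overlap plays a phone sound at the character's location, shows the WidgetComms overlay and destroys the box so it cannot fire again.
; After a short delay it adds WidgetCommFrancis14, then removes both widgets after a longer delay.
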(event OnComponentBeginOverlap(Box)
  (params (OverlappedComponent :type Primitive%20Component%20Object%20Reference) (OtherActor :type Actor%20Object%20Reference) (OtherComp :type Primitive%20Component%20Object%20Reference) (OtherBodyIndex :type Integer) (bFromSweep :type Boolean) (SweepResult :type Hit%20Result%20Structure%20%28by%20ref%29))
  (bind _asbp_dude (Utilities|Casting|CastToBP_Dude OtherActor))
  (Audio|SpawnSoundatLocation "/Game/SpaceState/Sounds/85344__j008b__phone02-j008b_Cue.85344__j008b__phone02-j008b_Cue" (Transformation|GetActorLocation _asbp_dude))
  (bind _returnvalue (UserInterface|CreateWidget "/Game/SpaceState/Blueprint/Comms/WidgetComms.WidgetComms_C"))
  (UserInterface|Viewport|AddtoViewport _returnvalue 0)
  (Components|DestroyComponent (Variables|Default|GetBox))
  (Utilities|FlowControl|Delay 2.0)
  (bind _returnvalue_2 (UserInterface|CreateWidget "/Game/SpaceState/Blueprint/Comms/WidgetCommFrancis14.WidgetCommFrancis14_C"))
  (UserInterface|Viewport|AddtoViewport _returnvalue_2 0)
  (Utilities|FlowControl|Delay 5.0)
  (Widget|RemovefromParent _returnvalue_2)
  (Widget|RemovefromParent _returnvalue))

(event EventBeginPlay)

(event Collision|EventActorBeginOverlap
  (params (OtherActor :type Actor%20Object%20Reference)))

(event EventTick
  (params (DeltaSeconds :type Float%20%28single-precision%29)))

(fn ConstructionScript)