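; Map pawn that lets the player cycle through points of interest and open the level tied to the selected one.
; It starts at the first entry of its POI array, and the forward and back inputs step the index with wraparound, teleporting the pawn to that POI's location.
; The Shoot input opens the level named by the current POI's LevelToOpen.
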(event EventBeginPlay
  (Transformation|SetActorLocation (Transformation|GetActorLocation (Utilities|Array|Get(acopy) (Variables|Default|GetPOIs))) false false))

(event Collision|EventActorBeginOverlap
  (params (OtherActor :type Actor%20Object%20Reference)))

(event EventTick
  (params (DeltaSeconds :type Float%20%28single-precision%29)))

(event Input|ActionEvents|InputActionCyclemapFoward
  (params (Key :type Key%20Structure :default "AnyKey"))
  (:Pressed
    (bind _output_get (Variables|Default|SetCurrentPOI (+ (Variables|Default|GetCurrentPOI) 1)))
    (if (> _output_get (- (Utilities|Array|Length (Variables|Default|GetPOIs)) 1))
      (Variables|Default|SetCurrentPOI 0))
    (Transformation|SetActorLocation (Transformation|GetActorLocation (Utilities|Array|Get(acopy) (Variables|Default|GetPOIs) _output_get)) false false)))

(event Input|ActionEvents|InputActionCycleMapBack
  (params (Key :type Key%20Structure :default "AnyKey"))
  (:Pressed
    (bind _output_get (Variables|Default|SetCurrentPOI (- (Variables|Default|GetCurrentPOI) 1)))
    (if (< _output_get 0)
      (Variables|Default|SetCurrentPOI (- (Utilities|Array|Length (Variables|Default|GetPOIs)) 1)))
    (Transformation|SetActorLocation (Transformation|GetActorLocation (Utilities|Array|Get(acopy) (Variables|Default|GetPOIs) _output_get)) false false)))

(event Input|ActionEvents|InputActionShoot
  (params (Key :type Key%20Structure :default "AnyKey"))
  (:Pressed
    (Game|OpenLevel(byName) (Variables|/Game/SpaceState/Blueprint/BP_POI.BP_POI_C|GetLevelToOpen (Utilities|Array|Get(acopy) (Variables|Default|GetPOIs) (Variables|Default|GetCurrentPOI))))))

(fn ConstructionScript)