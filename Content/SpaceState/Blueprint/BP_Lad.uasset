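; Climbable ladder that builds itself in the construction script from paper sprite rungs between Top and Bottom, fitting its trigger box and top mesh.
; The box marks it usable for BP_Dude; Use toggles climbing.
; While climbing, the player uses Flying movement, with MoveUp driving vertical velocity and animation state, until leaving restores Walking.
; Other actors entering above the top mesh are dropped down, with AI_Enemy switched to Falling.
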(event OnComponentBeginOverlap(Box)
  (params (OverlappedComponent :type Primitive%20Component%20Object%20Reference) (OtherActor :type Actor%20Object%20Reference) (OtherComp :type Primitive%20Component%20Object%20Reference) (OtherBodyIndex :type Integer) (bFromSweep :type Boolean) (SweepResult :type Hit%20Result%20Structure%20%28by%20ref%29))
  (bind _returnvalue (Transformation|GetActorLocation OtherActor))
  ;[1 1 1] Overlap
  (if (Utilities|Enum|Equal(Enum) (Utilities|GetDisplayName OtherActor) "BP_Dude")
    (Class|BPInterface|CanbeInteractedwith(Message) OtherActor self true)
    (Collision|SetCollisionEnabled (Variables|Default|GetStaticMesh) "QueryAndPhysics")
    (elif (< (.z (Transformation|GetWorldLocation (Variables|Default|GetStaticMesh))) (.z (Transformation|GetActorLocation OtherActor)))
      (Transformation|SetActorLocation OtherActor (Math|Vector|MakeVector (.x _returnvalue) (.y _returnvalue) (- (.z _returnvalue) 6e+01)) false false)
      (bind _asai_enemy (Utilities|Casting|CastToAI_Enemy OtherActor))
      (Pawn|Components|CharacterMovement|SetMovementMode (Variables|/Script/Engine.Character|GetCharacterMovement _asai_enemy) "MOVE_Falling" 0))))

(event OnComponentEndOverlap(Box)
  (params (OverlappedComponent :type Primitive%20Component%20Object%20Reference) (OtherActor :type Actor%20Object%20Reference) (OtherComp :type Primitive%20Component%20Object%20Reference) (OtherBodyIndex :type Integer))
  ;[1 1 1] OverlapEnd
  (if (Utilities|Enum|Equal(Enum) (Utilities|GetDisplayName OtherActor) "BP_Dude")
    (Utilities|FlowControl|Sequence
      (:then_0
        (Class|BPInterface|CanbeInteractedwith(Message) OtherActor self false))
      (:then_1
        (Variables|Default|Setonlad false)
        (Input|EnableInput (Game|GetPlayerController 0))
        (Pawn|Components|CharacterMovement|SetMovementMode (Variables|/Script/Engine.Character|GetCharacterMovement (Game|GetPlayerCharacter 0)) "MOVE_Walking" 0)
        (bind _asbp_dude (Utilities|Casting|CastToBP_Dude OtherActor))
        (Variables|/Game/SpaceState/Blueprint/BP_Dude/BP_Dude.BP_Dude_C|SetState _asbp_dude "NewEnumerator0")))
    (else
      (bind _asai_enemy (Utilities|Casting|CastToAI_Enemy OtherActor))
      (Pawn|Components|CharacterMovement|SetMovementMode (Variables|/Script/Engine.Character|GetCharacterMovement _asai_enemy) "MOVE_Walking" 0))))

(event EventUse
  (params (InteractedObject :type Actor%20Object%20Reference) (IsUsable :type Boolean))
  (bind _returnvalue (Game|GetPlayerController 0))
  (bind _returnvalue_2 (Game|GetPlayerCharacter 0))
  (bind _charactermovement (Variables|/Script/Engine.Character|GetCharacterMovement _returnvalue_2))
  ;[1 1 1] OnLad
  (if (Variables|Default|Getonlad)
    ;[1 1 1] OverlapEnd
    (Variables|Default|Setonlad false)
    (Input|EnableInput _returnvalue)
    (Pawn|Components|CharacterMovement|SetMovementMode _charactermovement "MOVE_Walking" 0)
    (bind _asbp_dude (Utilities|Casting|CastToBP_Dude (stale OnComponentEndOverlap(Box) OtherActor)))
    (Variables|/Game/SpaceState/Blueprint/BP_Dude/BP_Dude.BP_Dude_C|SetState _asbp_dude "NewEnumerator0")
    (else
      (Variables|Default|Setonlad true)
      (Pawn|Components|CharacterMovement|SetMovementMode _charactermovement "MOVE_Flying" 0)
      (Input|EnableInput _returnvalue))))

(event Input|AxisEvents|InputAxisMoveUp
  (params (AxisValue :type Float%20%28single-precision%29))
  (bind _returnvalue (Game|GetPlayerCharacter 0))
  (bind _charactermovement (Variables|/Script/Engine.Character|GetCharacterMovement _returnvalue))
  ;[1 1 1] ClimbUpDown
  (if (Variables|Default|Getonlad)
    (if (== AxisValue 0.0)
      (bind _asbp_dude (Utilities|Casting|CastToBP_Dude (Game|GetPlayerCharacter 0)))
      (if (Variables|/Game/SpaceState/Blueprint/BP_Dude/BP_Dude.BP_Dude_C|GetIsshooting _asbp_dude)
        (Variables|/Game/SpaceState/Blueprint/BP_Dude/BP_Dude.BP_Dude_C|SetState _asbp_dude "NewEnumerator17")
        (else
          (Variables|/Game/SpaceState/Blueprint/BP_Dude/BP_Dude.BP_Dude_C|SetState _asbp_dude "NewEnumerator8")))
      (Pawn|Components|CharacterMovement|SetMovementMode (Variables|/Script/Engine.Character|GetCharacterMovement (Game|GetPlayerCharacter 0)) "MOVE_Flying" 0)
      (Variables|/Script/Engine.MovementComponent|SetVelocity (Variables|/Script/Engine.Character|GetCharacterMovement (Game|GetPlayerCharacter 0)) "0.000000, 0,0.000000")
      (Utilities|FlowControl|Delay 0.2)
      (else
        (bind _asbp_dude_2 (Utilities|Casting|CastToBP_Dude (Game|GetPlayerCharacter 0)))
        (Variables|/Game/SpaceState/Blueprint/BP_Dude/BP_Dude.BP_Dude_C|SetState _asbp_dude_2 "NewEnumerator9")
        (Pawn|Components|CharacterMovement|SetMovementMode _charactermovement "MOVE_Flying" 0)
        (Variables|/Script/Engine.MovementComponent|SetVelocity _charactermovement (Math|Vector|MakeVector 0.0 0.0 (* AxisValue 75.0)))
        (Utilities|FlowControl|Delay 0.05)))))

(fn ConstructionScript
  (bind _top (Variables|Default|GetTop))
  (bind _bottom (Variables|Default|GetBottom))
  (bind _rungoffset (Variables|Default|GetRungoffset))
  (bind _box (Variables|Default|GetBox))
  (bind _returnvalue (- _top _bottom))
  (bind _returnvalue_2 (/ (.z _returnvalue) 2.0))
  (Utilities|FlowControl|Sequence
    (:then_0
      (for _index (range 0 (Math|Float|Truncate (/ (.z _returnvalue) _rungoffset)))
        (bind _returnvalue_3 (AddComponent|AddPaperSpriteComponent false (Math|Transform|MakeTransform (Math|Vector|MakeVector 0.0 0.0 (* _index _rungoffset)) "0, 0, 0" "1.000000,1.000000,1.000000")))
        (Rendering|Components|Sprite|SetSprite _returnvalue_3 "/Game/SpaceState/Sprites/Env/NewFolder/Tiles_Sprite_15.Tiles_Sprite_15")
        (Collision|SetCollisionResponsetoAllChannels _returnvalue_3 "ECR_Overlap")
        (Variables|Default|SetSpriteComponent _returnvalue_3))
      (Transformation|SetRelativeScale3D _box (Math|Vector|MakeVector 0.5 0.5 _returnvalue_2))
      (Transformation|SetRelativeLocation _box (Math|Vector|MakeVector 0.0 0.0 _returnvalue_2) false false))
    (:then_1
      (Transformation|SetRelativeLocation (Variables|Default|GetStaticMesh) _top false false)
      (Collision|SetCollisionResponsetoAllChannels _returnvalue_3 "ECR_Block")
      (Collision|SetCollisionResponsetoChannel _returnvalue_3 "ECC_GameTraceChannel4" "ECR_Overlap")
      (Collision|SetCollisionResponsetoChannel _returnvalue_3 "ECC_Pawn" "ECR_Overlap"))))