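; BP_TAmmo is an ammo pickup drop that adds cells to the player character, BP_Dude.
; On Hit by BP_Dude, it calls CellSystem with BulletPlus, but only while CurrentCells is below a hardcoded cap of ten.
; A successful pickup plays the Q_HealthPickup sound at the hit location and destroys the sprite and box components, leaving the actor itself in place.
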(event EventBeginPlay)

(event Collision|EventActorBeginOverlap
  (params (OtherActor :type Actor%20Object%20Reference)))

(event EventTick
  (params (DeltaSeconds :type Float%20%28single-precision%29)))

(event Collision|EventHit
  (params (MyComp :type Primitive%20Component%20Object%20Reference) (Other :type Actor%20Object%20Reference) (OtherComp :type Primitive%20Component%20Object%20Reference) (bSelfMoved :type Boolean) (HitLocation :type Vector) (HitNormal :type Vector :default "0, 0, 0") (NormalImpulse :type Vector :default "0, 0, 0") (Hit :type Hit%20Result%20Structure%20%28by%20ref%29))
  (bind _asbp_dude (Utilities|Casting|CastToBP_Dude Other))
  (if (not (>= (Variables|/Game/SpaceState/Blueprint/BP_Dude.BP_Dude_C|GetCurrentCells _asbp_dude) 10))
    (Default|CellSystem _asbp_dude (Variables|Default|GetBulletPlus))
    (Components|DestroyComponent (Variables|Default|GetPaperSprite))
    (Audio|SpawnSoundatLocation "/Game/SpaceState/Allsounds/Sounds/Q_HealthPickup.Q_HealthPickup" HitLocation)
    (Components|DestroyComponent (Variables|Default|GetBox))))

(fn ConstructionScript)