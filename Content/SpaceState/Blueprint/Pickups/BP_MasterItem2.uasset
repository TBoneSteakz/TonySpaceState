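; BP_MasterItem2 is a weapon pickup that the player can collect into the HUD inventory.
; The construction script fills the ItemInfo struct from custom properties, which drive its sprite, clip count and prompt text.
; Box overlap toggles an on-screen prompt and range flag; BP_Dude's PickupItem dispatcher then hides the actor and adds it to inventory and weapon array.
; Useaction always equips the player's first weapon slot.
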(event OnComponentBeginOverlap(Box)
  (params (OverlappedComponent :type Primitive%20Component%20Object%20Reference) (OtherActor :type Actor%20Object%20Reference) (OtherComp :type Primitive%20Component%20Object%20Reference) (OtherBodyIndex :type Integer) (bFromSweep :type Boolean) (SweepResult :type Hit%20Result%20Structure%20%28by%20ref%29))
  ;[1 1 1] OverlapTriggerScript
  (Utilities|Casting|CastToBP_Dude OtherActor)
  (UserInterface|Viewport|AddtoViewport (Variables|Default|GetPickupTextRef) 0)
  (Variables|Default|SetIsInRange true))

(event OnComponentEndOverlap(Box)
  (params (OverlappedComponent :type Primitive%20Component%20Object%20Reference) (OtherActor :type Actor%20Object%20Reference) (OtherComp :type Primitive%20Component%20Object%20Reference) (OtherBodyIndex :type Integer))
  ;[1 1 1] OverlapTriggerScript
  (Utilities|Casting|CastToBP_Dude OtherActor)
  (Widget|RemovefromParent (Variables|Default|GetPickupTextRef))
  (Variables|Default|SetIsInRange false))

(event Custom|PickupItem_Event_0
  (bind _player (Variables|Default|GetPlayer))
  (bind _player_2 (Variables|Default|GetPlayer))
  (bind _widethudref (Variables|/Game/SpaceState/Blueprint/BP_Dude/BP_Dude.BP_Dude_C|GetWidetHudRef _player_2))
  ;[1 1 1] PickupItems
  (if (and (Collision|GetActorEnableCollision) (Variables|Default|GetIsInRange))
    (Utilities|Array|Add (Variables|/Game/SpaceState/Blueprint/HUD/Widget_HUD.Widget_HUD_C|GetInventory _widethudref) (Variables|Default|GetItemInfo))
    (Widget|RemovefromParent (Variables|Default|GetPickupTextRef))
    (Rendering|SetActorHiddenInGame true)
    (Collision|SetActorEnableCollision false)
    (Default|RefreshInventory _widethudref)
    (Utilities|Array|Add (Variables|/Game/SpaceState/Blueprint/BP_Dude/BP_Dude.BP_Dude_C|GetWeaponArray _player) (Utilities|String|StringToName (Utilities|String|ToString(Integer) (Variables|Default|GetWeapon))))
    (Default|NewWeapon _player)))

(event EventUseaction
  (bind _player (Variables|Default|GetPlayer))
  ;[1 1 1] UseItem
  (Variables|/Game/SpaceState/Blueprint/BP_Dude/BP_Dude.BP_Dude_C|SetWeaponIndex _player 0)
  (Default|EquipWeapon _player))

(event EventBeginPlay
  (bind _iteminfo (Variables|Default|GetItemInfo))
  (bind (_item _itemimage _pickuptext _actiontext _itemsprite _consumable _clipcount) (Utilities|Struct|BreakInventoryStrut _iteminfo))
  ;[1 1 1] EventBeginPlay
  (bind _returnvalue (UserInterface|CreateWidget "/Game/SpaceState/Inventory/PickupText.PickupText_C"))
  (Variables|Default|SetPickupTextRef _returnvalue)
  (Utilities|Struct|SetmembersinInventoryStrut _iteminfo self)
  (Variables|/Game/SpaceState/Inventory/PickupText.PickupText_C|SetPickupActor (Variables|Default|GetPickupTextRef) _item)
  (Variables|/Game/SpaceState/Inventory/PickupText.PickupText_C|SetPickupText (Variables|Default|GetPickupTextRef) _pickuptext)
  (Variables|Default|SetClipCount _clipcount)
  (Rendering|Components|Sprite|SetSprite (Variables|Default|GetItemSprite) _itemsprite)
  (bind _asbp_dude (Utilities|Casting|CastToBP_Dude (Game|GetPlayerCharacter 0)))
  (bind _output_get (Variables|Default|SetPlayer _asbp_dude))
  (EventDispatchers|AssignPickupItem _output_get (delegate Custom|PickupItem_Event_0)))

(fn ConstructionScript
  (Utilities|Struct|SetmembersinInventoryStrut (Variables|Default|GetItemInfo) self (Variables|Default|GetCustomImage) (Variables|Default|GetCustomPickupText) (Variables|Default|GetCustomActionText) (Variables|Default|GetCustomSprite) false (Variables|Default|GetCustomClip)))