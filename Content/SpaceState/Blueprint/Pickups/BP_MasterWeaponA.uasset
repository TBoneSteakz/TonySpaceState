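; Master weapon pickup that the player (BP_Dude) or an AI_Enemy can take.
; BeginPlay fills item info, sprite and prompt widget from an InventoryDT row chosen by WeaponIndex; Dropped re-runs part of that setup.
; Capsule overlap toggles interactability and the prompt.
; Use hides the actor, adding it to the player's inventory and weapons or writing weapon and clip count to the enemy's Blackboard; Useaction equips the player's weapon index zero.
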(event OnComponentBeginOverlap(CapsuleComponent)
  (params (OverlappedComponent :type Primitive%20Component%20Object%20Reference) (OtherActor :type Actor%20Object%20Reference) (OtherComp :type Primitive%20Component%20Object%20Reference) (OtherBodyIndex :type Integer) (bFromSweep :type Boolean) (SweepResult :type Hit%20Result%20Structure%20%28by%20ref%29))
  (bind _output_get (Variables|Default|SetActor OtherActor))
  ;[1 1 1] OverlapTriggerScript
  (Class|BPInterface|CanbeInteractedwith(Message) _output_get self true)
  (UserInterface|Viewport|AddtoViewport (Variables|Default|GetPickupTextRef) 0))

(event OnComponentEndOverlap(CapsuleComponent)
  (params (OverlappedComponent :type Primitive%20Component%20Object%20Reference) (OtherActor :type Actor%20Object%20Reference) (OtherComp :type Primitive%20Component%20Object%20Reference) (OtherBodyIndex :type Integer))
  (bind _output_get (Variables|Default|SetActor OtherActor))
  ;[1 1 1] OverlapTriggerScript
  (Class|BPInterface|CanbeInteractedwith(Message) _output_get self false)
  (Widget|RemovefromParent (Variables|Default|GetPickupTextRef)))

(event Custom|Dropped
  (bind _iteminfo (Variables|Default|GetItemInfo))
  (bind (_item _itemimage _pickuptext _actiontext _itemsprite _consumable _clipcount _weapon) (Utilities|Struct|BreakInventoryStrut _iteminfo))
  ;[1 1 1] EventBeginPlay
  (Variables|Default|SetPickupTextRef (stale EventBeginPlay _returnvalue_2))
  (Utilities|Struct|SetmembersinInventoryStrut _iteminfo self)
  (Variables|/Game/SpaceState/Blueprint/Pickups/Inventory/PickupText.PickupText_C|SetPickupActor (Variables|Default|GetPickupTextRef) _item)
  (Variables|/Game/SpaceState/Blueprint/Pickups/Inventory/PickupText.PickupText_C|SetPickupText (Variables|Default|GetPickupTextRef) _pickuptext)
  (Variables|Default|SetClipCount _clipcount)
  (Variables|Default|SetCustomWeapon _weapon)
  (Rendering|Components|Sprite|SetSprite (Variables|Default|GetPaperSprite) _itemsprite))

(event EventUseaction
  ;[1 1 1] UseItem
  (Variables|/Game/SpaceState/Blueprint/BP_Dude/BP_Dude.BP_Dude_C|SetWeaponIndex (stale EventUse _asbp_dude) 0)
  (Default|EquipWeapon (stale EventUse _asbp_dude)))

(event EventBeginPlay
  ;[1 1 1] EventBeginPlay
  (bind _outrownames (DataTable|GetDataTableRowNames "/Game/SpaceState/Blueprint/Pickups/Inventory/InventoryDT.InventoryDT"))
  (Variables|Default|SetArray _outrownames)
  (bind _returnvalue (Utilities|GetDataTableRow "/Game/SpaceState/Blueprint/Pickups/Inventory/InventoryDT.InventoryDT" (Utilities|Array|Get(acopy) (Variables|Default|GetArray) (Variables|Default|GetWeaponIndex)))
    (:then
      (Variables|Default|SetItemInfo _returnvalue)
      (bind _returnvalue_2 (UserInterface|CreateWidget "/Game/SpaceState/Blueprint/Pickups/Inventory/PickupText.PickupText_C"))
      (Variables|Default|SetPickupTextRef _returnvalue_2)
      (Utilities|Struct|SetmembersinInventoryStrut (Variables|Default|GetItemInfo) self)
      (Variables|/Game/SpaceState/Blueprint/Pickups/Inventory/PickupText.PickupText_C|SetPickupActor (Variables|Default|GetPickupTextRef) (.Item (Utilities|Struct|BreakInventoryStrut (Variables|Default|GetItemInfo))))
      (Variables|/Game/SpaceState/Blueprint/Pickups/Inventory/PickupText.PickupText_C|SetPickupText (Variables|Default|GetPickupTextRef) (.PickUpText (Utilities|Struct|BreakInventoryStrut (Variables|Default|GetItemInfo))))
      (Variables|Default|SetClipCount (.ClipCount (Utilities|Struct|BreakInventoryStrut (Variables|Default|GetItemInfo))))
      (Variables|Default|SetCustomWeapon (.Weapon (Utilities|Struct|BreakInventoryStrut (Variables|Default|GetItemInfo))))
      (Rendering|Components|Sprite|SetSprite (Variables|Default|GetPaperSprite) (.ItemSprite (Utilities|Struct|BreakInventoryStrut (Variables|Default|GetItemInfo)))))))

(event EventUse
  (params (InteractedObject :type Actor%20Object%20Reference) (IsUsable :type Boolean))
  (bind _actor (Variables|Default|GetActor))
  ;[1 1 1] PickupItems
  (if (Utilities|Enum|Equal(Enum) (Utilities|GetDisplayName InteractedObject) "BP_Dude")
    (bind _asbp_dude (Utilities|Casting|CastToBP_Dude _actor))
    (Utilities|Array|Add (Variables|/Game/SpaceState/Blueprint/HUD/Widget_HUD.Widget_HUD_C|GetInventory (Variables|/Game/SpaceState/Blueprint/BP_Dude/BP_Dude.BP_Dude_C|GetWidetHudRef _asbp_dude)) (Variables|Default|GetItemInfo))
    (Widget|RemovefromParent (Variables|Default|GetPickupTextRef))
    (Rendering|SetActorHiddenInGame true)
    (Collision|SetActorEnableCollision false)
    (Default|RefreshInventory (Variables|/Game/SpaceState/Blueprint/BP_Dude/BP_Dude.BP_Dude_C|GetWidetHudRef _asbp_dude))
    (Utilities|Array|Add (Variables|/Game/SpaceState/Blueprint/BP_Dude/BP_Dude.BP_Dude_C|GetWeaponArray _asbp_dude) (Utilities|String|StringToName (Utilities|String|ToString(Integer) (Variables|Default|GetCustomWeapon))))
    (Default|NewWeapon _asbp_dude)
    (else
      (bind _asai_enemy (Utilities|Casting|CastToAI_Enemy _actor))
      (Class|BlackboardComponent|SetValueasInt (AI|GetBlackboard (Pawn|GetController _asai_enemy)) (Variables|Default|GetBlackBoardKeySecondWeaponIndex) (Variables|Default|GetCustomWeapon))
      (Class|BlackboardComponent|SetValueasInt (AI|GetBlackboard (Pawn|GetController _asai_enemy)) (Variables|Default|GetBlackBoardKeyClipCount) (Variables|Default|GetClipCount))
      (Rendering|SetActorHiddenInGame true)
      (Collision|SetActorEnableCollision false))))

(fn ConstructionScript)