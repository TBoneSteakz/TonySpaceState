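; Master weapon pickup actor that configures itself from the InventoryDT row selected by WeaponIndex, setting its sprite, clip count, weapon and prompt text.
; Box overlap with BP_Dude toggles the prompt widget and an in-range flag checked by the handler bound through AssignPickupItem.
; Pickup hides the actor, disables collision, and updates HUD inventory and the player's weapon array.
; Dropped re-enters setup after widget creation; Useaction equips weapon index zero.
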(event OnComponentBeginOverlap(Box)
  (params (OverlappedComponent :type Primitive%20Component%20Object%20Reference) (OtherActor :type Actor%20Object%20Reference) (OtherComp :type Primitive%20Component%20Object%20Reference) (OtherBodyIndex :type Integer) (bFromSweep :type Boolean) (SweepResult :type Hit%20Result%20Structure%20%28by%20ref%29))
  ;[1 1 1] OverlapTriggerScript
  (Utilities|Casting|CastToBP_Dude OtherActor)
  (UserInterface|Viewport|AddtoViewport (Variables|Default|GetPickupTextRef) 0)
  (Variables|Default|SetIsInRange true))

(event OnComponentEndOverlap(Box)
  (params (OverlappedComponent :type Primitive%20Component%20Object%20Reference) (OtherActor :type Actor%20Object%20Reference) (OtherComp :type Primitive%20Component%20Object%20Reference) (OtherBodyIndex :type Integer))
  ;[1 1 1] OverlapTriggerScript
  (Utilities|Casting|CastToBP_Dude OtherActor)
  (Widget|RemovefromParent (Variables|Default|GetPickupTextRef))
  (Variables|Default|SetIsInRange false))

(event Custom|PickupItem_Event_0
  (bind _player (Variables|Default|GetPlayer))
  (bind _player_2 (Variables|Default|GetPlayer))
  (bind _widethudref (Variables|/Game/SpaceState/Blueprint/BP_Dude/BP_Dude.BP_Dude_C|GetWidetHudRef _player_2))
  ;[1 1 1] PickupItems
  (if (and (Collision|GetActorEnableCollision) (Variables|Default|GetIsInRange))
    (Utilities|Array|Add (Variables|/Game/SpaceState/Blueprint/HUD/Widget_HUD.Widget_HUD_C|GetInventory _widethudref) (Variables|Default|GetItemInfo))
    (Widget|RemovefromParent (Variables|Default|GetPickupTextRef))
    (Rendering|SetActorHiddenInGame true)
    (Collision|SetActorEnableCollision false)
    (Default|RefreshInventory _widethudref)
    (Utilities|Array|Add (Variables|/Game/SpaceState/Blueprint/BP_Dude/BP_Dude.BP_Dude_C|GetWeaponArray _player) (Utilities|String|StringToName (Utilities|String|ToString(Integer) (Variables|Default|GetCustomWeapon))))
    (Default|NewWeapon _player)))

(event Custom|Dropped
  (bind _iteminfo (Variables|Default|GetItemInfo))
  (bind (_item _itemimage _pickuptext _actiontext _itemsprite _consumable _clipcount _weapon) (Utilities|Struct|BreakInventoryStrut _iteminfo))
  ;[1 1 1] EventBeginPlay
  (Variables|Default|SetPickupTextRef (stale EventBeginPlay _returnvalue_2))
  (Utilities|Struct|SetmembersinInventoryStrut _iteminfo self)
  (Variables|/Game/SpaceState/Blueprint/Pickups/Inventory/PickupText.PickupText_C|SetPickupActor (Variables|Default|GetPickupTextRef) _item)
  (Variables|/Game/SpaceState/Blueprint/Pickups/Inventory/PickupText.PickupText_C|SetPickupText (Variables|Default|GetPickupTextRef) _pickuptext)
  (Variables|Default|SetClipCount _clipcount)
  (Variables|Default|SetCustomWeapon _weapon)
  (Rendering|Components|Sprite|SetSprite (Variables|Default|GetItemSprite) _itemsprite)
  (bind _asbp_dude (Utilities|Casting|CastToBP_Dude (Game|GetPlayerCharacter 0)))
  (bind _output_get (Variables|Default|SetPlayer _asbp_dude))
  (EventDispatchers|AssignPickupItem _output_get (delegate Custom|PickupItem_Event_0)))

(event EventUseaction
  (bind _player (Variables|Default|GetPlayer))
  ;[1 1 1] UseItem
  (Variables|/Game/SpaceState/Blueprint/BP_Dude/BP_Dude.BP_Dude_C|SetWeaponIndex _player 0)
  (Default|EquipWeapon _player))

(event EventBeginPlay
  ;[1 1 1] EventBeginPlay
  (bind _outrownames (DataTable|GetDataTableRowNames "/Game/SpaceState/Blueprint/Pickups/Inventory/InventoryDT.InventoryDT"))
  (Variables|Default|SetArray _outrownames)
  (bind _returnvalue (Utilities|GetDataTableRow "/Game/SpaceState/Blueprint/Pickups/Inventory/InventoryDT.InventoryDT" (Utilities|Array|Get(acopy) (Variables|Default|GetArray) (Variables|Default|GetWeaponIndex)))
    (:then
      (Variables|Default|SetItemInfo _returnvalue)
      (bind _returnvalue_2 (UserInterface|CreateWidget "/Game/SpaceState/Blueprint/Pickups/Inventory/PickupText.PickupText_C"))
      (Variables|Default|SetPickupTextRef _returnvalue_2)
      (Utilities|Struct|SetmembersinInventoryStrut (Variables|Default|GetItemInfo) self)
      (Variables|/Game/SpaceState/Blueprint/Pickups/Inventory/PickupText.PickupText_C|SetPickupActor (Variables|Default|GetPickupTextRef) (.Item (Utilities|Struct|BreakInventoryStrut (Variables|Default|GetItemInfo))))
      (Variables|/Game/SpaceState/Blueprint/Pickups/Inventory/PickupText.PickupText_C|SetPickupText (Variables|Default|GetPickupTextRef) (.PickUpText (Utilities|Struct|BreakInventoryStrut (Variables|Default|GetItemInfo))))
      (Variables|Default|SetClipCount (.ClipCount (Utilities|Struct|BreakInventoryStrut (Variables|Default|GetItemInfo))))
      (Variables|Default|SetCustomWeapon (.Weapon (Utilities|Struct|BreakInventoryStrut (Variables|Default|GetItemInfo))))
      (Rendering|Components|Sprite|SetSprite (Variables|Default|GetItemSprite) (.ItemSprite (Utilities|Struct|BreakInventoryStrut (Variables|Default|GetItemInfo))))
      (bind _asbp_dude (Utilities|Casting|CastToBP_Dude (Game|GetPlayerCharacter 0)))
      (bind _output_get (Variables|Default|SetPlayer _asbp_dude))
      (EventDispatchers|AssignPickupItem _output_get (delegate Custom|PickupItem_Event_0)))))

(fn ConstructionScript)