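; BP_TAmmo is an ammo pickup that refills the cells of BP_Dude.
; When BP_Dude overlaps its Box and CurrentCells is below a fixed cap, it passes BulletPlus to the character's CellSystem.
; It then destroys its sprite and Box, leaving the actor itself in place, and plays a health-pickup sound spawned at the world origin rather than at the pickup.
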(event OnComponentBeginOverlap(Box)
  (params (OverlappedComponent :type Primitive%20Component%20Object%20Reference) (OtherActor :type Actor%20Object%20Reference) (OtherComp :type Primitive%20Component%20Object%20Reference) (OtherBodyIndex :type Integer) (bFromSweep :type Boolean) (SweepResult :type Hit%20Result%20Structure%20%28by%20ref%29))
  (bind _asbp_dude (Utilities|Casting|CastToBP_Dude OtherActor))
  (if (not (>= (Variables|/Game/SpaceState/Blueprint/BP_Dude.BP_Dude_C|GetCurrentCells _asbp_dude) 10))
    (Default|CellSystem _asbp_dude (Variables|Default|GetBulletPlus))
    (Components|DestroyComponent (Variables|Default|GetPaperSprite))
    (Audio|SpawnSoundatLocation "/Game/SpaceState/Sounds/Q_HealthPickup.Q_HealthPickup" "0, 0, 0")
    (Components|DestroyComponent (Variables|Default|GetBox))))

(event EventBeginPlay)

(event Collision|EventActorBeginOverlap
  (params (OtherActor :type Actor%20Object%20Reference)))

(event EventTick
  (params (DeltaSeconds :type Float%20%28single-precision%29)))

(fn ConstructionScript)