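; BP_Bag is a bag pickup that expands the player's inventory as soon as BP_Dude overlaps its box.
; The construction script fills the ItemInfo struct from custom properties as a non-consumable, and BeginPlay applies it to the sprite and a PickupText widget.
; On overlap it reveals five extra HUD slots, sets item capacity to 15, refreshes the inventory, removes the text widget, and hides the actor without destroying it.
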(event OnComponentBeginOverlap(Box)
  (params (OverlappedComponent :type Primitive%20Component%20Object%20Reference) (OtherActor :type Actor%20Object%20Reference) (OtherComp :type Primitive%20Component%20Object%20Reference) (OtherBodyIndex :type Integer) (bFromSweep :type Boolean) (SweepResult :type Hit%20Result%20Structure%20%28by%20ref%29))
  (bind _player (Variables|Default|GetPlayer))
  (bind _widethudref (Variables|/Game/SpaceState/Blueprint/BP_Dude/BP_Dude.BP_Dude_C|GetWidetHudRef _player))
  ;[1 1 1] OverlapTriggerScript
  (Utilities|Casting|CastToBP_Dude OtherActor)
  ;[1 1 1] PickupItems
  (Widget|SetVisibility (Variables|/Game/SpaceState/Blueprint/HUD/Widget_HUD.Widget_HUD_C|GetSlot_10 _widethudref) "Visible")
  (Variables|/Game/SpaceState/Blueprint/BP_Dude/BP_Dude.BP_Dude_C|SetItemCapacity _player 15)
  (Widget|RemovefromParent (Variables|Default|GetPickupTextRef))
  (Rendering|SetActorHiddenInGame true)
  (Collision|SetActorEnableCollision false)
  (Default|RefreshInventory _widethudref))

(event EventBeginPlay
  (bind _iteminfo (Variables|Default|GetItemInfo))
  (bind (_item _itemimage _pickuptext _actiontext _itemsprite) (Utilities|Struct|BreakInventoryStrut _iteminfo))
  (bind _returnvalue (UserInterface|CreateWidget "/Game/SpaceState/Inventory/PickupText.PickupText_C"))
  (Variables|Default|SetPickupTextRef _returnvalue)
  (Utilities|Struct|SetmembersinInventoryStrut _iteminfo self)
  (Variables|/Game/SpaceState/Inventory/PickupText.PickupText_C|SetPickupActor (Variables|Default|GetPickupTextRef) _item)
  (Variables|/Game/SpaceState/Inventory/PickupText.PickupText_C|SetPickupText (Variables|Default|GetPickupTextRef) _pickuptext)
  (Rendering|Components|Sprite|SetSprite (Variables|Default|GetItemSprite) _itemsprite)
  (bind _asbp_dude (Utilities|Casting|CastToBP_Dude (Game|GetPlayerCharacter 0)))
  (Variables|Default|SetPlayer _asbp_dude))

(fn ConstructionScript
  (Utilities|Struct|SetmembersinInventoryStrut (Variables|Default|GetItemInfo) self (Variables|Default|GetCustomImage) (Variables|Default|GetCustomPickupText) (Variables|Default|GetCustomActionText) (Variables|Default|GetCustomSprite) false))