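; Switch_A is an interactable sprite switch that resets a horizontal or "H" lift (BP_LiftH) to its default location.
; Overlap begin and end message the other actor whether the switch is usable, darkening the sprite and restoring it to white.
; The tint's player check has identical branches.
; Use finds the first BP_LiftH in the level and moves its sprite component to DefaultLoc without sweeping.
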(event EventBeginPlay)

(event Collision|EventActorBeginOverlap
  (params (OtherActor :type Actor%20Object%20Reference))
  (bind _papersprite (Variables|Default|GetPaperSprite))
  ;[1 1 1] CanBeInteractedWith
  (Class|BPInterface|CanbeInteractedwith(Message) OtherActor self true)
  (bind _asbp_dude (Utilities|Casting|CastToBP_Dude (Game|GetPlayerCharacter 0)))
  (if (== _asbp_dude OtherActor)
    (Sprite|SetSpriteColor _papersprite "(R=0.190000,G=0.190000,B=0.190000,A=1.000000)")
    (else
      (Sprite|SetSpriteColor _papersprite "(R=0.190000,G=0.190000,B=0.190000,A=1.000000)"))))

(event EventTick
  (params (DeltaSeconds :type Float%20%28single-precision%29)))

(event Collision|EventActorEndOverlap
  (params (OtherActor :type Actor%20Object%20Reference))
  ;[1 1 1] CantUse
  (Class|BPInterface|CanbeInteractedwith(Message) OtherActor self false)
  (Sprite|SetSpriteColor (Variables|Default|GetPaperSprite) "(R=1.000000,G=1.000000,B=1.000000,A=1.000000)"))

(event EventUse
  (params (InteractedObject :type Actor%20Object%20Reference) (IsUsable :type Boolean))
  ;[1 1 1] LiftReset
  (bind _outactors (Actor|GetAllActorsOfClass "/Game/SpaceState/Blueprint/BP_LiftH.BP_LiftH_C"))
  (Variables|Default|SetLiftH _outactors)
  (bind _asbp_lift_h (Utilities|Casting|CastToBP_LiftH (Utilities|Array|Get(acopy) (Variables|Default|GetLiftH))))
  (Transformation|SetWorldLocation (Variables|/Game/SpaceState/Blueprint/BP_LiftH.BP_LiftH_C|GetPaperSprite _asbp_lift_h) (Variables|/Game/SpaceState/Blueprint/BP_LiftH.BP_LiftH_C|GetDefaultLoc _asbp_lift_h) false false))

(fn ConstructionScript)