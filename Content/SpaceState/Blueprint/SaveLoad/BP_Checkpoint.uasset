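; Trigger-box checkpoint or save point that saves player progress when an actor tagged "Mark" overlaps it.
; It copies BP_Dude's location, level, ammo, weapons, health and credits into a new Save_info and writes slot "Loc".
; The Checkpoint flag picks one of two near-identical one-shot branches, storing either weapon count or weapon index in CheckWeapons.
; The construction script sizes the box from ChangeHitbox and sets the billboard sprite by that flag.
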(event EventBeginPlay)

(event EventTick
  (params (DeltaSeconds :type Float%20%28single-precision%29)))

(event Collision|EventActorBeginOverlap
  (params (OtherActor :type Actor%20Object%20Reference))
  (if (Actor|ActorHasTag OtherActor "Mark")
    (bind _returnvalue (SaveGame|CreateSaveGameObject "/Game/SpaceState/Blueprint/SaveLoad/Save_info.Save_info_C"))
    (bind _assave_info (Utilities|Casting|CastToSave_info _returnvalue))
    (Variables|Default|SetSaveInfo _assave_info)
    (bind _asbp_dude (Utilities|Casting|CastToBP_Dude (Game|GetPlayerCharacter 0)))
    (Variables|Default|SetCharInfo _asbp_dude)
    (if (Variables|Default|GetCheckpoint)
      (Utilities|FlowControl|DoOnce false
        (:Completed
          (Variables|/Game/SpaceState/Blueprint/SaveLoad/Save_info.Save_info_C|SetCheckLocation (Variables|Default|GetSaveInfo) (Math|Vector|MakeVector (.x (Transformation|GetActorLocation (Variables|Default|GetCharInfo))) (.y (Transformation|GetActorLocation (Variables|Default|GetCharInfo))) (.z (Transformation|GetActorLocation (Variables|Default|GetCharInfo)))))
          (bind _returnvalue_2 (Game|GetCurrentLevelName true))
          (Variables|/Game/SpaceState/Blueprint/SaveLoad/Save_info.Save_info_C|SetCurrentLevel (Variables|Default|GetSaveInfo) (Utilities|String|StringToName _returnvalue_2))
          (Variables|/Game/SpaceState/Blueprint/SaveLoad/Save_info.Save_info_C|SetCheckBullets (Variables|Default|GetSaveInfo) (Variables|/Game/SpaceState/Blueprint/BP_Dude.BP_Dude_C|GetCurrentBullets (Variables|Default|GetCharInfo)))
          (Variables|/Game/SpaceState/Blueprint/SaveLoad/Save_info.Save_info_C|SetCheckCells (Variables|Default|GetSaveInfo) (Variables|/Game/SpaceState/Blueprint/BP_Dude.BP_Dude_C|GetCurrentCells (Variables|Default|GetCharInfo)))
          (Variables|/Game/SpaceState/Blueprint/SaveLoad/Save_info.Save_info_C|SetCheckFuel (Variables|Default|GetSaveInfo) (Variables|/Game/SpaceState/Blueprint/BP_Dude.BP_Dude_C|GetCurrentFuel (Variables|Default|GetCharInfo)))
          (Variables|/Game/SpaceState/Blueprint/SaveLoad/Save_info.Save_info_C|SetCheckShells (Variables|Default|GetSaveInfo) (Variables|/Game/SpaceState/Blueprint/BP_Dude.BP_Dude_C|GetCurrentShells (Variables|Default|GetCharInfo)))
          (Variables|/Game/SpaceState/Blueprint/SaveLoad/Save_info.Save_info_C|SetCheckWeapons (Variables|Default|GetSaveInfo) (Variables|/Game/SpaceState/Blueprint/BP_Dude.BP_Dude_C|GetCurrentNoOfWeaps (Variables|Default|GetCharInfo)))
          (Variables|/Game/SpaceState/Blueprint/SaveLoad/Save_info.Save_info_C|SetCheckHP (Variables|Default|GetSaveInfo) (Variables|/Game/SpaceState/Blueprint/BP_Dude.BP_Dude_C|GetHealth%20Current (Variables|Default|GetCharInfo)))
          (Variables|/Game/SpaceState/Blueprint/SaveLoad/Save_info.Save_info_C|SetCheckCreds (Variables|Default|GetSaveInfo) (Variables|/Game/SpaceState/Blueprint/BP_Dude.BP_Dude_C|GetCharCredits (Variables|Default|GetCharInfo)))
          (SaveGame|SaveGametoSlot (Variables|Default|GetSaveInfo) "Loc")))
      (else
        (|DoOnceMultiInput
          (:A%20Out
            (Variables|/Game/SpaceState/Blueprint/SaveLoad/Save_info.Save_info_C|SetCheckLocation (Variables|Default|GetSaveInfo) (Math|Vector|MakeVector (.x (Transformation|GetActorLocation (Variables|Default|GetCharInfo))) (.y (Transformation|GetActorLocation (Variables|Default|GetCharInfo))) (.z (Transformation|GetActorLocation (Variables|Default|GetCharInfo)))))
            (bind _returnvalue_3 (Game|GetCurrentLevelName true))
            (Variables|/Game/SpaceState/Blueprint/SaveLoad/Save_info.Save_info_C|SetCurrentLevel (Variables|Default|GetSaveInfo) (Utilities|String|StringToName _returnvalue_3))
            (Variables|/Game/SpaceState/Blueprint/SaveLoad/Save_info.Save_info_C|SetCheckBullets (Variables|Default|GetSaveInfo) (Variables|/Game/SpaceState/Blueprint/BP_Dude.BP_Dude_C|GetCurrentBullets (Variables|Default|GetCharInfo)))
            (Variables|/Game/SpaceState/Blueprint/SaveLoad/Save_info.Save_info_C|SetCheckCells (Variables|Default|GetSaveInfo) (Variables|/Game/SpaceState/Blueprint/BP_Dude.BP_Dude_C|GetCurrentCells (Variables|Default|GetCharInfo)))
            (Variables|/Game/SpaceState/Blueprint/SaveLoad/Save_info.Save_info_C|SetCheckFuel (Variables|Default|GetSaveInfo) (Variables|/Game/SpaceState/Blueprint/BP_Dude.BP_Dude_C|GetCurrentFuel (Variables|Default|GetCharInfo)))
            (Variables|/Game/SpaceState/Blueprint/SaveLoad/Save_info.Save_info_C|SetCheckShells (Variables|Default|GetSaveInfo) (Variables|/Game/SpaceState/Blueprint/BP_Dude.BP_Dude_C|GetCurrentShells (Variables|Default|GetCharInfo)))
            (Variables|/Game/SpaceState/Blueprint/SaveLoad/Save_info.Save_info_C|SetCheckWeapons (Variables|Default|GetSaveInfo) (Variables|/Game/SpaceState/Blueprint/BP_Dude.BP_Dude_C|GetWeaponIndex (Variables|Default|GetCharInfo)))
            (Variables|/Game/SpaceState/Blueprint/SaveLoad/Save_info.Save_info_C|SetCheckHP (Variables|Default|GetSaveInfo) (Variables|/Game/SpaceState/Blueprint/BP_Dude.BP_Dude_C|GetHealth%20Current (Variables|Default|GetCharInfo)))
            (Variables|/Game/SpaceState/Blueprint/SaveLoad/Save_info.Save_info_C|SetCheckCreds (Variables|Default|GetSaveInfo) (Variables|/Game/SpaceState/Blueprint/BP_Dude.BP_Dude_C|GetCharCredits (Variables|Default|GetCharInfo)))
            (SaveGame|SaveGametoSlot (Variables|Default|GetSaveInfo) "Loc")))))))

(fn ConstructionScript
  (Components|Box|SetBoxExtent (Variables|Default|GetBox) (Variables|Default|GetChangeHitbox) true)
  (if (Variables|Default|GetCheckpoint)
    (Rendering|Components|Sprite|SetSprite (Variables|Default|GetBillboard) "/Game/SpaceState/Sprites/check.check")
    (else
      (Rendering|Components|Sprite|SetSprite (Variables|Default|GetBillboard) "/Game/SpaceState/Sprites/save.save"))))