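; BP_Lift is a sprite lift that shuttles between its origin and an editable end location.
; A timeline lerps the sprite's position, and on finishing fades audio out, waits StopDelay, fades audio in and runs the opposite direction.
; A safety collider reverses the active timeline when BP_Dude overlaps it.
; The construction script applies the lift colour and can preview the end position.
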(event OnComponentBeginOverlap(SafetyCollider)
  (params (OverlappedComponent :type Primitive%20Component%20Object%20Reference) (OtherActor :type Actor%20Object%20Reference) (OtherComp :type Primitive%20Component%20Object%20Reference) (OtherBodyIndex :type Integer) (bFromSweep :type Boolean) (SweepResult :type Hit%20Result%20Structure%20%28by%20ref%29))
  (bind _lift_timeline (Variables|Default|GetLift_Timeline))
  (Utilities|Casting|CastToBP_Dude OtherActor)
  (if (Components|Activation|IsActive _lift_timeline)
    (if (Audio|Components|Audio|IsPlaying _lift_timeline)
      (bind (_direction _lerp_alpha) (Timeline|Lift_Timeline Reverse)
        (:Update
          (Transformation|SetRelativeLocation (Variables|Default|GetPaperSprite) (Math|Vector|Lerp(Vector) "0, 0, 0" (Variables|LiftControls|GetEndLocation) _lerp_alpha) false false))
        (:Finished
          (Audio|Components|Audio|FadeOut (Variables|Default|GetAudio) 0.1 0.0 :!class /Script/Engine.AudioComponent)
          (Utilities|FlowControl|Delay (Variables|LiftControls|GetStopDelay))
          (Audio|Components|Audio|FadeIn (Variables|Default|GetAudio) 0.1 1.0 0.0 :!class /Script/Engine.AudioComponent)
          (switch Utilities|FlowControl|Switch|SwitchonETimelineDirection _direction
            (:Forward
              (CallFunction|LiftBackward))
            (:Backward
              (CallFunction|LiftForward)))))
      (else
        (Timeline|Lift_Timeline Reverse)))))

(event Custom|LiftForward
  (bind (_direction _lerp_alpha) (Timeline|Lift_Timeline PlayFromStart)
    (:Update
      (Transformation|SetRelativeLocation (Variables|Default|GetPaperSprite) (Math|Vector|Lerp(Vector) "0, 0, 0" (Variables|LiftControls|GetEndLocation) _lerp_alpha) false false))
    (:Finished
      (Audio|Components|Audio|FadeOut (Variables|Default|GetAudio) 0.1 0.0 :!class /Script/Engine.AudioComponent)
      (Utilities|FlowControl|Delay (Variables|LiftControls|GetStopDelay))
      (Audio|Components|Audio|FadeIn (Variables|Default|GetAudio) 0.1 1.0 0.0 :!class /Script/Engine.AudioComponent)
      (switch Utilities|FlowControl|Switch|SwitchonETimelineDirection _direction
        (:Forward
          (CallFunction|LiftBackward))
        (:Backward
          (CallFunction|LiftForward))))))

(event Custom|LiftBackward
  (bind (_direction _lerp_alpha) (Timeline|Lift_Timeline ReverseFromEnd)
    (:Update
      (Transformation|SetRelativeLocation (Variables|Default|GetPaperSprite) (Math|Vector|Lerp(Vector) "0, 0, 0" (Variables|LiftControls|GetEndLocation) _lerp_alpha) false false))
    (:Finished
      (Audio|Components|Audio|FadeOut (Variables|Default|GetAudio) 0.1 0.0 :!class /Script/Engine.AudioComponent)
      (Utilities|FlowControl|Delay (Variables|LiftControls|GetStopDelay))
      (Audio|Components|Audio|FadeIn (Variables|Default|GetAudio) 0.1 1.0 0.0 :!class /Script/Engine.AudioComponent)
      (switch Utilities|FlowControl|Switch|SwitchonETimelineDirection _direction
        (:Forward
          (CallFunction|LiftBackward))
        (:Backward
          (CallFunction|LiftForward))))))

(fn ConstructionScript
  (bind _papersprite (Variables|Default|GetPaperSprite))
  (Transformation|SetRelativeLocation _papersprite (Math|Vector|SelectVector (Variables|LiftControls|GetEndLocation) "0, 0, 0" (Variables|LiftControls|GetTestEndLocation)) false false)
  (Sprite|SetSpriteColor _papersprite (Variables|LiftControls|GetLiftColour)))