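; BP_Shot is a weapon shot actor that damages enemies on hit and plays ricochet sounds.
; On Hit, it confirms the player is BP_Dude, plays a one-time impact sound and starts a short delayed destroy, skipped when the player's current WeaponIndex is 4.
; Hits on a BP_MasterBad also call DMGBadman with the shot's Damage and play a second one-time sound.
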(event Custom|Hit
  (Utilities|FlowControl|Delay 0.25)
  (if (not (== (Variables|/Game/SpaceState/Blueprint/BP_Dude.BP_Dude_C|GetWeaponIndex (stale Collision|EventHit _asbp_dude)) 4))
    (Actor|DestroyActor)))

(event Custom|Sound
  (Utilities|FlowControl|DoOnce false
    (:Completed
      (Audio|SpawnSoundatLocation "/Game/SpaceState/Allsounds/Sounds/Ricochet.Ricochet" (stale Collision|EventHit HitLocation)))))

(event Custom|HitSound
  (Utilities|FlowControl|DoOnce false
    (:Completed
      (Audio|SpawnSoundatLocation "/Game/SpaceState/Allsounds/Sounds/Ricochet2.Ricochet2" (stale Collision|EventHit HitLocation)))))

(event Collision|EventActorBeginOverlap
  (params (OtherActor :type Actor%20Object%20Reference)))

(event Collision|EventHit
  (params (MyComp :type Primitive%20Component%20Object%20Reference) (Other :type Actor%20Object%20Reference) (OtherComp :type Primitive%20Component%20Object%20Reference) (bSelfMoved :type Boolean) (HitLocation :type Vector) (HitNormal :type Vector :default "0, 0, 0") (NormalImpulse :type Vector :default "0, 0, 0") (Hit :type Hit%20Result%20Structure%20%28by%20ref%29))
  (bind _asbp_dude (Utilities|Casting|CastToBP_Dude (Game|GetPlayerCharacter 0)))
  (CallFunction|Sound)
  (CallFunction|Hit)
  (bind _asbp_master_bad (Utilities|Casting|CastToBP_MasterBad Other))
  (Default|DMGBadman _asbp_master_bad (Variables|Default|GetDamage))
  (CallFunction|HitSound))

(fn ConstructionScript)