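; BP_CoverBox is a 2D sprite cover object that the player and AI enemies can toggle in and out of.
; Box overlaps message actors when it becomes usable or unusable.
; Use flips InCover on BP_Dude or AI_EnemyController, enabling sprite collision on a custom channel while in cover and disabling it on exit.
; Entering snaps the user flush to the nearer side using sprite bounds; the player also crouches and loses movement until leaving.
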(event OnComponentBeginOverlap(Box)
  (params (OverlappedComponent :type Primitive%20Component%20Object%20Reference) (OtherActor :type Actor%20Object%20Reference) (OtherComp :type Primitive%20Component%20Object%20Reference) (OtherBodyIndex :type Integer) (bFromSweep :type Boolean) (SweepResult :type Hit%20Result%20Structure%20%28by%20ref%29))
  (Class|BPInterface|CanbeInteractedwith(Message) OtherActor self true))

(event OnComponentEndOverlap(Box)
  (params (OverlappedComponent :type Primitive%20Component%20Object%20Reference) (OtherActor :type Actor%20Object%20Reference) (OtherComp :type Primitive%20Component%20Object%20Reference) (OtherBodyIndex :type Integer))
  ;[1 1 1] CantUse
  (Class|BPInterface|CanbeInteractedwith(Message) OtherActor self false))

(event EventBeginPlay)

(event Collision|EventActorBeginOverlap
  (params (OtherActor :type Actor%20Object%20Reference)))

(event EventTick
  (params (DeltaSeconds :type Float%20%28single-precision%29)))

(event EventUse
  (params (InteractedObject :type Actor%20Object%20Reference) (IsUsable :type Boolean))
  (bind _self self)
  (bind _self_2 self)
  (bind _self_3 self)
  (bind _papersprite (Variables|Default|GetPaperSprite))
  (bind _papersprite_2 (Variables|Default|GetPaperSprite))
  (bind _returnvalue (Transformation|GetActorLocation _self_3))
  (bind _returnvalue_2 (Transformation|GetActorLocation _self))
  (bind _returnvalue_3 (Transformation|GetActorLocation _self_2))
  (bind _output_get (Variables|Default|SetObject InteractedObject))
  (if (== _output_get (Game|GetPlayerCharacter 0))
    (bind _asbp_dude (Utilities|Casting|CastToBP_Dude (Game|GetPlayerCharacter 0)))
    (if (Variables|/Game/SpaceState/Blueprint/BP_Dude/BP_Dude.BP_Dude_C|GetInCover _asbp_dude)
      (Variables|/Game/SpaceState/Blueprint/BP_Dude/BP_Dude.BP_Dude_C|SetInCover _asbp_dude false)
      (Variables|/Game/SpaceState/Blueprint/BP_Dude/BP_Dude.BP_Dude_C|SetCanMove _asbp_dude true)
      (Collision|SetCollisionEnabled _papersprite_2 "NoCollision")
      (else
        (Variables|/Game/SpaceState/Blueprint/BP_Dude/BP_Dude.BP_Dude_C|SetInCover _asbp_dude true)
        (Variables|/Game/SpaceState/Blueprint/BP_Dude/BP_Dude.BP_Dude_C|SetCanMove _asbp_dude false)
        (Collision|SetCollisionEnabled _papersprite_2 "QueryAndPhysics")
        (Collision|SetCollisionObjectType _papersprite_2 "ECC_GameTraceChannel2")
        (if (> (.x (Transformation|GetActorLocation _asbp_dude)) (.x (Transformation|GetActorLocation self)))
          (Transformation|Teleport _asbp_dude (Math|Vector|MakeVector (+ (+ (.x (.BoxExtent (Collision|GetComponentBounds (Variables|/Script/Paper2D.PaperCharacter|GetSprite _asbp_dude)))) (.x (.BoxExtent (Collision|GetComponentBounds (Variables|Default|GetPaperSprite))))) (.x _returnvalue_3)) (.y _returnvalue_3) (.z _returnvalue_3)) "0, 0, 0")
          (Default|ForceCrouch _asbp_dude)
          (else
            (Transformation|Teleport _asbp_dude (Math|Vector|MakeVector (- (.x _returnvalue_2) (+ (.x (.BoxExtent (Collision|GetComponentBounds (Variables|/Script/Paper2D.PaperCharacter|GetSprite _asbp_dude)))) (.x (.BoxExtent (Collision|GetComponentBounds (Variables|Default|GetPaperSprite)))))) (.y _returnvalue_2) (.z _returnvalue_2)) "0, 0, 0")
            (Default|ForceCrouch _asbp_dude)))))
    (else
      (bind _asai_enemy (Utilities|Casting|CastToAI_Enemy (Variables|Default|GetObject)))
      (bind _asai_enemy_controller (Utilities|Casting|CastToAI_EnemyController (Pawn|GetController _asai_enemy)))
      (if (Variables|/Game/SpaceState/Blueprint/Enemies/AIEnemy/AI_Enemy/AI_EnemyController.AI_EnemyController_C|GetInCover _asai_enemy_controller)
        (Variables|/Game/SpaceState/Blueprint/Enemies/AIEnemy/AI_Enemy/AI_EnemyController.AI_EnemyController_C|SetInCover _asai_enemy_controller false)
        (Collision|SetCollisionEnabled _papersprite "NoCollision")
        (else
          (Variables|/Game/SpaceState/Blueprint/Enemies/AIEnemy/AI_Enemy/AI_EnemyController.AI_EnemyController_C|SetInCover _asai_enemy_controller true)
          (Collision|SetCollisionEnabled _papersprite "QueryAndPhysics")
          (Collision|SetCollisionObjectType _papersprite "ECC_GameTraceChannel2")
          (if (> (.x (Transformation|GetActorLocation (Pawn|GetControlledPawn _asai_enemy_controller))) (.x (Transformation|GetActorLocation self)))
            (Transformation|Teleport _asai_enemy (Math|Vector|MakeVector (+ (+ (.x (.BoxExtent (Collision|GetComponentBounds (Variables|/Script/Paper2D.PaperCharacter|GetSprite _asai_enemy)))) (.x (.BoxExtent (Collision|GetComponentBounds (Variables|Default|GetPaperSprite))))) (.x _returnvalue)) (.y _returnvalue) (.z _returnvalue)) "0, 0, 0")
            (else
              (Transformation|Teleport _asai_enemy (Math|Vector|MakeVector (- (.x (Transformation|GetActorLocation self)) (+ (.x (.BoxExtent (Collision|GetComponentBounds (Variables|/Script/Paper2D.PaperCharacter|GetSprite _asai_enemy)))) (.x (.BoxExtent (Collision|GetComponentBounds (Variables|Default|GetPaperSprite)))))) 0.0 0.0) "0, 0, 0"))))))))

(fn ConstructionScript)