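; CoverBox_A is a 2D interactable cover box that the player and AI enemies toggle in and out of.
; Its overlap box flags it usable; Use flips the player's InCover variable or the enemy's blackboard key, plus sprite collision.
; Entering cover teleports the user flush against the sprite using bounds extents.
; The player stays on their approach side, crouched and immobile, while enemies take the side opposite the player.
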(event OnComponentBeginOverlap(Box)
  (params (OverlappedComponent :type Primitive%20Component%20Object%20Reference) (OtherActor :type Actor%20Object%20Reference) (OtherComp :type Primitive%20Component%20Object%20Reference) (OtherBodyIndex :type Integer) (bFromSweep :type Boolean) (SweepResult :type Hit%20Result%20Structure%20%28by%20ref%29))
  (Class|BPInterface|CanbeInteractedwith(Message) OtherActor self true))

(event OnComponentEndOverlap(Box)
  (params (OverlappedComponent :type Primitive%20Component%20Object%20Reference) (OtherActor :type Actor%20Object%20Reference) (OtherComp :type Primitive%20Component%20Object%20Reference) (OtherBodyIndex :type Integer))
  ;[1 1 1] CantUse
  (Class|BPInterface|CanbeInteractedwith(Message) OtherActor self false))

(event EventUse
  (params (InteractedObject :type Actor%20Object%20Reference) (IsUsable :type Boolean))
  (bind _self self)
  (bind _self_2 self)
  (bind _self_3 self)
  (bind _self_4 self)
  (bind _papersprite (Variables|Default|GetPaperSprite))
  (bind _papersprite_2 (Variables|Default|GetPaperSprite))
  (bind _returnvalue (Transformation|GetActorLocation _self_3))
  (bind _returnvalue_2 (Transformation|GetActorLocation _self))
  (bind _returnvalue_3 (Transformation|GetActorLocation _self_4))
  (bind _returnvalue_4 (Transformation|GetActorLocation _self_2))
  (bind _output_get (Variables|Default|SetObject InteractedObject))
  (if (== _output_get (Game|GetPlayerCharacter 0))
    (bind _asbp_dude (Utilities|Casting|CastToBP_Dude (Game|GetPlayerCharacter 0)))
    (if (Variables|/Game/SpaceState/Blueprint/BP_Dude/BP_Dude.BP_Dude_C|GetInCover _asbp_dude)
      (Variables|/Game/SpaceState/Blueprint/BP_Dude/BP_Dude.BP_Dude_C|SetInCover _asbp_dude false)
      (Variables|/Game/SpaceState/Blueprint/BP_Dude/BP_Dude.BP_Dude_C|SetCanMove _asbp_dude true)
      (Collision|SetCollisionEnabled _papersprite_2 "NoCollision")
      (else
        (Variables|/Game/SpaceState/Blueprint/BP_Dude/BP_Dude.BP_Dude_C|SetInCover _asbp_dude true)
        (Variables|/Game/SpaceState/Blueprint/BP_Dude/BP_Dude.BP_Dude_C|SetCanMove _asbp_dude false)
        (Collision|SetCollisionEnabled _papersprite_2 "QueryAndPhysics")
        (Collision|SetCollisionObjectType _papersprite_2 "ECC_GameTraceChannel2")
        (if (> (.x (Transformation|GetActorLocation _asbp_dude)) (.x (Transformation|GetActorLocation self)))
          (Transformation|Teleport _asbp_dude (Math|Vector|MakeVector (+ (+ (.x (.BoxExtent (Collision|GetComponentBounds (Variables|/Script/Paper2D.PaperCharacter|GetSprite _asbp_dude)))) (.x (.BoxExtent (Collision|GetComponentBounds (Variables|Default|GetPaperSprite))))) (.x _returnvalue_4)) (.y _returnvalue_4) (.z _returnvalue_4)) "0, 0, 0")
          (Default|ForceCrouch _asbp_dude)
          (else
            (Transformation|Teleport _asbp_dude (Math|Vector|MakeVector (- (.x _returnvalue_2) (+ (.x (.BoxExtent (Collision|GetComponentBounds (Variables|/Script/Paper2D.PaperCharacter|GetSprite _asbp_dude)))) (.x (.BoxExtent (Collision|GetComponentBounds (Variables|Default|GetPaperSprite)))))) (.y _returnvalue_2) (.z _returnvalue_2)) "0, 0, 0")
            (Default|ForceCrouch _asbp_dude)))))
    (else
      (bind _asai_enemy_controler (Utilities|Casting|CastToAI_EnemyControler (Variables|Default|GetObject)))
      (bind _asai_enemy (Utilities|Casting|CastToAI_Enemy (Pawn|GetControlledPawn _asai_enemy_controler)))
      (bind _asbp_dude_2 (Utilities|Casting|CastToBP_Dude (Game|GetPlayerCharacter 0)))
      (if (ScalableFloat|GetValueasBool (AI|GetBlackboard _asai_enemy_controler) (Variables|Default|GetInCover))
        (AI|Components|Blackboard|SetValueasBool (Variables|/Script/AIModule.AIController|GetBlackboard _asai_enemy_controler) (Variables|Default|GetInCover) false)
        (Collision|SetCollisionEnabled _papersprite "NoCollision")
        (else
          (AI|Components|Blackboard|SetValueasBool (Variables|/Script/AIModule.AIController|GetBlackboard _asai_enemy_controler) (Variables|Default|GetInCover) true)
          (Collision|SetCollisionEnabled _papersprite "QueryAndPhysics")
          (Collision|SetCollisionObjectType _papersprite "ECC_GameTraceChannel2")
          (if (> (.x (Transformation|GetActorLocation self)) (.x (Transformation|GetActorLocation _asbp_dude_2)))
            (Transformation|Teleport _asai_enemy (Math|Vector|MakeVector (+ (+ (.x (.BoxExtent (Collision|GetComponentBounds (Variables|/Game/SpaceState/Blueprint/Enemies/AIEnemy/AI_Enemy/AI_Enemy.AI_Enemy_C|GetPaperFlipbook _asai_enemy)))) (.x (.BoxExtent (Collision|GetComponentBounds (Variables|Default|GetPaperSprite))))) (.x _returnvalue)) (.y _returnvalue) (.z _returnvalue)) "0, 0,0.000000")
            (else
              (Transformation|Teleport _asai_enemy (Math|Vector|MakeVector (- (.x _returnvalue_3) (+ (.x (.BoxExtent (Collision|GetComponentBounds (Variables|/Game/SpaceState/Blueprint/Enemies/AIEnemy/AI_Enemy/AI_Enemy.AI_Enemy_C|GetPaperFlipbook _asai_enemy)))) (.x (.BoxExtent (Collision|GetComponentBounds (Variables|Default|GetPaperSprite)))))) (.y _returnvalue_3) (.z _returnvalue_3)) "0, 0, 0"))))))))

(fn ConstructionScript)